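; BP_ShipFeedback_Alarm is a sound and light alarm actor that gives feedback when its ship gets hit.
; Setup binds it to the ship's hit event, which plays the audio and starts an actor sequence looping.
; A short Delay loop polls the audio play state, then stops the sequence and sets the spotlight intensity to zero once the sound has finished.
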(event Custom|BoatGotHit
  (Audio|Components|Audio|Play (Variables|Default|GetAudio) 0.0)
  (Class|MovieSceneSequencePlayer|PlayLooping (Variables|/Script/ActorSequence.ActorSequenceComponent|GetSequencePlayer (Variables|Default|GetActorSequence)) -1)
  (Utilities|FlowControl|Delay 0.01 :!label _label)
  (if (Utilities|Enum|Equal(Enum) (Audio|Components|Audio|GetPlayState (Variables|Default|GetAudio)) "Stopped")
    (Sequencer|Player|Stop (Variables|/Script/ActorSequence.ActorSequenceComponent|GetSequencePlayer (Variables|Default|GetActorSequence)) :!class /Script/MovieScene.MovieSceneSequencePlayer)
    (Utilities|FlowControl|Delay 0.2)
    (Rendering|Components|Light|SetIntensity (Variables|Default|GetSpotLight) 0.0)
    (else
      (goto _label))))

(event Custom|SetupSoundLightFeedback
  (params (Ship :type BP%20Ship%20Handler%20Object%20Reference))
  (EventDispatchers|BindEventtoOnShipHit Ship (delegate Custom|BoatGotHit)))

(event Collision|EventActorBeginOverlap
  (params (OtherActor :type Actor%20Object%20Reference)))

(event EventTick
  (params (DeltaSeconds :type Float%20%28single-precision%29)))

(fn ConstructionScript)