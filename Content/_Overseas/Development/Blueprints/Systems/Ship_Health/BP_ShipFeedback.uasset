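; BP_ShipFeedback coordinates audio, alarm and camera feedback when the ship is hit.
; SetupFeedbackOnHit passes the Ship to every BP_ShipFeedback_Alarm for sound and light setup, then binds ShipHit to the ship's hit event.
; On a hit, it waits, plays the Sound_Impact actor found at BeginPlay, then after another delay starts a BP_CamShake camera shake.
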(event Custom|SetupFeedbackOnHit
  (params (Ship :type BP%20Ship%20Handler%20Object%20Reference))
  (bind _outactors (Actor|GetAllActorsOfClass "/Game/_Overseas/Development/Blueprints/Systems/Ship_Health/BP_ShipFeedback_Alarm.BP_ShipFeedback_Alarm_C"))
  (Variables|Internal|SetAlarm%20Feedback _outactors)
  (for _array_element (Variables|Internal|GetAlarm%20Feedback)
    (Default|SetupSoundLightFeedback _array_element Ship))
  (EventDispatchers|BindEventtoOnShipHit Ship (delegate Custom|ShipHit)))

(event Custom|ShipHit
  (Utilities|FlowControl|Delay 6.0)
  (Audio|Components|Audio|Play (Variables|/Script/Engine.AmbientSound|GetAudioComponent (Variables|Internal|GetImpactSound)) 0.0)
  (Utilities|FlowControl|Delay 3.0)
  (CameraShakes|StartCameraShake (Game|GetPlayerCameraManager 0) "/Game/_Overseas/Development/Blueprints/Assets/Misc/BP_CamShake.BP_CamShake_C" 1.0 "CameraLocal" "0, 0, 0"))

(event EventBeginPlay
  (bind _returnvalue (Actor|GetActorOfClass "/Game/_Overseas/Development/Audio/Ship/Sound_Impact.Sound_Impact_C"))
  (Variables|Internal|SetImpactSound _returnvalue))

(event Collision|EventActorBeginOverlap
  (params (OtherActor :type Actor%20Object%20Reference)))

(event EventTick
  (params (DeltaSeconds :type Float%20%28single-precision%29)))

(fn ConstructionScript)

(fn OnRepCurrentCourse)