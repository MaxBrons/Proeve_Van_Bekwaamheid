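; Placeholder task actor in the task system, apparently for testing the task start and stop flow.
; On start it prints a debug greeting and immediately calls StopTask on the current pawn, and the stop event prints a completion message.
; IsTaskDone always returns true, and the default BeginPlay, overlap and Tick events are left unused.
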(event EventBeginPlay
  (|CallParentFunction) ; This node is disabled and will not be called.\nDrag off pins to build functionality.
)

(event Collision|EventActorBeginOverlap
  (params (OtherActor :type Actor%20Object%20Reference)))

(event EventTick
  (params (DeltaSeconds :type Float%20%28single-precision%29)))

(event EventOnTaskStart
  (Development|PrintString "Hello")
  (CallFunction|StopTask (Variables|Default|GetCurrent%20Pawn)))

(event EventOnTaskStop
  (Development|PrintString "Done"))

(fn ConstructionScript
  (|CallParentFunction))

(fn IsTaskDone
  (return true))