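; Task Blueprint for steering, completed when a pawn presses interact on the referenced steering wheel.
; On task start, a DoOnce-guarded step binds to the wheel's focus component press event and clears the done flag.
; The press handler unbinds itself, marks the task done and calls StopTask, which resets the guard.
; IsTaskDone reports the flag, while start and stop also call the parent task logic.
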(event Custom|On%20Interaction%20Pressed
  (params (Pawn :type BP%20Pawn%20Base%20Object%20Reference) (Souce%20Actor :type Actor%20Object%20Reference) (Hit%20Location :type Vector) (Hit%20Distance :type Float%20%28single-precision%29) (Hit%20Component :type Actor%20Component%20Object%20Reference))
  (EventDispatchers|UnbindEventfromPressedInteraction (stale EventStartTask _comp_focus) (delegate Custom|On%20Interaction%20Pressed))
  (Variables|Internal|SetTask%20Done true)
  (CallFunction|StopTask Pawn))

(event EventBeginPlay
  (|CallParentFunction))

(event EventStartTask
  (params (Pawn :type BP%20Pawn%20Base%20Object%20Reference))
  (|CallParentFunction Pawn)
  (Utilities|FlowControl|DoOnce false
    (:Completed
      (bind _steering_wheel (Variables|Settings|GetSteering%20Wheel)
        (:then
          (bind _comp_focus (Variables|/Game/_Overseas/Development/Blueprints/Assets/Ship/BP_SteeringWheel.BP_SteeringWheel_C|GetComp_Focus _steering_wheel)
            (:then
              (EventDispatchers|BindEventtoPressedInteraction _comp_focus (delegate Custom|On%20Interaction%20Pressed))
              (Variables|Internal|SetTask%20Done false))
            (:else)))
        (:else)))))

(event EventStopTask
  (params (Pawn :type BP%20Pawn%20Base%20Object%20Reference))
  (|CallParentFunction Pawn)
  (Utilities|FlowControl|DoOnce false) ; enters at Reset
)

(fn ConstructionScript
  (|CallParentFunction))

(fn IsTaskDone
  (return (Variables|Internal|GetTask%20Done)))