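; Task Blueprint that has the player turn a steering wheel to a target angle.
; On start it spawns a steering focus pawn at the player camera, bound to the controlled actor, and switches the player controller to it.
; A short Delay loop prints the current degrees until their truncated value exactly equals the target, then marks the task done.
; Stopping the task transfers control back from the focus pawn.
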(event EventBeginPlay
  (|CallParentFunction) ; This node is disabled and will not be called.\nDrag off pins to build functionality.
)

(event EventStartTask
  (bind _self self)
  (bind _player_pawn (CallFunction|GetMainPlayerPawn _self))
  (bind _returnvalue (Actor|GetComponentbyClass _player_pawn "/Script/Engine.CameraComponent"))
  (bind _returnvalue_2 (Transformation|GetWorldTransform _returnvalue))
  (|CallParentFunction)
  (Variables|Internal|SetTarget%20Reached false)
  (bind _returnvalue_3 (Game|SpawnActorfromClass "/Game/_Overseas/Development/Blueprints/Pawns/BP_Pawn_Focus_Steering.BP_Pawn_Focus_Steering_C" (Math|Transform|MakeTransform (.location _returnvalue_2) (.rotation _returnvalue_2) "1,1,1") "AlwaysSpawn" 0 (Variables|Settings|GetActor%20To%20Control) (Variables|Settings|GetSteering%20Speed) (Variables|Settings|GetSteering%20Offset) _player_pawn 0))
  (Variables|Internal|SetCurrent%20Focus%20Pawn _returnvalue_3)
  (bind _asbp_player_controller_main (Utilities|Casting|CastToBP_PlayerController_Main (Pawn|GetController _player_pawn)))
  (Default|SwitchPawn _asbp_player_controller_main _returnvalue_3)
  (bind _current_focus_pawn (Variables|Internal|GetCurrent%20Focus%20Pawn :!label _label)
    (:then
      (if (== (Variables|Settings|GetTarget%20Degrees) (Math|Float|Truncate (Default|GetCurrentDegrees _current_focus_pawn)))
        (Variables|Internal|SetTarget%20Reached true)
        (CallFunction|StopTask)
        (else
          (Utilities|FlowControl|Delay 0.05)
          (Development|PrintString (Utilities|String|ToString(Float) (Default|GetCurrentDegrees _current_focus_pawn)))
          (goto _label))))
    (:else)))

(event EventStopTask
  (|CallParentFunction)
  (bind _current_focus_pawn (Variables|Internal|GetCurrent%20Focus%20Pawn)
    (:then
      (Default|TransferBacktoPawn _current_focus_pawn))
    (:else)))

(fn ConstructionScript
  (|CallParentFunction))

(fn IsTaskDone
  (return (Variables|Internal|GetTarget%20Reached)))