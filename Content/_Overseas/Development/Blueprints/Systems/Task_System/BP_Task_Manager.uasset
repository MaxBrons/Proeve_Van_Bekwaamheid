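; BP_Task_Manager is an actor that keeps an ordered list of BP_Task actors and runs one as the current task for the main player pawn.
; On BeginPlay it polls until the task actor count stops growing, sorts by ascending TaskID and can auto-start.
; Starts and stops route through the pawn's HandleTask.
; An update binding advances to the next task on Stopped, preferring paused tasks over unfinished ones.
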(event Custom|Stop%20Task
  (params (Task%20To%20Stop :type BP%20Task%20Object%20Reference))
  ;[1 1 1] This event stops the task given as a parameter if the task is active.
  (if (Utilities|Enum|Equal(Enum) (Variables|/Game/_Overseas/Development/Blueprints/Systems/Task_System/BP_Task.BP_Task_C|GetTask%20State Task%20To%20Stop) "NewEnumerator2")
    (Default|HandleTask (CallFunction|GetMainPlayerPawn self) Task%20To%20Stop "NewEnumerator4")
    (Development|PrintString (Utilities|String|Append "Task Stopped/Paused: " (Utilities|GetObjectName Task%20To%20Stop)))))

(event Custom|Add%20Task
  (params (Task%20To%20Add :type BP%20Task%20Object%20Reference))
  ;[1 1 1] This event adds the task given as a parameter to the task list, than sorts that list and starts the tasks with the highest priority based on their Task ID.
  (Utilities|IsValid Task%20To%20Add
    (:Is%20Valid
      (Utilities|Array|Add (Variables|Internal|GetTask%20List) Task%20To%20Add)
      (CallFunction|SortTaskList)
      (if (Variables|Settings|GetStart%20Tasks%20Automatically)
        (Variables|Internal|GetCurrent%20Task
          (:then
            (CallFunction|StartTask (CallFunction|GetNextTask)))
          (:else))))))

(event Custom|Remove%20Task
  (params (Task%20To%20Remove :type BP%20Task%20Object%20Reference))
  (bind _current_task (Variables|Internal|GetCurrent%20Task))
  ;[1 1 1] This event removes a task from the task list and stops the current task if the task given as a parameter is the current task.
  (Utilities|IsValid Task%20To%20Remove
    (:Is%20Valid
      (Utilities|Array|RemoveItem (Variables|Internal|GetTask%20List) Task%20To%20Remove)
      (if (== Task%20To%20Remove _current_task)
        (CallFunction|StopTask _current_task)))))

(event Custom|On%20Current%20Task%20Update
  (params (Task%20Reference :type BP%20Task%20Object%20Reference) (Task%20Name :type Name) (Task%20ID :type Integer) (Task%20State :type E_Task_State%20Enum :default "NewEnumerator0") (Pawn :type BP%20Pawn%20Base%20Object%20Reference))
  (bind _next_task (CallFunction|GetNextTask))
  ;[1 1 1] This event fires when the current task is updated. We check if this task is done or paused. If the task is done, we start the next task in the list. If the task is paused, we only unsubscribe from the On Task Update event.
  (switch Utilities|FlowControl|Switch|SwitchonE_Task_State Task%20State
    (:NewEnumerator3
      (EventDispatchers|UnbindEventfromOnTaskUpdated Task%20Reference (delegate Custom|On%20Current%20Task%20Update) :!label _label))
    (:NewEnumerator4
      (Utilities|FlowControl|Sequence
        (:then_0
          (goto _label))
        (:then_1
          (Variables|Internal|SetCurrent%20Task 0)
          (if (Variables|Settings|GetStart%20Tasks%20Automatically)
            (Utilities|IsValid _next_task
              (:Is%20Valid
                (CallFunction|StartTask _next_task)))))))))

(event Custom|Start%20Task
  (params (Task%20To%20Start :type BP%20Task%20Object%20Reference))
  ;[1 1 1] This event starts the task that is given as a parameter. If there is an active task, than that task will be stoppen/paused first. We bind to the On Task Update event from the new task to check when that task is done or when it pauses so we can automatically start the next task if necessary.
  (bind _next_task (CallFunction|SetupNextTask Task%20To%20Start))
  (Utilities|IsValid _next_task
    (:Is%20Valid
      (EventDispatchers|BindEventtoOnTaskUpdated _next_task (delegate Custom|On%20Current%20Task%20Update))
      (Default|HandleTask (CallFunction|GetMainPlayerPawn self) _next_task "NewEnumerator1")
      (Development|PrintString (Utilities|String|Append "Tast Started: " (Utilities|GetObjectName _next_task))))))

(event EventBeginPlay
  ;[1 1 1] This event waits for all tasks to be loaded in the scene that are relevant to this manager based on their Task ID, than sorts the list based on their Task ID and starts the first task in the list that is not done yet.
  (Utilities|WaitforObjecttoValidate (Game|GetPlayerController 0) 0.05
    (:Is%20Valid
      (if (>= (Variables|Settings|GetTask%20Manager%20ID) 0)
        (bind _task_list (Utilities|WaitforAllRelevantTasks 0.5)
          (:Done
            (Variables|Internal|SetTask%20List _task_list)
            (CallFunction|SortTaskList)
            (if (Variables|Settings|GetStart%20Tasks%20Automatically)
              (bind _current_task (Variables|Internal|GetCurrent%20Task)
                (:then
                  (Default|StartTask _current_task (CallFunction|GetMainPlayerPawn self)))
                (:else
                  (CallFunction|StartTask (CallFunction|GetNextTask)))))))
        (else
          (Actor|DestroyActor))))))

(fn ConstructionScript)

(fn SetupNextTask
  (params (New%20Task :type BP%20Task%20Object%20Reference))
  (Utilities|IsValid New%20Task
    (:Is%20Valid
      (bind _current_task (Variables|Internal|GetCurrent%20Task)
        (:then
          (Default|StopTask _current_task))
        (:else
          _))
      (bind _output_get (Variables|Internal|SetCurrent%20Task New%20Task))
      (return _output_get))
    (:Is%20Not%20Valid
      (return 0))))

(fn GetNextTask
  (bind _task_list (Variables|Internal|GetTask%20List))
  (for _array_element _task_list
    (switch Utilities|FlowControl|Switch|SwitchonE_Task_State (Variables|/Game/_Overseas/Development/Blueprints/Systems/Task_System/BP_Task.BP_Task_C|GetTask%20State _array_element)
      (:NewEnumerator3
        (return _array_element))))
  (for _array_element_2 _task_list
    (if (not (Default|IsTaskDone _array_element_2))
      (return _array_element_2))))

(fn SortTaskList
  (bind _unsorted_list (LocalVariables|GetUnsorted%20List))
  (bind _sorted_task_list (LocalVariables|GetSorted%20Task%20List))
  (bind _sorted_task_list_2 (LocalVariables|GetSorted%20Task%20List))
  (bind _indexofmaxvalue (Math|Integer|MaxOfIntArray _unsorted_list))
  (LocalVariables|SetUnsorted%20Task%20List (Variables|Internal|GetTask%20List))
  (for _array_element (Variables|Internal|GetTask%20List)
    (Utilities|Array|Add _unsorted_list (Variables|/Game/_Overseas/Development/Blueprints/Systems/Task_System/BP_Task.BP_Task_C|GetTask%20ID _array_element)))
  (while (LocalVariables|GetLoop)
    (if (== (Utilities|Array|Length _sorted_task_list) (Utilities|Array|Length (Variables|Internal|GetTask%20List)))
      (LocalVariables|SetLoop false)
      (else
        (Utilities|Array|Add _sorted_task_list (Utilities|Array|Get(acopy) (LocalVariables|GetUnsorted%20Task%20List) _indexofmaxvalue))
        (Utilities|Array|RemoveIndex (LocalVariables|GetUnsorted%20Task%20List) _indexofmaxvalue)
        (Utilities|Array|RemoveIndex (LocalVariables|GetUnsorted%20List) _indexofmaxvalue))))
  (Utilities|Array|Reverse _sorted_task_list_2)
  (Variables|Internal|SetTask%20List _sorted_task_list_2))