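; Base task actor for the task system, meant to be subclassed with its own hooks and completion check.
; On BeginPlay it destroys itself if TaskID is negative, finds its manager by ID and can auto-start through the player pawn.
; Comp_Active toggles start and stop, driving start, pause, unpause and done states that are broadcast on change.
; Stopping an unfinished task pauses it; the default IsTaskDone returns true.
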(event ActiveStateChanged(Comp_Active)
  (params (Pawn :type BP%20Pawn%20Base%20Object%20Reference) (Comp%20Active :type Comp%20Active%20Object%20Reference) (New%20Active :type Boolean))
  ;[1 1 1] Activate or deactivate the task.
  (if New%20Active
    (CallFunction|StartTask Pawn)
    (else
      (CallFunction|StopTask Pawn))))

(event Custom|Update%20Task%20State
  (params (Pawn :type BP%20Pawn%20Base%20Object%20Reference) (Task%20State :type E_Task_State%20Enum :default "NewEnumerator0"))
  ;[1 1 1] This event sets the task state variable and calls the On Task Update event.
  (bind _output_get (Variables|Internal|SetTask%20State Task%20State))
  (Default|CallOnTaskUpdated self (Variables|SettingsBase|GetTask%20Name) (Variables|SettingsBase|GetTask%20ID) _output_get Pawn))

(event Custom|Start%20Task
  (params (Pawn :type BP%20Pawn%20Base%20Object%20Reference))
  (bind _task_state (Variables|Internal|GetTask%20State))
  ;[1 1 1] This event can only start if the task is not yet in progress. If the task is paused it will be unpaused, else it will call that is starts. This event should be overridden to implement your own functionality. Make sure to call this base event when overriding this event.
  (if (CallFunction|IsTaskDone)
    (CallFunction|StopTask Pawn)
    (elif (not (Utilities|Enum|Equal(Enum) _task_state "NewEnumerator2"))
      (Variables|Internal|SetCurrent%20Pawn Pawn)
      (if (Utilities|Enum|Equal(Enum) _task_state "NewEnumerator3")
        (CallFunction|UnpauseTask Pawn)
        (else
          (Default|CallOnTaskStarted self (Variables|SettingsBase|GetTask%20Name) (Variables|SettingsBase|GetTask%20ID) Pawn)
          (CallFunction|OnTaskStart)
          (CallFunction|UpdateTaskState Pawn "NewEnumerator1")
          (CallFunction|UpdateTaskState Pawn "NewEnumerator2"))))))

(event Custom|On%20Task%20Pause
  ;[1 1 1] Override this event to implement you own functionality
)

(event Custom|Unpause%20Task
  (params (Pawn :type BP%20Pawn%20Base%20Object%20Reference))
  ;[1 1 1] This event updates the task state back to in progress. This event should be overridden to implement your own functionality. Make sure to call this base event when overriding this event.
  (CallFunction|OnTaskUnpause)
  (CallFunction|UpdateTaskState Pawn "NewEnumerator2"))

(event Custom|Stop%20Task
  (params (Pawn :type BP%20Pawn%20Base%20Object%20Reference))
  ;[1 1 1] This event checks if the task is done, if not, it will pause the task. If the task is done, it will call that it is done. This event should be overridden to implement your own functionality. Make sure to call this base event when overriding this event.
  (if (CallFunction|IsTaskDone)
    (Default|CallOnTaskDone self (Variables|SettingsBase|GetTask%20Name) (Variables|SettingsBase|GetTask%20ID) Pawn)
    (CallFunction|OnTaskStop)
    (CallFunction|UpdateTaskState Pawn "NewEnumerator4")
    (else
      (CallFunction|PauseTask Pawn))))

(event Custom|Pause%20Task
  (params (Pawn :type BP%20Pawn%20Base%20Object%20Reference))
  ;[1 1 1] This event updates the task state to paused. This event should be overridden to implement your own functionality. Make sure to call this base event when overriding this event.
  (CallFunction|OnTaskPause)
  (CallFunction|UpdateTaskState Pawn "NewEnumerator3"))

(event Custom|On%20Task%20Unpause
  ;[1 1 1] Override this event to implement you own functionality
)

(event Custom|On%20Task%20Start
  ;[1 1 1] Override this event to implement you own functionality
)

(event Custom|Reset%20Task
  (bind _current_pawn (Variables|Internal|GetCurrent%20Pawn))
  (Default|CallOnTaskDone self (Variables|SettingsBase|GetTask%20Name) (Variables|SettingsBase|GetTask%20ID) _current_pawn)
  (CallFunction|OnTaskStop)
  (CallFunction|UpdateTaskState _current_pawn "NewEnumerator0"))

(event Custom|On%20Task%20Stop
  ;[1 1 1] Override this event to implement you own functionality
)

(event EventBeginPlay
  (bind _self self)
  ;[1 1 1] Check if the Task ID or Task Manager ID are not less than 0 because that would invalidate then and they will be destroyed so they don't interfere with the rest of the system.
  (Utilities|WaitforObjecttoValidate (Game|GetPlayerController 0) 0.05
    (:Is%20Valid
      (if (< (Variables|SettingsBase|GetTask%20ID) 0)
        (Actor|DestroyActor)
        (else
          (bind _task_manager (CallFunction|GetTaskManager))
          (Utilities|IsValid _task_manager
            (:Is%20Valid
              (Variables|Internal|SetTask%20Manager _task_manager))
            (:Is%20Not%20Valid
              _))
          (if (Variables|SettingsBase|GetStart%20On%20Spawn)
            (Default|HandleTask (CallFunction|GetMainPlayerPawn _self) _self "NewEnumerator1" false)))))))

(fn ConstructionScript)

(fn IsTaskDone
  (Development|PrintString "Is Task Done function not yet implemented. Task will automaticaly stop.")
  (return true))

(fn GetTaskManager
  (bind _outactors (Actor|GetAllActorsOfClass "/Game/_Overseas/Development/Blueprints/Systems/Task_System/BP_Task_Manager.BP_Task_Manager_C"))
  (for _array_element _outactors
    (if (== (Variables|/Game/_Overseas/Development/Blueprints/Systems/Task_System/BP_Task_Manager.BP_Task_Manager_C|GetTask%20Manager%20ID _array_element) (Variables|SettingsBase|GetTask%20Manager%20ID))
      (return _array_element)))
  (return 0))

(fn OnRepTaskManager)