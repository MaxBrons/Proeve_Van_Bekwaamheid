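; BP_Task_AI_DisableCommunication is a task system task that completes when a communication rack reaches its correct frequency.
; On task start it binds to the rack's CorrectFrequencyReached event, and only the authority generates the target frequency.
; When the frequency is reached, it unbinds, sets TaskDone, stops the task for the current pawn, then resets the flag.
; IsTaskDone simply reports that flag.
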(event Custom|Frequency%20Reached
  (params (Frequency :type Float%20%28single-precision%29) (Communication%20Rack%20Reference :type BP%20Communication%20Rack%20Object%20Reference))
  (EventDispatchers|UnbindEventfromCorrectFrequencyReached Communication%20Rack%20Reference (delegate Custom|Frequency%20Reached))
  (Variables|Internal|SetTask%20Done true)
  (CallFunction|StopTask (Variables|Default|GetCurrent%20Pawn))
  (Variables|Internal|SetTask%20Done false))

(event EventBeginPlay
  (|CallParentFunction) ; This node is disabled and will not be called.\nDrag off pins to build functionality.
)

(event EventOnTaskStart
  (bind _communication_rack (Variables|Settings|GetCommunication%20Rack)
    (:then
      (EventDispatchers|BindEventtoCorrectFrequencyReached _communication_rack (delegate Custom|Frequency%20Reached))
      (Networking|SwitchHasAuthority
        (:Authority
          (Default|GenerateCorrectFrequency (Variables|Settings|GetCommunication%20Rack)))))
    (:else)))

(event EventOnTaskStop)

(fn ConstructionScript
  (|CallParentFunction))

(fn IsTaskDone
  (return (Variables|Internal|GetTask%20Done)))