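; AI task that, going by its name, disables a cannon through a set of electrical boxes.
; On start it sets each valid box's active component to inactive, resets the counter and binds to switch updates.
; Each all-switches-on update increments the counter, and reaching the box count marks the task done, stops it, then clears the flag.
; On stop it unbinds from every box and sets it active again.
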(event Custom|Switches%20Updated
  (params (All%20Switches%20On :type Boolean))
  (if All%20Switches%20On
    (bind _result (Math|Integer|IncrementInt (Variables|Internal|GetActivated%20Boxes%20Count))
      (:%20%20
        (if (== _result (Utilities|Array|Length (Variables|Settings|GetElectrical%20Boxes%20To%20Deactivate)))
          (Variables|Internal|SetTask%20Done true)
          (CallFunction|StopTask (Variables|Default|GetCurrent%20Pawn))
          (Variables|Internal|SetTask%20Done false))))))

(event EventBeginPlay
  (|CallParentFunction) ; This node is disabled and will not be called.\nDrag off pins to build functionality.
)

(event EventOnTaskStop
  (for _array_element (Variables|Settings|GetElectrical%20Boxes%20To%20Deactivate)
    (EventDispatchers|UnbindEventfromOnSwitchesUpdated _array_element (delegate Custom|Switches%20Updated))
    (Default|SetActive (Variables|/Game/_Overseas/Development/Blueprints/Assets/Ship/BP_ElectricalBox.BP_ElectricalBox_C|GetComp_Active _array_element) (Variables|Default|GetCurrent%20Pawn) true)))

(event EventOnTaskStart
  (for _array_element (Variables|Settings|GetElectrical%20Boxes%20To%20Deactivate)
    (Utilities|IsValid (Actor|GetComponentbyClass _array_element "/Game/_Overseas/Development/Blueprints/Components/Core/Comp_Active.Comp_Active_C")
      (:Is%20Valid
        (Default|SetActive (Actor|GetComponentbyClass _array_element "/Game/_Overseas/Development/Blueprints/Components/Core/Comp_Active.Comp_Active_C") (Variables|Default|GetCurrent%20Pawn) false)
        (Variables|Internal|SetActivated%20Boxes%20Count 0)
        (EventDispatchers|BindEventtoOnSwitchesUpdated _array_element (delegate Custom|Switches%20Updated))))))

(fn ConstructionScript
  (|CallParentFunction))

(fn IsTaskDone
  (return (Variables|Internal|GetTask%20Done)))