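; Server-driven AI task that disables doors in multiplayer, stopping immediately if only one player is listed.
; It locks either the last entered door or every door of a room holding exactly one player, retrying until one qualifies outside a short post-entry transition window.
; Multicast-style events disable each door and its linked counterpart on clients and server.
; Unlocking a bound door marks the task done and stops it.
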(event Custom|Door%20Entered
  (params (Pawn :type BP%20Pawn%20Base%20Object%20Reference) (Souce%20Actor :type Actor%20Object%20Reference))
  (bind _asbp_door (Utilities|Casting|CastToBP_Door Souce%20Actor))
  (Variables|Internal|SetDoor%20To%20Lock _asbp_door)
  (Variables|Internal|SetPlayer%20In%20Transition true)
  (Utilities|FlowControl|Delay 3.0)
  (Variables|Internal|SetPlayer%20In%20Transition false))

(event Custom|Multi_Lock%20Door
  (params (Door%20To%20Deactivate :type BP%20Door%20Object%20Reference))
  (EventDispatchers|BindEventtoOnDoorUnlocked Door%20To%20Deactivate (delegate Custom|Door%20Unlocked))
  (CallFunction|DeactivateDoor Door%20To%20Deactivate))

(event Custom|Door%20Unlocked
  (params (Door%20Reference :type BP%20Door%20Object%20Reference))
  (EventDispatchers|UnbindEventfromOnDoorUnlocked Door%20Reference (delegate Custom|Door%20Unlocked))
  (Variables|Internal|SetTask%20Done true)
  (CallFunction|StopTask (Variables|Default|GetCurrent%20Pawn))
  (Variables|Internal|SetTask%20Done false))

(event Custom|Door%20Sequence%20Unlocked
  (params (Door%20Reference :type BP%20Door%20Object%20Reference))
  (EventDispatchers|UnbindEventfromOnDoorUnlocked Door%20Reference (delegate Custom|Door%20Sequence%20Unlocked))
  (Variables|Internal|SetTask%20Done true)
  (CallFunction|StopTask (Variables|Default|GetCurrent%20Pawn))
  (Variables|Internal|SetTask%20Done false))

(event Custom|Multi_Lock%20Room
  (Networking|SwitchHasAuthority
    (:Authority
      (bind _current_locked_room (Variables|Internal|GetCurrent%20Locked%20Room)
        (:then
          (for _array_element (Variables|/Game/_Overseas/Development/Blueprints/Assets/Ship/BP_Room.BP_Room_C|GetDoors%20To%20Room _current_locked_room)
            (CallFunction|LockDoor _array_element)))
        (:else)))
    (:Remote
      (Utilities|FlowControl|Delay 0.1)))
  (for _array_element_2 (Variables|/Game/_Overseas/Development/Blueprints/Assets/Ship/BP_Room.BP_Room_C|GetDoors%20To%20Room _current_locked_room)
    (EventDispatchers|BindEventtoOnDoorUnlocked _array_element_2 (delegate Custom|Door%20Sequence%20Unlocked))
    (CallFunction|DeactivateDoor _array_element_2)))

(event EventBeginPlay
  (|CallParentFunction)
  (Networking|SwitchHasAuthority
    (:Authority
      (bind _outactors (Actor|GetAllActorsOfClass "/Game/_Overseas/Development/Blueprints/Assets/Ship/BP_Door.BP_Door_C"))
      (for _array_element _outactors
        (EventDispatchers|BindEventtoDoorEntered _array_element (delegate Custom|Door%20Entered))))))

(event EventOnTaskStart
  (bind _door_to_lock (Variables|Internal|GetDoor%20To%20Lock))
  (Networking|SwitchHasAuthority
    (:Authority
      (bind _asbp_game_mode_main (Utilities|Casting|CastToBP_GameMode_Main (Game|GetGameMode)))
      (if (== (Utilities|Map|Length (Variables|/Game/_Overseas/Development/Game/BP_GameMode_Main.BP_GameMode_Main_C|GetPlayer%20List _asbp_game_mode_main)) 1)
        (CallFunction|StopTask (Variables|Default|GetCurrent%20Pawn))
        (elif (not (Variables|Settings|GetLock%20Only%20Last%20Entered%20Door))
          (bind _room (CallFunction|GetNextRoom :!label _label))
          (Utilities|IsValid _room
            (:Is%20Valid
              (Variables|Internal|SetCurrent%20Locked%20Room _room)
              (CallFunction|MultiLockRoom))
            (:Is%20Not%20Valid
              (Utilities|FlowControl|Delay 2.0)
              (goto _label)))
          (else
            (Utilities|WaitforObjecttoValidate _door_to_lock 0.05
              (:Is%20Valid
                (CallFunction|LockDoor _door_to_lock)
                (CallFunction|MultiLockDoor _door_to_lock)))))))))

(fn ConstructionScript
  (|CallParentFunction))

(fn IsTaskDone
  (return (Variables|Internal|GetTask%20Done)))

(fn GetNextRoom
  (for _array_element (Variables|Settings|GetRooms)
    (if (and (== (Default|GetPlayerCountInsideRoom _array_element) 1) (not (Variables|Internal|GetPlayer%20In%20Transition)))
      (return _array_element)))
  (return 0))

(fn OnRepCurrentLockedDoor)

(fn LockDoor
  (params (Door :type BP%20Door%20Object%20Reference))
  (bind _self self)
  (bind _player_pawn (CallFunction|GetMainPlayerPawn _self))
  (Default|Activate _player_pawn (Variables|/Game/_Overseas/Development/Blueprints/Assets/Ship/BP_Door.BP_Door_C|GetComp_Active Door) false)
  (bind _door_to_transfer_to (Variables|/Game/_Overseas/Development/Blueprints/Assets/Ship/BP_Door.BP_Door_C|GetDoor%20To%20Transfer%20To Door)
    (:then
      (Default|Activate _player_pawn (Variables|/Game/_Overseas/Development/Blueprints/Assets/Ship/BP_Door.BP_Door_C|GetComp_Active _door_to_transfer_to) true))
    (:else)))

(fn DeactivateDoor
  (params (Door :type BP%20Door%20Object%20Reference))
  (bind _door_to_transfer_to (Variables|/Game/_Overseas/Development/Blueprints/Assets/Ship/BP_Door.BP_Door_C|GetDoor%20To%20Transfer%20To Door)
    (:then
      (Default|DisableDoor Door)
      (Default|DisableDoor _door_to_transfer_to))
    (:else)))