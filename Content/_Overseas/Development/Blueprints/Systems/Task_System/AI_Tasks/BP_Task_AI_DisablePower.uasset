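; BP_Task_AI_DisablePower is an AI task that completes when an electrical handle is turned off.
; On start it switches Comp_Active on or off for two actor lists using the current pawn, then binds to the handle's turned event.
; When the handle reports inactive, it briefly sets TaskDone, stops the task for that pawn, then resets the flag.
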(event Custom|Handle%20Turned
  (params (Active :type Boolean))
  (if (not Active)
    (Variables|Default|SetTask%20Done true)
    (CallFunction|StopTask (Variables|Default|GetCurrent%20Pawn))
    (Variables|Default|SetTask%20Done false)))

(event EventBeginPlay
  (|CallParentFunction) ; This node is disabled and will not be called.\nDrag off pins to build functionality.
)

(event EventOnTaskStart
  (for _array_element (Variables|Settings|GetActors%20To%20Activate)
    (Utilities|IsValid (Actor|GetComponentbyClass _array_element "/Game/_Overseas/Development/Blueprints/Components/Core/Comp_Active.Comp_Active_C")
      (:Is%20Valid
        (Default|SetActive (Actor|GetComponentbyClass _array_element "/Game/_Overseas/Development/Blueprints/Components/Core/Comp_Active.Comp_Active_C") (Variables|Default|GetCurrent%20Pawn) true))))
  (for _array_element_2 (Variables|Settings|GetActors%20To%20Deactivate)
    (Utilities|IsValid (Actor|GetComponentbyClass _array_element_2 "/Game/_Overseas/Development/Blueprints/Components/Core/Comp_Active.Comp_Active_C")
      (:Is%20Valid
        (Default|SetActive (Actor|GetComponentbyClass _array_element_2 "/Game/_Overseas/Development/Blueprints/Components/Core/Comp_Active.Comp_Active_C") (Variables|Default|GetCurrent%20Pawn) false))))
  (bind _electrical_handle (Variables|Settings|GetElectrical%20Handle)
    (:then
      (EventDispatchers|BindEventtoHandleTurned _electrical_handle (delegate Custom|Handle%20Turned)))
    (:else)))

(fn ConstructionScript
  (|CallParentFunction))

(fn IsTaskDone
  (return (Variables|Default|GetTask%20Done)))