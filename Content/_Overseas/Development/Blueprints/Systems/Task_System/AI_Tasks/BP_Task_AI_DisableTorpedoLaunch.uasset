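; BP_Task_AI_DisableTorpedoLaunch is an AI task, named for disabling a torpedo launch, that completes once every wheel in WheelsToTurn is active.
; On start it binds to active-state changes on each wheel's Comp_Active, and unbinds on stop.
; Each change triggers IsTaskDone, which skips wheels without that component, and stops the task for CurrentPawn when all pass.
; Completion is event-driven, with no check at task start.
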(event Custom|Active%20State%20Changed
  (params (Pawn :type BP%20Pawn%20Base%20Object%20Reference) (Comp%20Active :type Comp%20Active%20Object%20Reference) (New%20Active :type Boolean))
  (if (CallFunction|IsTaskDone)
    (CallFunction|StopTask (Variables|Default|GetCurrent%20Pawn))))

(event EventBeginPlay
  (|CallParentFunction) ; This node is disabled and will not be called.\nDrag off pins to build functionality.
)

(event EventOnTaskStart
  (for _array_element (Variables|Settings|GetWheels%20To%20Turn)
    (Utilities|IsValid (Actor|GetComponentbyClass _array_element "/Game/_Overseas/Development/Blueprints/Components/Core/Comp_Active.Comp_Active_C")
      (:Is%20Valid
        (EventDispatchers|BindEventtoActiveStateChanged (Actor|GetComponentbyClass _array_element "/Game/_Overseas/Development/Blueprints/Components/Core/Comp_Active.Comp_Active_C") (delegate Custom|Active%20State%20Changed))))))

(event EventOnTaskStop
  (for _array_element (Variables|Settings|GetWheels%20To%20Turn)
    (Utilities|IsValid (Actor|GetComponentbyClass _array_element "/Game/_Overseas/Development/Blueprints/Components/Core/Comp_Active.Comp_Active_C")
      (:Is%20Valid
        (EventDispatchers|UnbindEventfromActiveStateChanged (Actor|GetComponentbyClass _array_element "/Game/_Overseas/Development/Blueprints/Components/Core/Comp_Active.Comp_Active_C") (delegate Custom|Active%20State%20Changed))))))

(fn ConstructionScript
  (|CallParentFunction))

(fn IsTaskDone
  (for _array_element (Variables|Settings|GetWheels%20To%20Turn)
    (Utilities|IsValid (Actor|GetComponentbyClass _array_element "/Game/_Overseas/Development/Blueprints/Components/Core/Comp_Active.Comp_Active_C")
      (:Is%20Valid
        (if (not (Default|IsActive (Actor|GetComponentbyClass _array_element "/Game/_Overseas/Development/Blueprints/Components/Core/Comp_Active.Comp_Active_C")))
          (return false)))))
  (return true))