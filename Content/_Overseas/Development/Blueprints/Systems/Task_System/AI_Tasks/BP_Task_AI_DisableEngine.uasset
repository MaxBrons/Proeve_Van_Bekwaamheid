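; AI task that knocks out the engine and deactivates the steering wheel for the current pawn.
; On start, the authority randomly picks either disabling through the engine manager or through the engine thermal system, applied via a multicast-named event.
; The matching engine-restarted or thermal-threshold callback unbinds itself, briefly flags the task done while stopping it, then reactivates the wheel.
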(event Custom|Multi_Disable%20Engine
  (params (Set :type Boolean))
  (if Set
    (bind _engine_manager (Variables|Settings|GetEngine%20Manager)
      (:then
        (Default|SetEngineEnabled _engine_manager false)
        (EventDispatchers|BindEventtoOnEngineRestarted _engine_manager (delegate Custom|Engine%20Restarted)))
      (:else))
    (else
      (bind _engine_thermal (Variables|Settings|GetEngine%20Thermal)
        (:then
          (Default|DisableEngine _engine_thermal)
          (EventDispatchers|BindEventtoThermalThresholdReached _engine_thermal (delegate Custom|Thermal%20Reached)))
        (:else)))))

(event Custom|Thermal%20Reached
  (params (Widget%20Reference :type WB%20Widget%20Engine%20Thermal%20Object%20Reference))
  (EventDispatchers|UnbindEventfromThermalThresholdReached Widget%20Reference (delegate Custom|Thermal%20Reached))
  (Variables|Internal|SetTask%20Done true)
  (CallFunction|StopTask (Variables|Default|GetCurrent%20Pawn))
  (Variables|Internal|SetTask%20Done false)
  (bind _steering_wheel (Variables|Settings|GetSteering%20Wheel)
    (:then
      (Default|SetActive (Variables|/Game/_Overseas/Development/Blueprints/Assets/Ship/BP_SteeringWheel.BP_SteeringWheel_C|GetComp_Active _steering_wheel) (Variables|Default|GetCurrent%20Pawn) true))
    (:else)))

(event Custom|Engine%20Restarted
  (params (Manager%20Engine%20Reference :type BP%20Manager%20Engine%20Object%20Reference))
  (EventDispatchers|UnbindEventfromOnEngineRestarted Manager%20Engine%20Reference (delegate Custom|Engine%20Restarted))
  (Variables|Internal|SetTask%20Done true)
  (CallFunction|StopTask (Variables|Default|GetCurrent%20Pawn))
  (Variables|Internal|SetTask%20Done false)
  (bind _steering_wheel (Variables|Settings|GetSteering%20Wheel)
    (:then
      (Default|SetActive (Variables|/Game/_Overseas/Development/Blueprints/Assets/Ship/BP_SteeringWheel.BP_SteeringWheel_C|GetComp_Active _steering_wheel) (Variables|Default|GetCurrent%20Pawn) true))
    (:else)))

(event EventBeginPlay
  (|CallParentFunction) ; This node is disabled and will not be called.\nDrag off pins to build functionality.
)

(event EventOnTaskStart
  (bind _steering_wheel (Variables|Settings|GetSteering%20Wheel)
    (:then
      (Default|SetActive (Variables|/Game/_Overseas/Development/Blueprints/Assets/Ship/BP_SteeringWheel.BP_SteeringWheel_C|GetComp_Active _steering_wheel) (Variables|Default|GetCurrent%20Pawn) false)
      (Networking|SwitchHasAuthority
        (:Authority
          (CallFunction|MultiDisableEngine (Math|Random|RandomBool)))))
    (:else)))

(fn ConstructionScript
  (|CallParentFunction))

(fn IsTaskDone
  (return (Variables|Internal|GetTask%20Done)))