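; Enemy AI that cycles through random BP_Task_AI tasks found in the level, with random breaks between them.
; On authority it picks a task different from the last, retries later if its state rules it out, and hands it to the pawn's HandleTask.
; Task completion starts the next cycle, with a gated retriggerable delay as timeout fallback.
; Remote instances only start an already valid current task once after BeginPlay.
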(event Custom|On%20Task%20Done
  (params (Task%20Reference :type BP%20Task%20Object%20Reference) (Task%20Name :type Name) (Task%20ID :type Integer) (Pawn :type BP%20Pawn%20Base%20Object%20Reference))
  (EventDispatchers|UnbindEventfromOnTaskDone Task%20Reference (delegate Custom|On%20Task%20Done))
  (Utilities|FlowControl|Sequence
    (:then_0
      (goto _label_2 Close))
    (:then_1
      (Utilities|FlowControl|Delay (Math|Random|RandomFloatinRange (Variables|Settings|GetMin%20Break%20Time) (Variables|Settings|GetMax%20Break%20Time)))
      (bind _output_get (Variables|Internal|SetCurrent%20AI%20Task (CallFunction|GetRandomAITask) :!label _label))
      (if (Utilities|Enum|NotEqual(Enum) (Variables|/Game/_Overseas/Development/Blueprints/Systems/Task_System/BP_Task.BP_Task_C|GetTask%20State _output_get) "NewEnumerator2")
        (EventDispatchers|BindEventtoOnTaskDone (Variables|Internal|GetCurrent%20AI%20Task) (delegate Custom|On%20Task%20Done))
        (Default|HandleTask (CallFunction|GetMainPlayerPawn self) _output_get "NewEnumerator1" false)
        (Utilities|FlowControl|Sequence
          (:then_0
            (goto _label_2 Open))
          (:then_1
            (Utilities|FlowControl|RetriggerableDelay (Variables|Settings|GetMin%20Break%20Time))
            (Utilities|FlowControl|Gate true :!label _label_2
              (:Exit
                (CallFunction|OnTaskDone (Variables|Internal|GetCurrent%20AI%20Task) "None")))))
        (else
          (Utilities|FlowControl|Delay 5.0)
          (goto _label))))))

(event EventBeginPlay
  (Utilities|FlowControl|Delay 1.0)
  (bind _outactors (Actor|GetAllActorsOfClass "/Game/_Overseas/Development/Blueprints/Systems/Task_System/BP_Task_AI.BP_Task_AI_C"))
  (bind _output_get (Variables|Internal|SetAI%20Tasks _outactors))
  (if (> (Utilities|Array|Length _output_get) 0)
    (Networking|SwitchHasAuthority
      (:Authority
        (Utilities|FlowControl|Delay (Math|Random|RandomFloatinRange (Variables|Settings|GetMin%20Break%20Time) (Variables|Settings|GetMax%20Break%20Time)))
        (bind _output_get_2 (Variables|Internal|SetCurrent%20AI%20Task (CallFunction|GetRandomAITask) :!label _label))
        (if (Utilities|Enum|NotEqual(Enum) (Variables|/Game/_Overseas/Development/Blueprints/Systems/Task_System/BP_Task.BP_Task_C|GetTask%20State _output_get_2) "NewEnumerator2")
          (EventDispatchers|BindEventtoOnTaskDone (Variables|Internal|GetCurrent%20AI%20Task) (delegate Custom|On%20Task%20Done))
          (Default|HandleTask (CallFunction|GetMainPlayerPawn self) _output_get_2 "NewEnumerator1" false)
          (Utilities|FlowControl|Sequence
            (:then_0
              (goto _label_2 Open))
            (:then_1
              (Utilities|FlowControl|RetriggerableDelay (Variables|Settings|GetMin%20Break%20Time))
              (Utilities|FlowControl|Gate true :!label _label_2
                (:Exit
                  (CallFunction|OnTaskDone (Variables|Internal|GetCurrent%20AI%20Task) "None")))))
          (else
            (Utilities|FlowControl|Delay 5.0)
            (goto _label))))
      (:Remote
        (bind _current_ai_task (Variables|Internal|GetCurrent%20AI%20Task)
          (:then
            (Default|StartTask _current_ai_task (CallFunction|GetMainPlayerPawn self)))
          (:else))))))

(fn ConstructionScript)

(fn GetRandomAITask
  (bind _ai_tasks (Variables|Internal|GetAI%20Tasks))
  (bind _returnvalue (Utilities|Array|Length _ai_tasks))
  (if (<= _returnvalue 1)
    (return (Utilities|Array|Get(acopy) (Variables|Internal|GetAI%20Tasks)))
    (else
      (bind _output_get (LocalVariables|SetTask (Utilities|Array|Get(acopy) _ai_tasks (Math|Random|RandomInteger _returnvalue)) :!label _label))
      (if (!= _output_get (Variables|Internal|GetCurrent%20AI%20Task))
        (return _output_get)
        (else
          (goto _label))))))