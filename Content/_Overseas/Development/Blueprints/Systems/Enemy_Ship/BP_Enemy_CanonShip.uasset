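; BP_Enemy_CanonShip is an enemy cannon ship Blueprint that tracks the ship's health.
; On BeginPlay it runs the parent logic, then sets Health from StartHealt.
; DoDamage removes one point per call, prints the remaining Health and returns whether it has reached zero or below, with no death handling of its own.
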(event EventBeginPlay
  (|CallParentFunction)
  (Variables|Default|SetHealth (Variables|Default|GetStartHealt)))

(event Collision|EventActorBeginOverlap
  (params (OtherActor :type Actor%20Object%20Reference)))

(event EventTick
  (params (DeltaSeconds :type Float%20%28single-precision%29)))

(fn ConstructionScript
  (|CallParentFunction))

(fn DoDamage
  (bind _output_get (Variables|Default|SetHealth (- (Variables|Default|GetHealth) 1)))
  (Development|PrintString (Utilities|String|ToString(Integer) _output_get))
  (return (<= _output_get 0)))