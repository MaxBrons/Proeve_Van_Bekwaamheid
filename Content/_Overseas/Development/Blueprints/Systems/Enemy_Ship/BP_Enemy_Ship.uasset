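; BP_Enemy_Ship is the enemy ship Blueprint, which runs an endless chain of randomly chosen actions.
; On BeginPlay it gathers its Comp_Enemy_Ship_Action components and starts one via StartActionRPC.
; Each action's executed callback unbinds itself and starts the next random pick, whose index range excludes the last component when several exist.
; ShipSetup stores the ship's course and type, and prints the type.
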(event Custom|Execute%20Ship%20Action
  (params (Ship%20Action%20To%20Execute :type Comp%20Enemy%20Ship%20Action%20Object%20Reference))
  (Utilities|IsValid Ship%20Action%20To%20Execute
    (:Is%20Valid
      (bind _output_get (Variables|Internal|SetCurrent%20Ship%20Action Ship%20Action%20To%20Execute))
      (EventDispatchers|BindEventtoOnActionExecuted _output_get (delegate Custom|On%20Action%20Executed))
      (Default|StartActionRPC _output_get))))

(event Custom|On%20Action%20Executed
  (EventDispatchers|UnbindEventfromOnActionExecuted (stale Custom|Execute%20Ship%20Action _output_get) (delegate Custom|On%20Action%20Executed))
  (CallFunction|ExecuteShipAction (CallFunction|GetRandomShipAction)))

(event Custom|ShipSetup
  (params (CourseShipIsAt :type Float%20%28single-precision%29) (ShipType :type E_Enemy_Type%20Enum :default "NewEnumerator0"))
  (Variables|Default|SetCourse CourseShipIsAt)
  (bind _output_get (Variables|Default|SetShipType ShipType))
  (Development|PrintString (Utilities|String|EnumtoString _output_get)))

(event EventBeginPlay
  (bind _output_get (Variables|Internal|SetShip%20Actions (Actor|GetComponentsByClass "/Game/_Overseas/Development/Blueprints/Systems/Enemy_Ship/Comp_Enemy_Ship_Action.Comp_Enemy_Ship_Action_C")))
  (if (> (Utilities|Array|Length _output_get) 0)
    (CallFunction|ExecuteShipAction (CallFunction|GetRandomShipAction))))

(fn ConstructionScript)

(fn GetRandomShipAction
  (bind _ship_actions (Variables|Internal|GetShip%20Actions))
  (return (Utilities|Array|Get(acopy) _ship_actions (Math|Random|RandomInteger (- (Utilities|Array|Length _ship_actions) 1)))))