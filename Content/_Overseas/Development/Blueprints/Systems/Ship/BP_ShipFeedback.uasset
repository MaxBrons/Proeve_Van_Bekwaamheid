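; Ship feedback Blueprint meant to react to ship hits, currently mostly disconnected.
; On BeginPlay it finds the Sound_Impact actor in the level and stops its audio.
; The setup and hit events are empty, leaving unreachable logic that would gather alarm lights, bind to the ship's hit event, and play a delayed impact sound and camera shake.
; The Current Course replication handler is also empty.
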(event Custom|SetupFeedbackOnHit
  (params (Ship :type BP%20Ship%20Object%20Reference)))

(event Custom|ShipHit)

(event EventBeginPlay
  (bind _returnvalue (Actor|GetActorOfClass "/Game/_Overseas/Development/Audio/Ship/Sound_Impact.Sound_Impact_C"))
  (bind _output_get (Variables|Internal|SetImpactSound _returnvalue))
  (Audio|Components|Audio|Stop (Variables|/Script/Engine.AmbientSound|GetAudioComponent _output_get)))

(event Collision|EventActorBeginOverlap
  (params (OtherActor :type Actor%20Object%20Reference)))

(event EventTick
  (params (DeltaSeconds :type Float%20%28single-precision%29)))

(fn ConstructionScript)

(fn OnRepCurrentCourse)