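; Interaction component that lets a player focus on its owning actor, moving camera and input from the pawn to that actor.
; On interaction, the owning side switches input through BP_PlayerController_Main, blends the view target to the actor and hides the pawn.
; Unfocus switches input and blends back, then waits out the blend before showing the pawn, firing OnUnfocus and clearing the stored pawn.
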(event Custom|Unfocus
  ;[1 1 1] Unfocus the player from the focus pawn, back to the previous pawn
  (bind _interacting_pawn (Variables|Internal|GetInteracting%20Pawn)
    (:then
      (Utilities|IsReplicatedOwner _interacting_pawn
        (:Owner
          (Variables|Internal|GetInteracting%20Pawn
            (:then
              (bind _asbp_player_controller_main (Utilities|Casting|CastToBP_PlayerController_Main (Pawn|GetController (Variables|Internal|GetInteracting%20Pawn))))
              (Default|SwitchInput _asbp_player_controller_main (Variables|Internal|GetInteracting%20Pawn) (Components|GetOwner) false)
              (Game|Player|SetViewTargetwithBlend _asbp_player_controller_main (Variables|Internal|GetInteracting%20Pawn) (Variables|Settings|GetFocus%20Time) (Variables|Settings|GetFocus%20Motion%20Type) 0.0 false)
              (Utilities|FlowControl|Delay (Variables|Settings|GetFocus%20Time))
              (Rendering|SetVisibility (Variables|/Script/Engine.Actor|GetRootComponent (Variables|Internal|GetInteracting%20Pawn)) true true)
              (Default|CallOnUnfocus)
              (Variables|Internal|SetInteracting%20Pawn 0))
            (:else)))))
    (:else)))

(event Custom|Focus
  (params (Pawn :type BP%20Pawn%20Base%20Object%20Reference))
  ;[1 1 1] Spawn in the focus pawn in when the player starts the focus event. Also switch to the new focus pawn.
  (Utilities|IsReplicatedOwner Pawn
    (:Owner
      (Variables|Internal|GetInteracting%20Pawn
        (:then)
        (:else
          (bind _output_get (Variables|Internal|SetInteracting%20Pawn Pawn))
          (Utilities|IsValid _output_get
            (:Is%20Valid
              (bind _asbp_player_controller_main (Utilities|Casting|CastToBP_PlayerController_Main (Pawn|GetController (Variables|Internal|GetInteracting%20Pawn))))
              (Default|SwitchInput _asbp_player_controller_main (Variables|Internal|GetInteracting%20Pawn) (Components|GetOwner) true)
              (Game|Player|SetViewTargetwithBlend _asbp_player_controller_main (Components|GetOwner) (Variables|Settings|GetFocus%20Time) (Variables|Settings|GetFocus%20Motion%20Type) 0.0 false)
              (Rendering|SetVisibility (Variables|/Script/Engine.Actor|GetRootComponent (Variables|Internal|GetInteracting%20Pawn)) false true))))))))

(event EventInteractionPressed
  (params (Pawn :type BP%20Pawn%20Base%20Object%20Reference) (Source%20Actor :type Actor%20Object%20Reference) (Hit%20Location :type Vector :default "0, 0, 0") (Hit%20Distance :type Float%20%28single-precision%29) (Hit%20Component :type Actor%20Component%20Object%20Reference))
  ;[1 1 1] Focus the player when the player has started interacting with this interaction component
  (|CallParentFunction Pawn Source%20Actor Hit%20Location Hit%20Distance Hit%20Component)
  (Utilities|IsReplicatedOwner Pawn
    (:Owner
      (CallFunction|Focus Pawn))))