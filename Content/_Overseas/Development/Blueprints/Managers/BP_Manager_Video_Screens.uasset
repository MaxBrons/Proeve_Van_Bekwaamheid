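; Manager actor that switches groups of video screen actors on or off through their Comp_Active components.
; Shortly after BeginPlay it gathers all actors of the configured classes and applies the default active state.
; SetScreensActive sets every component to one state, passing the main player pawn.
; SetScreensActiveRandom runs only on authority, giving each screen a weighted random state through the main player pawn's Activate call.
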(event Custom|Set%20Screens%20Active
  (params (Set :type Boolean))
  (for _array_element (Variables|Internal|GetActors%20To%20Control)
    (Utilities|IsValid (Actor|GetComponentbyClass _array_element "/Game/_Overseas/Development/Blueprints/Components/Core/Comp_Active.Comp_Active_C")
      (:Is%20Valid
        (Default|SetActive (Actor|GetComponentbyClass _array_element "/Game/_Overseas/Development/Blueprints/Components/Core/Comp_Active.Comp_Active_C") (CallFunction|GetMainPlayerPawn self) Set)))))

(event Custom|Set%20Screens%20Active%20Random
  (Networking|SwitchHasAuthority
    (:Authority
      (for _array_element (Variables|Internal|GetActors%20To%20Control)
        (Utilities|IsValid (Actor|GetComponentbyClass _array_element "/Game/_Overseas/Development/Blueprints/Components/Core/Comp_Active.Comp_Active_C")
          (:Is%20Valid
            (bind _output_get (Variables|Settings|SetRandom%20Bool (Math|Random|RandomBoolwithWeight 0.33)))
            (Default|Activate (CallFunction|GetMainPlayerPawn self) (Actor|GetComponentbyClass _array_element "/Game/_Overseas/Development/Blueprints/Components/Core/Comp_Active.Comp_Active_C") _output_get)))))))

(event EventBeginPlay
  (Utilities|FlowControl|Delay 0.2)
  (for _array_element (Variables|Settings|GetActor%20Classes%20To%20Control)
    (bind _outactors (Actor|GetAllActorsOfClass _array_element))
    (Utilities|Array|AppendArray (Variables|Internal|GetActors%20To%20Control) _outactors))
  (CallFunction|SetScreensActive (Variables|Settings|GetDefault%20Active%20State)))

(fn ConstructionScript)