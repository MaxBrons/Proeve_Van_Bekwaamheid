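; Manager actor that coordinates torpedo loading between a torpedo rack, an in hole and an out hole, destroying itself at BeginPlay if any is missing.
; It listens to the in hole's update event and, when that hole is occupied and closed, transfers the torpedo to the out hole.
; Each update also enables rack interaction only while the in hole is open and both holes are empty.
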(event Custom|On%20Hole%20In%20Updated
  (params (Opened :type Boolean) (Occupied :type Boolean))
  (if (and Occupied (not Opened))
    (CallFunction|TransferTorpedo false))
  (CallFunction|UpdateContent))

(event Custom|Transfer%20Torpedo
  (params (Loading%20In :type Boolean))
  (bind _torpedo_hole_in (Variables|Settings|GetTorpedo%20Hole%20In)
    (:then
      (Default|SetTorpedoActive _torpedo_hole_in Loading%20In)
      (bind _torpedo_hole_out (Variables|Settings|GetTorpedo%20Hole%20Out)
        (:then
          (Default|SetTorpedoVisible _torpedo_hole_out (not Loading%20In)))
        (:else)))
    (:else)))

(event EventBeginPlay
  (Variables|Settings|GetTorpedo%20Hole%20Out
    (:then
      (Variables|Settings|GetTorpedo%20Rack
        (:then
          (bind _torpedo_hole_in (Variables|Settings|GetTorpedo%20Hole%20In)
            (:then
              (EventDispatchers|BindEventtoTorpedoHoleUpdated _torpedo_hole_in (delegate Custom|On%20Hole%20In%20Updated))
              (CallFunction|UpdateContent))
            (:else
              (Actor|DestroyActor :!label _label))))
        (:else
          (goto _label))))
    (:else
      (goto _label))))

(event EventUpdateContent
  (bind _torpedo_rack (Variables|Settings|GetTorpedo%20Rack)
    (:then
      (Default|SetInteractionEnabled (Variables|/Game/_Overseas/Development/Blueprints/Assets/Ship/Torpedo/BP_Torpedo_Rack.BP_Torpedo_Rack_C|GetComp_Focus _torpedo_rack) (CallFunction|AllowedtoLoadTorpedoin)))
    (:else)))

(fn ConstructionScript)

(fn AllowedtoLoadTorpedoin
  (bind _torpedo_hole_in (Variables|Settings|GetTorpedo%20Hole%20In))
  (return (Math|Boolean|ANDBoolean (Default|IsOpened _torpedo_hole_in) (not (Default|IsOccupied _torpedo_hole_in)) (not (Default|IsOccupied (Variables|Settings|GetTorpedo%20Hole%20Out))))))