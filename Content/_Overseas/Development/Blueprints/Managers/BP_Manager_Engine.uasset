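; BP_Manager_Engine is a manager that restarts the engine once every restart screen reports a restart within a short time window.
; It binds to each RestartScreens entry and counts their restart events.
; An incomplete count opens a Gate, and a two-second Delay then resets it.
; A full count closes the Gate, resets the counter, enables the engine on all screens and calls OnEngineRestarted.
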(event Custom|Restarted
  (params (Engine%20Restart%20Reference :type WB%20Widget%20Engine%20Restart%20Object%20Reference))
  (bind _result (Math|Integer|IncrementInt (Variables|Internal|GetAmount%20Restarted))
    (:%20%20
      (if (== _result (Utilities|Array|Length (Variables|Settings|GetRestart%20Screens)))
        (Utilities|FlowControl|Sequence
          (:then_0
            (goto _label Close))
          (:then_1
            (Variables|Internal|SetAmount%20Restarted 0)
            (CallFunction|SetEngineEnabled true)
            (Default|CallOnEngineRestarted self)))
        (else
          (Utilities|FlowControl|Sequence
            (:then_0
              (goto _label Open))
            (:then_1
              (Utilities|FlowControl|Delay 2.0)
              (Utilities|FlowControl|Gate true :!label _label
                (:Exit
                  (Variables|Internal|SetAmount%20Restarted 0))))))))))

(event Custom|Set%20Engine%20Enabled
  (params (Enabled :type Boolean))
  (for _array_element (Variables|Settings|GetRestart%20Screens)
    (Default|SetEngineEnabled _array_element Enabled)))

(event EventBeginPlay
  (for _array_element (Variables|Settings|GetRestart%20Screens)
    (EventDispatchers|BindEventtoEngineRestarted _array_element (delegate Custom|Restarted))))

(fn ConstructionScript)