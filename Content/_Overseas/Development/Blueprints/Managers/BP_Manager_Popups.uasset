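; Manager actor for on-screen popups that fronts a single WB_Screen_Popups widget.
; On BeginPlay it creates the widget and adds it to the main player's BP_Pawn_Screen as the "Popups" HUD layer.
; Its events forward screen open and close, popup add and remove, and task step updates to that widget.
; Only add and remove check that the widget is valid first.
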(event Custom|Close%20Task%20Screen
  (Default|CloseScreen (Variables|Internal|GetPopup%20Screen)))

(event Custom|Open%20Task%20Screen
  (Default|OpenScreen (Variables|Internal|GetPopup%20Screen)))

(event Custom|Remove%20Popup
  (params (Popup%20Reference :type WB%20Screen%20Popups%20Popup%20Object%20Reference))
  (bind _popup_screen (Variables|Internal|GetPopup%20Screen)
    (:then
      (Default|RemovePopup _popup_screen Popup%20Reference))
    (:else)))

(event Custom|Add%20Popup
  (params (Popup%20Reference :type WB%20Screen%20Popups%20Popup%20Object%20Reference))
  (bind _popup_screen (Variables|Internal|GetPopup%20Screen)
    (:then
      (Default|AddPopup _popup_screen Popup%20Reference))
    (:else)))

(event Custom|Update%20Popup%20Task
  (params (Popup :type WB%20Screen%20Popups%20Popup%20Object%20Reference) (Task%20Step%20Index :type Integer))
  (Default|UpdateTaskStep (Variables|Internal|GetPopup%20Screen) Popup Task%20Step%20Index))

(event EventBeginPlay
  (bind _returnvalue (UserInterface|CreateWidget "/Game/_Overseas/Development/Blueprints/Widgets/HUD/Popups/WB_Screen_Popups.WB_Screen_Popups_C" 0 0 0))
  (Variables|Internal|SetPopup%20Screen _returnvalue)
  (bind _asbp_pawn_screen (Utilities|Casting|CastToBP_Pawn_Screen (CallFunction|GetMainPlayerPawn self)))
  (Default|AddWidgettoViewport _asbp_pawn_screen "Popups" (Variables|Internal|GetPopup%20Screen) 1))

(fn ConstructionScript)