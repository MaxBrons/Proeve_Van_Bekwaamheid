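; Manager for the ship's torpedo launch sequence, built around turning several launch keys within a time margin.
; Key turns count only while the tube is closed and occupied; a Gate and Delay time the window, then broadcast the result or reset.
; CanLaunch exposes the all-keys-turned state.
; BeginPlay and launch events are empty: setup, key binding, replicated firing, enemy hit and sound logic sit disconnected.
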(event Custom|Torpedo%20Launched)

(event Custom|Multi_Launch%20Torpedo
  (params (Right :type Boolean)))

(event Custom|On%20Pressed
  (params (Pawn :type BP%20Pawn%20Base%20Object%20Reference) (Souce%20Actor :type Actor%20Object%20Reference) (Hit%20Location :type Vector) (Hit%20Distance :type Float%20%28single-precision%29) (Hit%20Component :type Actor%20Component%20Object%20Reference))
  (bind _torpedo_tube (Variables|Settings|GetTorpedo%20Tube)
    (:then
      (if (and (Default|IsClosed _torpedo_tube) (Default|IsOccupied _torpedo_tube))
        (Variables|Settings|GetLaunch%20Button
          (:then)
          (:else))))
    (:else)))

(event Custom|On%20Key%20Turned
  (params (Key%20Reference :type BP%20Torpedo%20Launch%20Key%20Object%20Reference))
  (if (not (Utilities|Array|ContainsItem (Variables|Internal|GetTurned%20Keys) Key%20Reference))
    (if (CallFunction|CanFireTorpedo)
      (Math|Integer|IncrementInt (Variables|Internal|GetKeys%20Turned)
        (:%20%20
          (Utilities|Array|Add (Variables|Internal|GetTurned%20Keys) Key%20Reference)
          (if (== (Variables|Internal|GetKeys%20Turned) (Utilities|Array|Length (Variables|Settings|GetKeys%20To%20Turn)))
            (Utilities|FlowControl|Sequence
              (:then_0
                _)
              (:then_1
                (goto _label Close)))
            (else
              (Utilities|FlowControl|Sequence
                (:then_0
                  (goto _label Open))
                (:then_1
                  (Utilities|FlowControl|Delay (Variables|Internal|GetKeys%20Turned%20Time%20Margin))))))
          (Utilities|FlowControl|Gate true :!label _label
            (:Exit
              (if (== (Variables|Internal|GetKeys%20Turned) (Utilities|Array|Length (Variables|Settings|GetKeys%20To%20Turn)))
                (bind _launch_button (Variables|Settings|GetLaunch%20Button)
                  (:then)
                  (:else
                    _)))
              (Variables|Internal|SetAll%20Keys%20Turned (== (Variables|Internal|GetKeys%20Turned) (Utilities|Array|Length (Variables|Settings|GetKeys%20To%20Turn))))
              (Default|CallLaunchKeysTurned (== (Variables|Internal|GetKeys%20Turned) (Utilities|Array|Length (Variables|Settings|GetKeys%20To%20Turn))))
              (Variables|Internal|SetKeys%20Turned 0)
              (Utilities|Array|Clear (Variables|Internal|GetTurned%20Keys)))))))))

(event Custom|Launch%20Torpedo
  (params (Right :type Boolean)))

(event Custom|Server_Launch%20Torpedo
  (params (Right :type Boolean)))

(event EventBeginPlay)

(fn ConstructionScript)

(fn OnRepKeysTurned)

(fn CanFireTorpedo
  (bind _torpedo_tube (Variables|Settings|GetTorpedo%20Tube)
    (:then
      (return (and (Default|IsClosed _torpedo_tube) (Default|IsOccupied _torpedo_tube))))
    (:else)))

(fn CanLaunch
  (return (Variables|Internal|GetAll%20Keys%20Turned)))