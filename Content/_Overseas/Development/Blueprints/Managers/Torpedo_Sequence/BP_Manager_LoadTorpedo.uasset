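; Manager for a torpedo loading sequence between a rack, an in hole and an out hole, currently non-functional.
; All its events are empty, and the logic for validation, occupancy binding, interaction updates and transfer is left disconnected.
; That orphaned logic would destroy the actor on missing references and gate interaction through AllowedToLoadTorpedoIn.
; That function requires the in hole open and both holes unoccupied.
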(event Custom|On%20Hole%20In%20Updated)

(event Custom|Transfer%20Torpedo
  (params (Loading%20In :type Boolean)))

(event EventBeginPlay)

(event EventUpdateContent)

(fn ConstructionScript)

(fn AllowedtoLoadTorpedoin
  (bind _torpedo_hole_in (Variables|Settings|GetTorpedo%20Hole%20In))
  (return (Math|Boolean|ANDBoolean (Default|IsOpened _torpedo_hole_in) (not (Default|IsOccupied _torpedo_hole_in)) (not (Default|IsOccupied (Variables|Settings|GetTorpedo%20Hole%20Out))))))