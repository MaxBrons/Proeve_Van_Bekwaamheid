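; Manager that runs the left and right torpedo loading and launch sequences independently, looping each after launch.
; Each step enables an interactable through Comp_Active, awaits its event, then broadcasts a step index per side.
; Steps run through loading doors, rack transfers, authority-only tube loading, keys, and launch button.
; All keys on a side must be turned within a short gate-and-delay window, otherwise they re-arm for retry.
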(event Custom|Torpedo%20Door%20Right%20Opened
  ;[1 1 1] Wait for the player to open the left torpedo door.
  (EventDispatchers|UnbindEventfromTorpedoDoorOpened (stale Custom|Reset%20Right _rightloadingtubein) (delegate Custom|Torpedo%20Door%20Right%20Opened))
  (Default|SetInteractionEnabled (Variables|/Game/_Overseas/Development/Blueprints/Assets/Ship/Munition/BP_Torpedo_Hole_In.BP_Torpedo_Hole_In_C|GetComp_Interaction (stale Custom|Reset%20Right _rightloadingtubein)) false)
  (Default|CallOnSequenceUpdate 1 "NewEnumerator1")
  (CallFunction|WaitTorpedoRightTransfered))

(event Custom|Wait%20Torpedo%20Loaded%20On%20Right%20Rack
  ;[1 1 1] Torpedo loading Rack
  (bind _righttorpedoloadingrack (Variables|Settings|TorpedoRight|GetRightTorpedoLoadingRack)
    (:then
      (Variables|/Game/_Overseas/Development/Blueprints/Assets/Ship/Torpedo/BP_LoadingRack.BP_LoadingRack_C|GetCurrent%20Torpedo _righttorpedoloadingrack
        (:then
          (Default|CallOnSequenceUpdate 5 "NewEnumerator1")
          (Variables|/Game/_Overseas/Development/Blueprints/Assets/Ship/Torpedo/BP_LoadingRack.BP_LoadingRack_C|SetCurrent%20Torpedo (Variables|Settings|TorpedoRight|GetRightTorpedoLoadingRack) 0)
          (CallFunction|WaitTorpedoTubeRightOccupied))
        (:else
          (EventDispatchers|BindEventtoTorpedoLoadedonRack _righttorpedoloadingrack (delegate Custom|Torpedo%20Loaded%20On%20Rack%20Right)))))
    (:else)))

(event Custom|Multi_CloseTubeDoorRight
  ;[1 1 1] Wait fort the player to close the left torpedo tube door.
  (if (not (Default|IsClosed (stale Custom|Wait%20Torpedo%20Tube%20Right%20Occupied _righttorpedotube)))
    (EventDispatchers|BindEventtoTubeDoorClosed (stale Custom|Wait%20Torpedo%20Tube%20Right%20Occupied _righttorpedotube) (delegate Custom|Torpedo%20Tube%20Door%20Right%20Closed))
    (Default|SetActive (Variables|/Game/_Overseas/Development/Blueprints/Assets/Ship/Torpedo/BP_Torpedo_Tube.BP_Torpedo_Tube_C|GetComp_Active (stale Custom|Wait%20Torpedo%20Tube%20Right%20Occupied _righttorpedotube)) (Variables|Internal|GetPlayer%20Pawn) true)
    (else
      (Default|CallOnSequenceUpdate 6 "NewEnumerator1")
      (CallFunction|WaitKeysRightTurned))))

(event Custom|Door%20Left%20Opened
  ;[1 1 1] Wait for the player to open the left torpedo door.
  (EventDispatchers|UnbindEventfromTorpedoDoorOpened (stale Custom|Reset%20Left _leftloadingtubein) (delegate Custom|Door%20Left%20Opened))
  (Default|SetInteractionEnabled (Variables|/Game/_Overseas/Development/Blueprints/Assets/Ship/Munition/BP_Torpedo_Hole_In.BP_Torpedo_Hole_In_C|GetComp_Interaction (stale Custom|Reset%20Left _leftloadingtubein)) false)
  (Default|CallOnSequenceUpdate 1 "NewEnumerator0")
  (CallFunction|WaitTorpedoLeftTransfered))

(event Custom|Torpedo%20Transfered%20Left
  (params (Torpedo%20Rack :type BP%20Torpedo%20Rack%20Object%20Reference))
  ;[1 1 1] Wait for the player to transfer the torpedo from the torpedo rack to the torpedo loading tube.
  (EventDispatchers|UnbindEventfromTorpedoTransfered Torpedo%20Rack (delegate Custom|Torpedo%20Transfered%20Left))
  (Default|SetActive (Variables|/Game/_Overseas/Development/Blueprints/Assets/Ship/Torpedo/BP_Torpedo_Rack.BP_Torpedo_Rack_C|GetComp_Active Torpedo%20Rack) (Variables|Internal|GetPlayer%20Pawn) false)
  (Default|CallOnSequenceUpdate 2 "NewEnumerator0")
  (CallFunction|WaitTorpedoDoorLeftClosed))

(event Custom|Torpedo%20Door%20Left%20Closed
  ;[1 1 1] Wait for the player to close the torpedo loading tube door.
  (EventDispatchers|UnbindEventfromTorpedoDoorClosed (stale Custom|Wait%20Torpedo%20Door%20Left%20Closed _leftloadingtubein) (delegate Custom|Torpedo%20Door%20Left%20Closed))
  (Default|SetActive (Variables|/Game/_Overseas/Development/Blueprints/Assets/Ship/Munition/BP_Torpedo_Hole_In.BP_Torpedo_Hole_In_C|GetComp_Active (stale Custom|Wait%20Torpedo%20Door%20Left%20Closed _leftloadingtubein)) (Variables|Internal|GetPlayer%20Pawn) false)
  (Default|SetInteractionEnabled (Variables|/Game/_Overseas/Development/Blueprints/Assets/Ship/Munition/BP_Torpedo_Hole_In.BP_Torpedo_Hole_In_C|GetComp_Interaction (stale Custom|Wait%20Torpedo%20Door%20Left%20Closed _leftloadingtubein)) false)
  (Default|CallOnSequenceUpdate 3 "NewEnumerator0")
  (CallFunction|WaitTorpedoTubeDoorLeftOpened))

(event Custom|Tube%20Door%20Opened%20Left
  (params (Torpedo%20Tube%20Reference :type BP%20Torpedo%20Tube%20Object%20Reference))
  ;[1 1 1] Wait for the player to open the torpedo tube door in the left torpedo room.
  (EventDispatchers|UnbindEventfromTubeDoorOpened Torpedo%20Tube%20Reference (delegate Custom|Tube%20Door%20Opened%20Left))
  (Default|SetActive (Variables|/Game/_Overseas/Development/Blueprints/Assets/Ship/Torpedo/BP_Torpedo_Tube.BP_Torpedo_Tube_C|GetComp_Active (stale Custom|Wait%20Torpedo%20Tube%20Door%20Left%20Opened _lefttorpedotube)) 0 false)
  (Default|CallOnSequenceUpdate 4 "NewEnumerator0")
  (CallFunction|WaitTorpedoLoadedonLeftRack))

(event Custom|Tube%20Occupied%20Left
  ;[1 1 1] Wait for the player to have loaded the torpedo in the left torpedo tube.
  (EventDispatchers|UnbindEventfromTubeOccupied (stale Custom|Wait%20Torpedo%20Tube%20Left%20Occupied _lefttorpedotube) (delegate Custom|Tube%20Occupied%20Left))
  (CallFunction|MultiCloseTubeDoorLeft))

(event Custom|Torpedo%20Tube%20Door%20Closed%20Left
  (params (Torpedo%20Tube%20Reference :type BP%20Torpedo%20Tube%20Object%20Reference))
  ;[1 1 1] Wait fort the player to close the left torpedo tube door.
  (EventDispatchers|UnbindEventfromTubeDoorClosed Torpedo%20Tube%20Reference (delegate Custom|Torpedo%20Tube%20Door%20Closed%20Left))
  (Default|SetActive (Variables|/Game/_Overseas/Development/Blueprints/Assets/Ship/Torpedo/BP_Torpedo_Tube.BP_Torpedo_Tube_C|GetComp_Active Torpedo%20Tube%20Reference) (Variables|Internal|GetPlayer%20Pawn) false)
  (Default|CallOnSequenceUpdate 6 "NewEnumerator0")
  (CallFunction|WaitKeysLeftTurned))

(event Custom|Key%20Turned%20Left
  (params (Key%20Reference :type BP%20Torpedo%20Launch%20Key%20Object%20Reference))
  ;[1 1 1] Wait for all the keys to be turned.
  (EventDispatchers|UnbindEventfromOnKeyTurned Key%20Reference (delegate Custom|Key%20Turned%20Left))
  (bind _result (Math|Integer|IncrementInt (Variables|Internal|GetKeys%20Turned%20Left))
    (:%20%20
      ;[1 1 1] If all keys are turned, continue.
      (if (== _result (Utilities|Array|Length (Variables|Settings|TorpedoLeft|GetLeftTorpedoKeys)))
        (for _array_element (Variables|Settings|TorpedoLeft|GetLeftTorpedoKeys)
          (EventDispatchers|UnbindEventfromOnKeyTurned _array_element (delegate Custom|Key%20Turned%20Left))
          (Default|SetActive (Variables|/Game/_Overseas/Development/Blueprints/Assets/Ship/Torpedo/BP_Torpedo_LaunchKey.BP_Torpedo_LaunchKey_C|GetComp_Active _array_element) (Variables|Internal|GetPlayer%20Pawn) false))
        ;[1 1 1] If not all keys are turned in time, let the player try again.
        (Utilities|FlowControl|Sequence
          (:then_0
            (goto _label Close))
          (:then_1
            (Default|CallOnSequenceUpdate 7 "NewEnumerator0")
            (CallFunction|WaitButtonLeftPressed)))
        (else
          (Utilities|FlowControl|Sequence
            (:then_0
              (goto _label Open))
            (:then_1
              (Utilities|FlowControl|Delay 2.0)
              (Utilities|FlowControl|Gate true :!label _label
                (:Exit
                  (Variables|Internal|SetKeys%20Turned%20Left 0)
                  (for _array_element_2 (Variables|Settings|TorpedoLeft|GetLeftTorpedoKeys)
                    (EventDispatchers|BindEventtoOnKeyTurned _array_element_2 (delegate Custom|Key%20Turned%20Left))
                    (Default|SetActive (Variables|/Game/_Overseas/Development/Blueprints/Assets/Ship/Torpedo/BP_Torpedo_LaunchKey.BP_Torpedo_LaunchKey_C|GetComp_Active _array_element_2) (Variables|Internal|GetPlayer%20Pawn) true)))))))))))

(event Custom|Button%20Pressed%20Left
  ;[1 1 1] Wait for the launch button to be pressed.
  (EventDispatchers|UnbindEventfromButtonPressed (stale Custom|Wait%20Button%20Left%20Pressed _lefttorpedobutton) (delegate Custom|Button%20Pressed%20Left))
  (Default|SetActive (Variables|/Game/_Overseas/Development/Blueprints/Assets/Ship/Torpedo/BP_Torpedo_Launch_Button.BP_Torpedo_Launch_Button_C|GetComp_Active (stale Custom|Wait%20Button%20Left%20Pressed _lefttorpedobutton)) (Variables|Internal|GetPlayer%20Pawn) false)
  (Variables|Internal|SetKeys%20Turned%20Left 0)
  (Default|CallOnSequenceUpdate 8 "NewEnumerator0")
  (CallFunction|LaunchTorpedoLeft))

(event Custom|Multi_CloseTubeDoorLeft
  ;[1 1 1] Wait fort the player to close the left torpedo tube door.
  (if (not (Default|IsClosed (stale Custom|Wait%20Torpedo%20Tube%20Left%20Occupied _lefttorpedotube)))
    (EventDispatchers|BindEventtoTubeDoorClosed (stale Custom|Wait%20Torpedo%20Tube%20Left%20Occupied _lefttorpedotube) (delegate Custom|Torpedo%20Tube%20Door%20Closed%20Left))
    (Default|SetActive (Variables|/Game/_Overseas/Development/Blueprints/Assets/Ship/Torpedo/BP_Torpedo_Tube.BP_Torpedo_Tube_C|GetComp_Active (stale Custom|Wait%20Torpedo%20Tube%20Left%20Occupied _lefttorpedotube)) (Variables|Internal|GetPlayer%20Pawn) true)
    (else
      (Default|CallOnSequenceUpdate 6 "NewEnumerator0")
      (CallFunction|WaitKeysLeftTurned))))

(event Custom|Torpedo%20Right%20Transfered
  (params (Torpedo%20Rack :type BP%20Torpedo%20Rack%20Object%20Reference))
  ;[1 1 1] Wait for the player to transfer the torpedo from the torpedo rack to the torpedo loading tube.
  (EventDispatchers|UnbindEventfromTorpedoTransfered Torpedo%20Rack (delegate Custom|Torpedo%20Right%20Transfered))
  (Default|SetActive (Variables|/Game/_Overseas/Development/Blueprints/Assets/Ship/Torpedo/BP_Torpedo_Rack.BP_Torpedo_Rack_C|GetComp_Active Torpedo%20Rack) (Variables|Internal|GetPlayer%20Pawn) false)
  (Default|CallOnSequenceUpdate 2 "NewEnumerator1")
  (CallFunction|WaitTorpedoDoorRightClosed))

(event Custom|Wait%20Torpedo%20Loaded%20On%20Left%20Rack
  ;[1 1 1] Torpedo loading Rack
  (bind _lefttorpedoloadingrack (Variables|Settings|TorpedoLeft|GetLeftTorpedoLoadingRack)
    (:then
      (Variables|/Game/_Overseas/Development/Blueprints/Assets/Ship/Torpedo/BP_LoadingRack.BP_LoadingRack_C|GetCurrent%20Torpedo _lefttorpedoloadingrack
        (:then
          (Default|CallOnSequenceUpdate 5 "NewEnumerator0")
          (Variables|/Game/_Overseas/Development/Blueprints/Assets/Ship/Torpedo/BP_LoadingRack.BP_LoadingRack_C|SetCurrent%20Torpedo (Variables|Settings|TorpedoLeft|GetLeftTorpedoLoadingRack) 0)
          (CallFunction|WaitTorpedoTubeLeftOccupied))
        (:else
          (EventDispatchers|BindEventtoTorpedoLoadedonRack _lefttorpedoloadingrack (delegate Custom|Torpedo%20Loaded%20On%20Rack%20Left)))))
    (:else)))

(event Custom|Torpedo%20Loaded%20On%20Rack%20Left
  ;[1 1 1] Torpedo loading Rack
  (EventDispatchers|UnbindEventfromTorpedoLoadedonRack (stale Custom|Wait%20Torpedo%20Loaded%20On%20Left%20Rack _lefttorpedoloadingrack) (delegate Custom|Torpedo%20Loaded%20On%20Rack%20Left))
  (Default|CallOnSequenceUpdate 5 "NewEnumerator0")
  (Variables|/Game/_Overseas/Development/Blueprints/Assets/Ship/Torpedo/BP_LoadingRack.BP_LoadingRack_C|SetCurrent%20Torpedo (Variables|Settings|TorpedoLeft|GetLeftTorpedoLoadingRack) 0)
  (CallFunction|WaitTorpedoTubeLeftOccupied))

(event Custom|Reset%20Left
  ;[1 1 1] Wait for the player to open the left torpedo door.
  (bind _leftloadingtubein (Variables|Settings|TorpedoLeft|GetLeftLoadingTubeIn)
    (:then
      (if (Default|IsOpened _leftloadingtubein)
        (Default|CallOnSequenceUpdate 1 "NewEnumerator0")
        (CallFunction|WaitTorpedoLeftTransfered)
        (else
          (EventDispatchers|BindEventtoTorpedoDoorOpened _leftloadingtubein (delegate Custom|Door%20Left%20Opened))
          (Default|SetInteractionEnabled (Variables|/Game/_Overseas/Development/Blueprints/Assets/Ship/Munition/BP_Torpedo_Hole_In.BP_Torpedo_Hole_In_C|GetComp_Interaction _leftloadingtubein) true)
          (Default|CallOnSequenceUpdate 0 "NewEnumerator0"))))
    (:else)))

(event Custom|Torpedo%20Tube%20Door%20Right%20Opened
  (params (Torpedo%20Tube%20Reference :type BP%20Torpedo%20Tube%20Object%20Reference))
  ;[1 1 1] Wait for the player to open the torpedo tube door in the left torpedo room.
  (EventDispatchers|UnbindEventfromTubeDoorOpened Torpedo%20Tube%20Reference (delegate Custom|Torpedo%20Tube%20Door%20Right%20Opened))
  (Default|SetActive (Variables|/Game/_Overseas/Development/Blueprints/Assets/Ship/Torpedo/BP_Torpedo_Tube.BP_Torpedo_Tube_C|GetComp_Active (stale Custom|Wait%20Torpedo%20Tube%20Door%20Right%20Opened _righttorpedotube)) 0 false)
  (Default|CallOnSequenceUpdate 4 "NewEnumerator1")
  (CallFunction|WaitTorpedoLoadedonRightRack))

(event Custom|Reset%20Right
  ;[1 1 1] Wait for the player to open the left torpedo door.
  (bind _rightloadingtubein (Variables|Settings|TorpedoRight|GetRightLoadingTubeIn)
    (:then
      (if (Default|IsOpened _rightloadingtubein)
        (Default|CallOnSequenceUpdate 1 "NewEnumerator1")
        (CallFunction|WaitTorpedoRightTransfered)
        (else
          (EventDispatchers|BindEventtoTorpedoDoorOpened _rightloadingtubein (delegate Custom|Torpedo%20Door%20Right%20Opened))
          (Default|SetInteractionEnabled (Variables|/Game/_Overseas/Development/Blueprints/Assets/Ship/Munition/BP_Torpedo_Hole_In.BP_Torpedo_Hole_In_C|GetComp_Interaction _rightloadingtubein) true)
          (Default|CallOnSequenceUpdate 0 "NewEnumerator1"))))
    (:else)))

(event Custom|On%20update
  (params (Index :type Integer) (Direction :type E_Torpedo_Direction%20Enum :default "NewEnumerator0"))
  ;[1 1 1] Update the sequence index.
  (switch Utilities|FlowControl|Switch|SwitchonE_Torpedo_Direction Direction
    (:NewEnumerator0
      (Variables|Internal|SetSequence%20Index%20Left Index))
    (:NewEnumerator1
      (Variables|Internal|SetSequence%20Index%20Right Index))))

(event Custom|Wait%20Torpedo%20Left%20Transfered
  ;[1 1 1] Wait for the player to transfer the torpedo from the torpedo rack to the torpedo loading tube.
  (bind _lefttorpedorack (Variables|Settings|TorpedoLeft|GetLeftTorpedoRack)
    (:then
      (Default|SetActive (Variables|/Game/_Overseas/Development/Blueprints/Assets/Ship/Torpedo/BP_Torpedo_Rack.BP_Torpedo_Rack_C|GetComp_Active _lefttorpedorack) (Variables|Internal|GetPlayer%20Pawn) true)
      (EventDispatchers|BindEventtoTorpedoTransfered _lefttorpedorack (delegate Custom|Torpedo%20Transfered%20Left)))
    (:else)))

(event Custom|Wait%20Torpedo%20Door%20Left%20Closed
  ;[1 1 1] Wait for the player to close the torpedo loading tube door.
  (bind _leftloadingtubein (Variables|Settings|TorpedoLeft|GetLeftLoadingTubeIn)
    (:then
      (if (Default|IsOpened _leftloadingtubein)
        (EventDispatchers|AssignTorpedoDoorClosed _leftloadingtubein (delegate Custom|Torpedo%20Door%20Left%20Closed))
        (Default|SetActive (Variables|/Game/_Overseas/Development/Blueprints/Assets/Ship/Munition/BP_Torpedo_Hole_In.BP_Torpedo_Hole_In_C|GetComp_Active _leftloadingtubein) (Variables|Internal|GetPlayer%20Pawn) true)
        (Default|SetInteractionEnabled (Variables|/Game/_Overseas/Development/Blueprints/Assets/Ship/Munition/BP_Torpedo_Hole_In.BP_Torpedo_Hole_In_C|GetComp_Interaction _leftloadingtubein) true)
        (else
          (Default|CallOnSequenceUpdate 3 "NewEnumerator0")
          (CallFunction|WaitTorpedoTubeDoorLeftOpened))))
    (:else)))

(event Custom|Wait%20Torpedo%20Tube%20Door%20Left%20Opened
  ;[1 1 1] Wait for the player to open the torpedo tube door in the left torpedo room.
  (bind _lefttorpedotube (Variables|Settings|TorpedoLeft|GetLeftTorpedoTube)
    (:then
      (if (Default|IsClosed _lefttorpedotube)
        (EventDispatchers|BindEventtoTubeDoorOpened _lefttorpedotube (delegate Custom|Tube%20Door%20Opened%20Left))
        (Default|SetActive (Variables|/Game/_Overseas/Development/Blueprints/Assets/Ship/Torpedo/BP_Torpedo_Tube.BP_Torpedo_Tube_C|GetComp_Active _lefttorpedotube) (Variables|Internal|GetPlayer%20Pawn) true)
        ;[1 1 1] Spawn a torpedo in in the left torpedo room.
        (bind _lefttorpedotubeout (Variables|Settings|TorpedoLeft|GetLeftTorpedoTubeOut)
          (:then
            (Default|SetActive (Variables|/Game/_Overseas/Development/Blueprints/Assets/Ship/Munition/BP_Torpedo_Hole_Out.BP_Torpedo_Hole_Out_C|GetComp_Active _lefttorpedotubeout) (Variables|Internal|GetPlayer%20Pawn) true))
          (:else))
        (else
          (Default|CallOnSequenceUpdate 4 "NewEnumerator0")
          (CallFunction|WaitTorpedoLoadedonLeftRack))))
    (:else)))

(event Custom|Wait%20Keys%20Left%20Turned
  ;[1 1 1] Wait for all the keys to be turned.
  (if (!= (Variables|Internal|GetKeys%20Turned%20Left) (Utilities|Array|Length (Variables|Settings|TorpedoLeft|GetLeftTorpedoKeys)))
    (Variables|Internal|SetKeys%20Turned%20Left 0)
    (for _array_element (Variables|Settings|TorpedoLeft|GetLeftTorpedoKeys)
      (EventDispatchers|BindEventtoOnKeyTurned _array_element (delegate Custom|Key%20Turned%20Left))
      (Default|SetActive (Variables|/Game/_Overseas/Development/Blueprints/Assets/Ship/Torpedo/BP_Torpedo_LaunchKey.BP_Torpedo_LaunchKey_C|GetComp_Active _array_element) (Variables|Internal|GetPlayer%20Pawn) true))
    (else
      ;[1 1 1] If not all keys are turned in time, let the player try again.
      (Utilities|FlowControl|Sequence
        (:then_0
          (Utilities|FlowControl|Gate true) ; enters at Close
        )
        (:then_1
          (Default|CallOnSequenceUpdate 7 "NewEnumerator0")
          (CallFunction|WaitButtonLeftPressed))))))

(event Custom|Launch%20Torpedo%20Left
  ;[1 1 1] Launch the torpedo from the torpedo tube.
  (bind _lefttorpedotube (Variables|Settings|TorpedoLeft|GetLeftTorpedoTube)
    (:then
      (Default|LaunchTorpedo _lefttorpedotube)
      ;[1 1 1] Turn off the confirmation light.
      (bind _lefttorpedolight (Variables|Settings|TorpedoLeft|GetLeftTorpedoLight)
        (:then
          (Default|SetActive (Variables|/Game/_Overseas/Development/Blueprints/Assets/Ship/Torpedo/BP_Torpedo_Launch_Lamp.BP_Torpedo_Launch_Lamp_C|GetComp_Active _lefttorpedolight) (Variables|Internal|GetPlayer%20Pawn) false)
          (Default|CallOnSequenceEnd "NewEnumerator0")
          (CallFunction|ResetLeft))
        (:else)))
    (:else)))

(event Custom|Wait%20Torpedo%20Tube%20Left%20Occupied
  ;[1 1 1] Wait for the player to have loaded the torpedo in the left torpedo tube.
  (bind _lefttorpedotube (Variables|Settings|TorpedoLeft|GetLeftTorpedoTube)
    (:then
      (if (Default|IsOccupied _lefttorpedotube)
        ;[1 1 1] Wait fort the player to close the left torpedo tube door.
        (if (not (Default|IsClosed _lefttorpedotube))
          (EventDispatchers|BindEventtoTubeDoorClosed _lefttorpedotube (delegate Custom|Torpedo%20Tube%20Door%20Closed%20Left))
          (Default|SetActive (Variables|/Game/_Overseas/Development/Blueprints/Assets/Ship/Torpedo/BP_Torpedo_Tube.BP_Torpedo_Tube_C|GetComp_Active _lefttorpedotube) (Variables|Internal|GetPlayer%20Pawn) true)
          (else
            (Default|CallOnSequenceUpdate 6 "NewEnumerator0")
            (CallFunction|WaitKeysLeftTurned)))
        (else
          (Networking|SwitchHasAuthority
            (:Authority
              (EventDispatchers|AssignTubeOccupied _lefttorpedotube (delegate Custom|Tube%20Occupied%20Left))
              (Default|LoadTorpedo (Variables|Settings|TorpedoLeft|GetLeftTorpedoTube) (Variables|/Game/_Overseas/Development/Blueprints/Assets/Ship/Munition/BP_Torpedo_Hole_Out.BP_Torpedo_Hole_Out_C|GetSpawned%20Torpedo (Variables|Settings|TorpedoLeft|GetLeftTorpedoTubeOut))))))))
    (:else)))

(event Custom|Torpedo%20Door%20Right%20Closed
  ;[1 1 1] Wait for the player to close the torpedo loading tube door.
  (EventDispatchers|UnbindEventfromTorpedoDoorClosed (stale Custom|Wait%20Torpedo%20Door%20Right%20Closed _rightloadingtubein) (delegate Custom|Torpedo%20Door%20Right%20Closed))
  (Default|SetActive (Variables|/Game/_Overseas/Development/Blueprints/Assets/Ship/Munition/BP_Torpedo_Hole_In.BP_Torpedo_Hole_In_C|GetComp_Active (stale Custom|Wait%20Torpedo%20Door%20Right%20Closed _rightloadingtubein)) (Variables|Internal|GetPlayer%20Pawn) false)
  (Default|SetInteractionEnabled (Variables|/Game/_Overseas/Development/Blueprints/Assets/Ship/Munition/BP_Torpedo_Hole_In.BP_Torpedo_Hole_In_C|GetComp_Interaction (stale Custom|Wait%20Torpedo%20Door%20Right%20Closed _rightloadingtubein)) false)
  (Default|CallOnSequenceUpdate 3 "NewEnumerator1")
  (CallFunction|WaitTorpedoTubeDoorRightOpened))

(event Custom|Wait%20Button%20Left%20Pressed
  ;[1 1 1] Turn on the comfirmation light.
  (bind _lefttorpedolight (Variables|Settings|TorpedoLeft|GetLeftTorpedoLight)
    (:then
      (Default|SetActive (Variables|/Game/_Overseas/Development/Blueprints/Assets/Ship/Torpedo/BP_Torpedo_Launch_Lamp.BP_Torpedo_Launch_Lamp_C|GetComp_Active _lefttorpedolight) (Variables|Internal|GetPlayer%20Pawn) true))
    (:else
      _))
  ;[1 1 1] Wait for the launch button to be pressed.
  (bind _lefttorpedobutton (Variables|Settings|TorpedoLeft|GetLeftTorpedoButton)
    (:then
      (Default|SetActive (Variables|/Game/_Overseas/Development/Blueprints/Assets/Ship/Torpedo/BP_Torpedo_Launch_Button.BP_Torpedo_Launch_Button_C|GetComp_Active _lefttorpedobutton) 0 true)
      (EventDispatchers|BindEventtoButtonPressed _lefttorpedobutton (delegate Custom|Button%20Pressed%20Left)))
    (:else)))

(event Custom|Wait%20Torpedo%20Right%20Transfered
  ;[1 1 1] Wait for the player to transfer the torpedo from the torpedo rack to the torpedo loading tube.
  (bind _righttorpedorack (Variables|Settings|TorpedoRight|GetRightTorpedoRack)
    (:then
      (Default|SetActive (Variables|/Game/_Overseas/Development/Blueprints/Assets/Ship/Torpedo/BP_Torpedo_Rack.BP_Torpedo_Rack_C|GetComp_Active _righttorpedorack) (Variables|Internal|GetPlayer%20Pawn) true)
      (EventDispatchers|BindEventtoTorpedoTransfered _righttorpedorack (delegate Custom|Torpedo%20Right%20Transfered)))
    (:else)))

(event Custom|Wait%20Torpedo%20Door%20Right%20Closed
  ;[1 1 1] Wait for the player to close the torpedo loading tube door.
  (bind _rightloadingtubein (Variables|Settings|TorpedoRight|GetRightLoadingTubeIn)
    (:then
      (if (Default|IsOpened _rightloadingtubein)
        (EventDispatchers|AssignTorpedoDoorClosed _rightloadingtubein (delegate Custom|Torpedo%20Door%20Right%20Closed))
        (Default|SetActive (Variables|/Game/_Overseas/Development/Blueprints/Assets/Ship/Munition/BP_Torpedo_Hole_In.BP_Torpedo_Hole_In_C|GetComp_Active _rightloadingtubein) (Variables|Internal|GetPlayer%20Pawn) true)
        (Default|SetInteractionEnabled (Variables|/Game/_Overseas/Development/Blueprints/Assets/Ship/Munition/BP_Torpedo_Hole_In.BP_Torpedo_Hole_In_C|GetComp_Interaction _rightloadingtubein) true)
        (else
          (Default|CallOnSequenceUpdate 3 "NewEnumerator1")
          (CallFunction|WaitTorpedoTubeDoorRightOpened))))
    (:else)))

(event Custom|Wait%20Torpedo%20Tube%20Door%20Right%20Opened
  ;[1 1 1] Wait for the player to open the torpedo tube door in the left torpedo room.
  (bind _righttorpedotube (Variables|Settings|TorpedoRight|GetRightTorpedoTube)
    (:then
      (if (Default|IsClosed _righttorpedotube)
        (EventDispatchers|BindEventtoTubeDoorOpened _righttorpedotube (delegate Custom|Torpedo%20Tube%20Door%20Right%20Opened))
        (Default|SetActive (Variables|/Game/_Overseas/Development/Blueprints/Assets/Ship/Torpedo/BP_Torpedo_Tube.BP_Torpedo_Tube_C|GetComp_Active _righttorpedotube) (Variables|Internal|GetPlayer%20Pawn) true)
        ;[1 1 1] Spawn a torpedo in in the left torpedo room.
        (bind _righttorpedotubeout (Variables|Settings|TorpedoRight|GetRightTorpedoTubeOut)
          (:then
            (Default|SetActive (Variables|/Game/_Overseas/Development/Blueprints/Assets/Ship/Munition/BP_Torpedo_Hole_Out.BP_Torpedo_Hole_Out_C|GetComp_Active _righttorpedotubeout) (Variables|Internal|GetPlayer%20Pawn) true))
          (:else))
        (else
          (Default|CallOnSequenceUpdate 4 "NewEnumerator1")
          (CallFunction|WaitTorpedoLoadedonRightRack))))
    (:else)))

(event Custom|Wait%20Torpedo%20Tube%20Right%20Occupied
  ;[1 1 1] Wait for the player to have loaded the torpedo in the left torpedo tube.
  (bind _righttorpedotube (Variables|Settings|TorpedoRight|GetRightTorpedoTube)
    (:then
      (if (Default|IsOccupied _righttorpedotube)
        ;[1 1 1] Wait fort the player to close the left torpedo tube door.
        (if (not (Default|IsClosed _righttorpedotube))
          (EventDispatchers|BindEventtoTubeDoorClosed _righttorpedotube (delegate Custom|Torpedo%20Tube%20Door%20Right%20Closed))
          (Default|SetActive (Variables|/Game/_Overseas/Development/Blueprints/Assets/Ship/Torpedo/BP_Torpedo_Tube.BP_Torpedo_Tube_C|GetComp_Active _righttorpedotube) (Variables|Internal|GetPlayer%20Pawn) true)
          (else
            (Default|CallOnSequenceUpdate 6 "NewEnumerator1")
            (CallFunction|WaitKeysRightTurned)))
        (else
          (Networking|SwitchHasAuthority
            (:Authority
              (EventDispatchers|AssignTubeOccupied _righttorpedotube (delegate Custom|Torpedo%20Tube%20Right%20Occupied))
              (Default|LoadTorpedo (Variables|Settings|TorpedoRight|GetRightTorpedoTube) (Variables|/Game/_Overseas/Development/Blueprints/Assets/Ship/Munition/BP_Torpedo_Hole_Out.BP_Torpedo_Hole_Out_C|GetSpawned%20Torpedo (Variables|Settings|TorpedoRight|GetRightTorpedoTubeOut))))))))
    (:else)))

(event Custom|Wait%20Keys%20Right%20Turned
  ;[1 1 1] Wait for all the keys to be turned.
  (if (!= (Variables|Internal|GetKeys%20Turned%20Right) (Utilities|Array|Length (Variables|Settings|TorpedoRight|GetRightTorpedoKeys)))
    (Variables|Internal|SetKeys%20Turned%20Right 0)
    (for _array_element (Variables|Settings|TorpedoRight|GetRightTorpedoKeys)
      (EventDispatchers|BindEventtoOnKeyTurned _array_element (delegate Custom|Key%20Right%20Turned))
      (Default|SetActive (Variables|/Game/_Overseas/Development/Blueprints/Assets/Ship/Torpedo/BP_Torpedo_LaunchKey.BP_Torpedo_LaunchKey_C|GetComp_Active _array_element) (Variables|Internal|GetPlayer%20Pawn) true))
    (else
      ;[1 1 1] If not all keys are turned in time, let the player try again.
      (Utilities|FlowControl|Sequence
        (:then_0
          (Utilities|FlowControl|Gate true) ; enters at Close
        )
        (:then_1
          (Default|CallOnSequenceUpdate 7 "NewEnumerator1")
          (CallFunction|WaitButtonRightPressed))))))

(event Custom|Wait%20Button%20Right%20Pressed
  ;[1 1 1] Turn on the comfirmation light.
  (bind _righttorpedolight (Variables|Settings|TorpedoRight|GetRightTorpedoLight)
    (:then
      (Default|SetActive (Variables|/Game/_Overseas/Development/Blueprints/Assets/Ship/Torpedo/BP_Torpedo_Launch_Lamp.BP_Torpedo_Launch_Lamp_C|GetComp_Active _righttorpedolight) (Variables|Internal|GetPlayer%20Pawn) true))
    (:else
      _))
  ;[1 1 1] Wait for the launch button to be pressed.
  (bind _righttorpedobutton (Variables|Settings|TorpedoRight|GetRightTorpedoButton)
    (:then
      (Default|SetActive (Variables|/Game/_Overseas/Development/Blueprints/Assets/Ship/Torpedo/BP_Torpedo_Launch_Button.BP_Torpedo_Launch_Button_C|GetComp_Active _righttorpedobutton) 0 true)
      (EventDispatchers|BindEventtoButtonPressed _righttorpedobutton (delegate Custom|Button%20Right%20Pressed)))
    (:else)))

(event Custom|Launch%20Torpedo%20Right
  ;[1 1 1] Launch the torpedo from the torpedo tube.
  (bind _righttorpedotube (Variables|Settings|TorpedoRight|GetRightTorpedoTube)
    (:then
      (Default|LaunchTorpedo _righttorpedotube)
      ;[1 1 1] Turn off the confirmation light.
      (bind _righttorpedolight (Variables|Settings|TorpedoRight|GetRightTorpedoLight)
        (:then
          (Default|SetActive (Variables|/Game/_Overseas/Development/Blueprints/Assets/Ship/Torpedo/BP_Torpedo_Launch_Lamp.BP_Torpedo_Launch_Lamp_C|GetComp_Active _righttorpedolight) (Variables|Internal|GetPlayer%20Pawn) false)
          (Default|CallOnSequenceEnd "NewEnumerator0")
          (CallFunction|ResetRight))
        (:else)))
    (:else)))

(event Custom|Torpedo%20Tube%20Right%20Occupied
  ;[1 1 1] Wait for the player to have loaded the torpedo in the left torpedo tube.
  (EventDispatchers|UnbindEventfromTubeOccupied (stale Custom|Wait%20Torpedo%20Tube%20Right%20Occupied _righttorpedotube) (delegate Custom|Torpedo%20Tube%20Right%20Occupied))
  (CallFunction|MultiCloseTubeDoorRight))

(event Custom|Torpedo%20Loaded%20On%20Rack%20Right
  ;[1 1 1] Torpedo loading Rack
  (EventDispatchers|UnbindEventfromTorpedoLoadedonRack (stale Custom|Wait%20Torpedo%20Loaded%20On%20Right%20Rack _righttorpedoloadingrack) (delegate Custom|Torpedo%20Loaded%20On%20Rack%20Right))
  (Default|CallOnSequenceUpdate 5 "NewEnumerator1")
  (Variables|/Game/_Overseas/Development/Blueprints/Assets/Ship/Torpedo/BP_LoadingRack.BP_LoadingRack_C|SetCurrent%20Torpedo (Variables|Settings|TorpedoRight|GetRightTorpedoLoadingRack) 0)
  (CallFunction|WaitTorpedoTubeRightOccupied))

(event Custom|Torpedo%20Tube%20Door%20Right%20Closed
  (params (Torpedo%20Tube%20Reference :type BP%20Torpedo%20Tube%20Object%20Reference))
  ;[1 1 1] Wait fort the player to close the left torpedo tube door.
  (EventDispatchers|UnbindEventfromTubeDoorClosed Torpedo%20Tube%20Reference (delegate Custom|Torpedo%20Tube%20Door%20Right%20Closed))
  (Default|SetActive (Variables|/Game/_Overseas/Development/Blueprints/Assets/Ship/Torpedo/BP_Torpedo_Tube.BP_Torpedo_Tube_C|GetComp_Active Torpedo%20Tube%20Reference) (Variables|Internal|GetPlayer%20Pawn) false)
  (Default|CallOnSequenceUpdate 6 "NewEnumerator1")
  (CallFunction|WaitKeysRightTurned))

(event Custom|Key%20Right%20Turned
  (params (Key%20Reference :type BP%20Torpedo%20Launch%20Key%20Object%20Reference))
  ;[1 1 1] Wait for all the keys to be turned.
  (EventDispatchers|UnbindEventfromOnKeyTurned Key%20Reference (delegate Custom|Key%20Right%20Turned))
  (bind _result (Math|Integer|IncrementInt (Variables|Internal|GetKeys%20Turned%20Right))
    (:%20%20
      ;[1 1 1] If all keys are turned, continue.
      (if (== _result (Utilities|Array|Length (Variables|Settings|TorpedoRight|GetRightTorpedoKeys)))
        (for _array_element (Variables|Settings|TorpedoRight|GetRightTorpedoKeys)
          (EventDispatchers|UnbindEventfromOnKeyTurned _array_element (delegate Custom|Key%20Right%20Turned))
          (Default|SetActive (Variables|/Game/_Overseas/Development/Blueprints/Assets/Ship/Torpedo/BP_Torpedo_LaunchKey.BP_Torpedo_LaunchKey_C|GetComp_Active _array_element) (Variables|Internal|GetPlayer%20Pawn) false))
        ;[1 1 1] If not all keys are turned in time, let the player try again.
        (Utilities|FlowControl|Sequence
          (:then_0
            (goto _label Close))
          (:then_1
            (Default|CallOnSequenceUpdate 7 "NewEnumerator1")
            (CallFunction|WaitButtonRightPressed)))
        (else
          (Utilities|FlowControl|Sequence
            (:then_0
              (goto _label Open))
            (:then_1
              (Utilities|FlowControl|Delay 2.0)
              (Utilities|FlowControl|Gate true :!label _label
                (:Exit
                  (Variables|Internal|SetKeys%20Turned%20Right 0)
                  (for _array_element_2 (Variables|Settings|TorpedoRight|GetRightTorpedoKeys)
                    (EventDispatchers|BindEventtoOnKeyTurned _array_element_2 (delegate Custom|Key%20Right%20Turned))
                    (Default|SetActive (Variables|/Game/_Overseas/Development/Blueprints/Assets/Ship/Torpedo/BP_Torpedo_LaunchKey.BP_Torpedo_LaunchKey_C|GetComp_Active _array_element_2) (Variables|Internal|GetPlayer%20Pawn) true)))))))))))

(event Custom|Button%20Right%20Pressed
  ;[1 1 1] Wait for the launch button to be pressed.
  (EventDispatchers|UnbindEventfromButtonPressed (stale Custom|Wait%20Button%20Right%20Pressed _righttorpedobutton) (delegate Custom|Button%20Right%20Pressed))
  (Default|SetActive (Variables|/Game/_Overseas/Development/Blueprints/Assets/Ship/Torpedo/BP_Torpedo_Launch_Button.BP_Torpedo_Launch_Button_C|GetComp_Active (stale Custom|Wait%20Button%20Right%20Pressed _righttorpedobutton)) (Variables|Internal|GetPlayer%20Pawn) false)
  (Variables|Internal|SetKeys%20Turned%20Right 0)
  (Default|CallOnSequenceUpdate 8 "NewEnumerator1")
  (CallFunction|LaunchTorpedoRight))

(event EventBeginPlay
  (bind _self self)
  (bind _player_pawn (CallFunction|GetMainPlayerPawn _self))
  ;[1 1 1] Set the player pawn that is used for the active components.
  (Utilities|WaitforObjecttoValidate _player_pawn 0.05
    (:Is%20Valid
      (Variables|Internal|SetPlayer%20Pawn _player_pawn)
      (Utilities|FlowControl|Sequence
        (:then_0
          ;[1 1 1] Deactive all active components so that the player cannot interact with the objects.
          (bind _interactable_actors (CallFunction|GetInteractableArray (Utilities|Array|MakeArray (Variables|Settings|TorpedoLeft|GetLeftTorpedoRack) (Variables|Settings|TorpedoLeft|GetLeftTorpedoTubeOut) (Variables|Settings|TorpedoLeft|GetLeftTorpedoTube) (Variables|Settings|TorpedoLeft|GetLeftTorpedoLight) (Variables|Settings|TorpedoLeft|GetLeftTorpedoButton) (Variables|Settings|TorpedoRight|GetRightTorpedoRack) (Variables|Settings|TorpedoRight|GetRightTorpedoTubeOut) (Variables|Settings|TorpedoRight|GetRightTorpedoTube) (Variables|Settings|TorpedoRight|GetRightTorpedoLight) (Variables|Settings|TorpedoRight|GetRightTorpedoButton))))
          (for _array_element _interactable_actors
            (Utilities|IsValid _array_element
              (:Is%20Valid
                (Default|SetActive (Actor|GetComponentbyClass _array_element "/Game/_Overseas/Development/Blueprints/Components/Core/Comp_Active.Comp_Active_C") (Variables|Internal|GetPlayer%20Pawn) false)))))
        (:then_1
          ;[1 1 1] Update the sequence index.
          (EventDispatchers|BindEventtoOnSequenceUpdate (delegate Custom|On%20update)))
        (:then_2
          (CallFunction|ResetLeft))
        (:then_3
          (CallFunction|ResetRight))))))

(fn ConstructionScript)

(fn GetInteractableArray
  (params (Already%20Found :type Array%20of%20Actor%20Object%20References))
  (bind _output_get (LocalVariables|SetReturn Already%20Found))
  (Utilities|Array|AppendArray _output_get (Variables|Settings|TorpedoLeft|GetLeftTorpedoKeys))
  (Utilities|Array|AppendArray (LocalVariables|GetReturn) (Variables|Settings|TorpedoRight|GetRightTorpedoKeys))
  (return (LocalVariables|GetReturn)))