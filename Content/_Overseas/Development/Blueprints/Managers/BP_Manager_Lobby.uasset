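; Lobby manager actor that drives a widget-component lobby UI for player count, game start and voice chat settings.
; It updates the widget from the GameMode's login and logout events, and the start button runs servertravel to LevelName on the authority.
; The checkbox multicasts a FlipFlop between two GameInstance voice chat values.
; One second after a join, the stored setting is multicast again to sync players.
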(event Custom|PlayerJoined
  (Default|PlayerJoined (Variables|Default|GetLobbyWidget))
  (Utilities|FlowControl|Delay 1.0)
  (CallFunction|MulticastSetVoiceChatSettings (Variables|Default|GetSettings)))

(event Custom|StartGame
  (params (Source%20Actor :type Actor%20Object%20Reference) (Hit%20Location :type Vector) (Hit%20Component :type Actor%20Component%20Object%20Reference) (Button%20Reference :type WB%20Button%20Object%20Reference))
  (Networking|SwitchHasAuthority
    (:Authority
      (Development|ExecuteConsoleCommand (Utilities|String|Append "servertravel " (Variables|Default|GetLevelName)) 0)
      (Development|PrintString "Game start"))))

(event Custom|OnVOiceChatSettingsChange
  (params (Source%20Actor :type Actor%20Object%20Reference) (Hit%20Location :type Vector) (Hit%20Component :type Actor%20Component%20Object%20Reference) (Button%20Reference :type WB%20Button%20Object%20Reference))
  (CallFunction|MulticastChangeVoiceChatSettings))

(event Custom|Multicast_ChangeVoiceChatSettings
  (bind _asbp_game_instance_main (Utilities|Casting|CastToBP_GameInstance_Main (Game|GetGameInstance)))
  (Utilities|FlowControl|FlipFlop
    (:A
      (bind _output_get (Variables|/Game/_Overseas/Development/Game/BP_GameInstance_Main.BP_GameInstance_Main_C|SetVoiceChatSettings _asbp_game_instance_main "NewEnumerator0"))
      (Variables|Default|SetSettings _output_get))
    (:B
      (bind _output_get_2 (Variables|/Game/_Overseas/Development/Game/BP_GameInstance_Main.BP_GameInstance_Main_C|SetVoiceChatSettings _asbp_game_instance_main "NewEnumerator1"))
      (Variables|Default|SetSettings _output_get_2))))

(event Custom|Multicast_SetVoiceChatSettings
  (params (VoicechatSettings :type E_Voice_Chat_Modes%20Enum :default "NewEnumerator0"))
  (bind _asbp_game_instance_main (Utilities|Casting|CastToBP_GameInstance_Main (Game|GetGameInstance)))
  (Variables|/Game/_Overseas/Development/Game/BP_GameInstance_Main.BP_GameInstance_Main_C|SetVoiceChatSettings _asbp_game_instance_main VoicechatSettings))

(event Custom|Player%20Left
  (Default|PlayerLeft (Variables|Default|GetLobbyWidget)))

(event EventBeginPlay
  (bind _returnvalue (Game|GetGameMode))
  (|CallParentFunction)
  (bind _aswb_lobby (Utilities|Casting|CastToWB_Lobby (UserInterface|GetWidget (Variables|Default|GetComp_Widget))))
  (bind _output_get (Variables|Default|SetLobbyWidget _aswb_lobby))
  (EventDispatchers|BindEventtoButtonPressed (Variables|/Game/_Overseas/Development/Blueprints/Widgets/MainMenu/WB_Lobby.WB_Lobby_C|GetWB_Button_Normal _output_get) (delegate Custom|StartGame))
  (EventDispatchers|BindEventtoButtonPressed (Variables|/Game/_Overseas/Development/Blueprints/Widgets/MainMenu/WB_Lobby.WB_Lobby_C|GetWB_CheckBox (Variables|Default|GetLobbyWidget)) (delegate Custom|OnVOiceChatSettingsChange))
  (Utilities|IsValid _returnvalue
    (:Is%20Valid
      (bind _returnvalue_2 (Class|GameModeBase|GetNumPlayers _returnvalue))
      (Default|SetPlayerCount (Variables|Default|GetLobbyWidget) _returnvalue_2)
      (bind _asbp_game_mode_main (Utilities|Casting|CastToBP_GameMode_Main _returnvalue))
      (EventDispatchers|BindEventtoOnPlayerLogin _asbp_game_mode_main (delegate Custom|PlayerJoined))
      (EventDispatchers|BindEventtoOnPlayerLogOut _asbp_game_mode_main (delegate Custom|Player%20Left)))))

(event Collision|EventActorBeginOverlap
  (params (OtherActor :type Actor%20Object%20Reference)))

(event EventTick
  (params (DeltaSeconds :type Float%20%28single-precision%29))
  (|CallParentFunction DeltaSeconds))

(fn ConstructionScript
  (|CallParentFunction))