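; Base pawn that lets players select, highlight and activate actor components, and quits the game on Escape.
; Select and Activate events act locally for non-replicated owners, or route through server and multicast events for replicated ones.
; Hit-result helpers press or highlight eligible Comp_Select components directly, without that network routing.
; UpdateHUDColor asks BP_PlayerController_Main to turn the HUD red over selectable components, with a default color otherwise.
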(event Custom|Select
  (params (Select%20Component :type Comp%20Select%20Object%20Reference) (Hit%20Location :type Vector) (Hit%20Component :type Actor%20Component%20Object%20Reference))
  (bind _self self)
  (bind _self_2 self)
  ;[1 1 1] Call the select component over the server or locally if the select component's owner doesn't replicate
  ;;[0 0 0] Check to call the select component locally or over the server
  (Utilities|IsValid Select%20Component
    (:Is%20Valid
      (if (Variables|/Script/Engine.Actor|GetbReplicates (Components|GetOwner Select%20Component))
        (CallFunction|ServerSelect _self_2 Select%20Component _self_2 Hit%20Location)
        (else
          (Default|SelectPressed Select%20Component _self _self Hit%20Location Hit%20Component))))))

(event Custom|Multi_Select
  (params (Pawn :type BP%20Pawn%20Base%20Object%20Reference) (Select%20Component :type Comp%20Select%20Object%20Reference) (Source%20Actor :type Actor%20Object%20Reference) (Hit%20Location :type Vector) (Hit%20Component :type Actor%20Component%20Object%20Reference))
  ;[1 1 1] Call the select component over the server or locally if the select component's owner doesn't replicate
  ;;[0 0 0] Multicast the select component call to all clients
  (Default|SelectPressed Select%20Component Pawn Source%20Actor Hit%20Location Hit%20Component))

(event Custom|Multi_Activate
  (params (Pawn :type BP%20Pawn%20Base%20Object%20Reference) (Active%20Component :type Comp%20Active%20Object%20Reference) (Set :type Boolean))
  ;[1 1 1] Server Set Active State
  ;;[0 0 0] Multicast the active component call to all clients
  (Default|SetActive Active%20Component Pawn Set))

(event Custom|Server_Select
  (params (Pawn :type BP%20Pawn%20Base%20Object%20Reference) (Select%20Component :type Comp%20Select%20Object%20Reference) (Source%20Actor :type Actor%20Object%20Reference) (Hit%20Location :type Vector) (Hit%20Component :type Actor%20Component%20Object%20Reference))
  ;[1 1 1] Call the select component over the server or locally if the select component's owner doesn't replicate
  ;;[0 0 0] Call the select component over the server
  (CallFunction|MultiSelect Pawn Select%20Component Source%20Actor Hit%20Location Hit%20Component))

(event Custom|Server_Activate
  (params (Pawn :type BP%20Pawn%20Base%20Object%20Reference) (Active%20Component :type Comp%20Active%20Object%20Reference) (Set :type Boolean))
  ;[1 1 1] Server Set Active State
  ;;[0 0 0] Call the active component over the server
  (CallFunction|MultiActivate Pawn Active%20Component Set))

(event Custom|Activate
  (params (Active%20Component :type Comp%20Active%20Object%20Reference) (Set :type Boolean))
  ;[1 1 1] Server Set Active State
  ;;[0 0 0] Check to call the active component locally or over server
  (if (Variables|/Script/Engine.Actor|GetbReplicates (Components|GetOwner Active%20Component))
    (CallFunction|ServerActivate self Active%20Component Set)
    (else
      (Default|SetActive Active%20Component 0 Set))))

(event Input|KeyboardEvents|Escape
  (params (Key :type Key%20Structure :default "None"))
  ;[1 1 1] Quit the game when you press escape.
  (:Pressed
    (Game|QuitGame 0 "Quit" false)))

(fn ConstructionScript)

(fn TrytoSelect
  (params (Hit%20Result :type Hit%20Result%20Structure))
  (bind (_bblockinghit _binitialoverlap _time _distance _location _impactpoint _normal _impactnormal _physmat _hitactor _hitcomponent) (Collision|BreakHitResult Hit%20Result))
  (if _bblockinghit
    (Utilities|IsValid _hitactor
      (:Is%20Valid
        (for _array_element (Actor|GetComponentsByClass _hitactor "/Game/_Overseas/Development/Blueprints/Components/Utility/Comp_Select.Comp_Select_C")
          (bind _can_be_selected (Default|CanbeSelected _array_element _hitcomponent))
          (if _can_be_selected
            (Default|SelectPressed _array_element 0 self _location _hitcomponent)))))))

(fn TrytoHighlight
  (params (Hit%20Result :type Hit%20Result%20Structure))
  (bind (_bblockinghit _binitialoverlap _time _distance _location _impactpoint _normal _impactnormal _physmat _hitactor _hitcomponent) (Collision|BreakHitResult Hit%20Result))
  (if _bblockinghit
    (Utilities|IsValid _hitactor
      (:Is%20Valid
        (for _array_element (Actor|GetComponentsByClass _hitactor "/Game/_Overseas/Development/Blueprints/Components/Utility/Comp_Select.Comp_Select_C")
          (bind _can_be_selected (Default|CanbeSelected _array_element _hitcomponent))
          (if _can_be_selected
            (Default|SelectHighlight _array_element self _location (Math|Rotator|MakeRotfromZ _impactnormal) _hitcomponent)))))))

(fn UpdateHUDColor
  (params (Hit%20Result :type Hit%20Result%20Structure))
  (bind (_bblockinghit _binitialoverlap _time _distance _location _impactpoint _normal _impactnormal _physmat _hitactor _hitcomponent) (Collision|BreakHitResult Hit%20Result))
  (bind _returnvalue (Actor|GetComponentbyClass _hitactor "/Game/_Overseas/Development/Blueprints/Components/Utility/Comp_Select.Comp_Select_C"))
  (if _bblockinghit
    (Utilities|FlowControl|Sequence
      (:then_0
        (Utilities|FlowControl|Sequence
          (:then_0
            (Utilities|IsValid _returnvalue
              (:Is%20Valid
                (if (Utilities|Array|ContainsItem (Default|GetSelectableComponents _returnvalue) _hitcomponent)
                  (LocalVariables|SetColor%20To%20Set "(R=1.000000,G=0.000000,B=0.000000,A=1.000000)")
                  (else
                    (LocalVariables|SetUse%20Default true))))))
          (:then_1
            (bind _asbp_player_controller_main (Utilities|Casting|CastToBP_PlayerController_Main (Game|GetPlayerController 0) :!label _label))
            (Default|UpdateHUDColor _asbp_player_controller_main (LocalVariables|GetColor%20To%20Set) (LocalVariables|GetUse%20Default)))))
      (:then_1
        (goto _label_2 Reset)))
    (else
      (Utilities|FlowControl|DoOnce false :!label _label_2
        (:Completed
          (LocalVariables|SetUse%20Default true)
          (goto _label))))))