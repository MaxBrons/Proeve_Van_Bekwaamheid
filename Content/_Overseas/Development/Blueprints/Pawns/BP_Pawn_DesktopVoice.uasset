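; Desktop first-person player pawn with movement, mouse look, object selection and push-to-talk voice chat.
; Each tick a camera trace drives highlighting, HUD color and interaction hover, which shows prebuilt button widgets in viewport or world space.
; Holding Interact animates the button and triggers the component through a delay and gate.
; Space toggles speaking when nobody else talks, propagating a shared talking flag to all pawns with walkie-talkie sounds.
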(event Custom|Hide%20Character%20Mesh
  (Components|SkinnedMesh|HideBonebyName (Variables|Character|GetMesh) "head" "PBO_None"))

(event Custom|Setup%20Interaction%20Widgets
  (bind _interaction_settings (Variables|Default|GetInteraction%20Settings))
  (bind _value (Utilities|Map|Find _interaction_settings "NewEnumerator0"))
  (Utilities|IsValid _value
    (:Is%20Valid
      (bind _asda_interaction_settings_simple (Utilities|Casting|CastToDA_Interaction_Settings_Simple _value))
      (for _array_element (Variables|/Game/_Overseas/Development/DataAssets/Interaction/DA_Interaction_Settings_Simple.DA_Interaction_Settings_Simple_C|GetInteraction%20Settings _asda_interaction_settings_simple)
        (bind _returnvalue (UserInterface|CreateWidget (.interactionwidgetclasstoshow _array_element) 0 0 0))
        (Default|SetupWidget _returnvalue (Utilities|String|ToString(Name) (.buttoncontent (.buttonsettings _array_element))) (.buttonimage (.buttonsettings _array_element)) (.backgroundcolor (.buttonsettings _array_element)) (.bordersize (.buttonsettings _array_element)) (.bordercolor (.buttonsettings _array_element)))
        (Utilities|Map|Add (Variables|Internal|GetWidget%20List) (.interactioncode _array_element) _returnvalue)))))

(event Custom|Set%20to%20server
  (params (SomeoneIsTalking :type Boolean))
  (CallFunction|SettoAll SomeoneIsTalking))

(event Custom|Set%20to%20all
  (params (SomeoneIsTalking :type Boolean))
  (bind _outactors (Actor|GetAllActorsOfClass "/Game/_Overseas/Development/Blueprints/Pawns/BP_Pawn_Base.BP_Pawn_Base_C"))
  (for _array_element _outactors
    (bind _asbp_pawn_desktop_voice (Utilities|Casting|CastToBP_Pawn_DesktopVoice _array_element))
    (Variables|BP_Pawn_DesktopVoice_C|SetSomeoneIsTalking _asbp_pawn_desktop_voice SomeoneIsTalking))
  (if (Variables|VoiceChat|GetSomeoneIsTalking)
    (Audio|PlaySound2D "/Game/_Overseas/Development/Audio/Walkie_Talkie/WAV_TurnWalkieTalkieOn.WAV_TurnWalkieTalkieOn" 1.0 1.0 0.0 0 0)
    (else
      (Audio|PlaySound2D "/Game/_Overseas/Development/Audio/Walkie_Talkie/WAV_TurnWalkieTalkieOff.WAV_TurnWalkieTalkieOff" 1.0 1.0 0.0 0 0))))

(event EventBeginPlay
  ;[1 1 1] Attach the camera to the head of the player mesh and fade in
  (|CallParentFunction)
  (Transformation|AttachComponentToComponent (Variables|Default|GetSpringArm) (Variables|Character|GetMesh) "neck_01" "KeepWorld" "KeepWorld" "KeepWorld" true)
  (CameraFades|StartCameraFade :self (Game|GetPlayerCameraManager 0) :FromAlpha 1.0 :Duration 0.8)
  (CallFunction|HideCharacterMesh)
  (CallFunction|SetupInteractionWidgets)
  (bind _returnvalue (UserInterface|CreateWidget "/Game/_Overseas/Development/Blueprints/Widgets/HUD/Interaction/WB_Interaction_Initial.WB_Interaction_Initial_C" 0 0 self))
  (UserInterface|Viewport|AddtoViewport _returnvalue 99)
  (bind _output_get (Variables|Internal|SetInitial%20Interaction%20Widget _returnvalue))
  (Default|SetupWidget _output_get)
  (CallFunction|SetupInteractionWidget (Math|Transform|MakeTransform "0, 0, 0" "0, 0, 0" "0.200000,0.200000,0.200000") self true 1e+02 "(X=200.000000,Y=200.000000)"))

(event EventTick
  (params (DeltaSeconds :type Float%20%28single-precision%29))
  ;[1 1 1] Update the highlight, the hud color and the physics handle location;
  (|CallParentFunction DeltaSeconds)
  (Utilities|IsValid (Game|GetPlayerController 0)
    (:Is%20Valid
      (bind _hit_result (CallFunction|TraceMouse))
      (CallFunction|TrytoHighlight _hit_result)
      (CallFunction|UpdateHUDColor _hit_result)
      (CallFunction|TrytoHighlightInteract _hit_result))))

(event EventOnInteractionHover
  (params (Interaction%20Command :type Comp%20Interaction%20Object%20Reference))
  (bind _interaction_code (Default|GetUISettings Interaction%20Command))
  (bind _self self)
  (bind _widget_list (Variables|Internal|GetWidget%20List))
  (bind _hit_result (Variables|Default|GetHit%20Result))
  (bind (_value _returnvalue) (Utilities|Map|Find _widget_list _interaction_code))
  (bind (_bblockinghit _binitialoverlap _time _distance _location _impactpoint _normal _impactnormal _physmat _hitactor _hitcomponent) (Collision|BreakHitResult _hit_result))
  ;[1 1 1] Player Interaction is handles here. If a key is pressed the button animation will play and the current interaction component is called. If the player hovers over an interaction component, the right widget will be displayed on the screen.
  ;;[0 0 0] This event fires when a player comes close to an interaction component and aims at it. In this case an UI button is shown when the player comes close enough and aims at the interaction component.
  (Utilities|IsValid Interaction%20Command
    (:Is%20Valid
      (Utilities|FlowControl|DoOnce false :!label _label
        (:Completed
          (Utilities|FlowControl|Sequence
            (:then_0
              (if _returnvalue
                (CallFunction|HandleInteractionUI Interaction%20Command _value true)))
            (:then_1
              (goto _label_2 Reset))
            (:then_2
              (goto _label_3 Reset))))))
    (:Is%20Not%20Valid
      (Utilities|FlowControl|Sequence
        (:then_0
          (goto _label Reset))
        (:then_1
          (Utilities|FlowControl|DoOnce false :!label _label_2
            (:Completed
              (CallFunction|HandleInteractionUI 0 0 false))))
        (:then_2
          (Utilities|FlowControl|DoOnce false :!label _label_3
            (:Completed
              ;;[0 0 0] These events starts and stops the animation from the UI button. When the interaction is stopped it will also stop the execution flow of the interaction functionality that happends after the button is pressed for an amount N of seconds.
              (bind _previous_interaction_component (Variables|Default|GetPrevious%20Interaction%20Component)
                (:then
                  (Utilities|FlowControl|Sequence
                    (:then_0
                      (bind _initial_interaction_widget (Variables|Internal|GetInitial%20Interaction%20Widget)
                        (:then
                          (bind _current_button (Variables|/Game/_Overseas/Development/Blueprints/Widgets/HUD/Interaction/WB_Interaction_Initial.WB_Interaction_Initial_C|GetCurrent%20Button _initial_interaction_widget)
                            (:then
                              (bind _aswb_interaction_button (Utilities|Casting|CastToWB_Interaction_Button _current_button))
                              (Variables|Internal|SetCurrent%20Button _aswb_interaction_button))
                            (:else)))
                        (:else)))
                    (:then_1
                      (bind _current_button_2 (Variables|Internal|GetCurrent%20Button)
                        (:then
                          (Default|StopInteractionAnimation _current_button_2 (Variables|/Game/_Overseas/Development/Blueprints/Components/Core/Comp_Interaction.Comp_Interaction_C|GetInteraction%20Type _previous_interaction_component) (Variables|/Game/_Overseas/Development/Blueprints/Components/Core/Comp_Interaction.Comp_Interaction_C|GetInteraction%20Time _previous_interaction_component))
                          ;;[0 0 0] Handle the interaction when the player pressed the interaction button
                          (Utilities|FlowControl|Gate true) ; enters at Close
                        )
                        (:else)))))
                (:else)))))))))

(event Input|ActionEvents|InputActionInteract
  (params (Key :type Key%20Structure :default "None"))
  (bind _self self)
  (bind _hit_result (Variables|Default|GetHit%20Result))
  (bind (_bblockinghit _binitialoverlap _time _distance _location _impactpoint _normal _impactnormal _physmat _hitactor _hitcomponent) (Collision|BreakHitResult _hit_result))
  ;[1 1 1] Player Interaction is handles here. If a key is pressed the button animation will play and the current interaction component is called. If the player hovers over an interaction component, the right widget will be displayed on the screen.
  ;;[0 0 0] These events starts and stops the animation from the UI button. When the interaction is stopped it will also stop the execution flow of the interaction functionality that happends after the button is pressed for an amount N of seconds.
  (:Pressed
    (bind _previous_interaction_component (Variables|Default|GetPrevious%20Interaction%20Component)
      (:then
        (Utilities|FlowControl|Sequence
          (:then_0
            (bind _initial_interaction_widget (Variables|Internal|GetInitial%20Interaction%20Widget :!label _label)
              (:then
                (bind _current_button (Variables|/Game/_Overseas/Development/Blueprints/Widgets/HUD/Interaction/WB_Interaction_Initial.WB_Interaction_Initial_C|GetCurrent%20Button _initial_interaction_widget)
                  (:then
                    (bind _aswb_interaction_button (Utilities|Casting|CastToWB_Interaction_Button _current_button))
                    (Variables|Internal|SetCurrent%20Button _aswb_interaction_button))
                  (:else)))
              (:else)))
          (:then_1
            (bind _current_button_2 (Variables|Internal|GetCurrent%20Button)
              (:then
                (Default|StartInteractionAnimation _current_button_2 (Variables|/Game/_Overseas/Development/Blueprints/Components/Core/Comp_Interaction.Comp_Interaction_C|GetInteraction%20Type _previous_interaction_component) (Variables|/Game/_Overseas/Development/Blueprints/Components/Core/Comp_Interaction.Comp_Interaction_C|GetInteraction%20Time _previous_interaction_component))
                ;;[0 0 0] Handle the interaction when the player pressed the interaction button
                (Utilities|FlowControl|Sequence
                  (:then_0
                    (goto _label_2 Open))
                  (:then_1
                    (Utilities|FlowControl|RetriggerableDelay (Variables|/Game/_Overseas/Development/Blueprints/Components/Core/Comp_Interaction.Comp_Interaction_C|GetInteraction%20Time _previous_interaction_component))
                    (Utilities|FlowControl|Gate true :!label _label_2
                      (:Exit
                        (bind _previous_interaction_component_2 (Variables|Default|GetPrevious%20Interaction%20Component)
                          (:then
                            (Default|InteractionPressed _previous_interaction_component_2 _self _self _location _distance _hitcomponent))
                          (:else)))))))
              (:else)))))
      (:else)))
  (:Released
    (bind _previous_interaction_component_3 (Variables|Default|GetPrevious%20Interaction%20Component)
      (:then
        (Utilities|FlowControl|Sequence
          (:then_0
            (goto _label))
          (:then_1
            (bind _current_button_3 (Variables|Internal|GetCurrent%20Button)
              (:then
                (Default|StopInteractionAnimation _current_button_3 (Variables|/Game/_Overseas/Development/Blueprints/Components/Core/Comp_Interaction.Comp_Interaction_C|GetInteraction%20Type _previous_interaction_component_3) (Variables|/Game/_Overseas/Development/Blueprints/Components/Core/Comp_Interaction.Comp_Interaction_C|GetInteraction%20Time _previous_interaction_component_3))
                (goto _label_2 Close))
              (:else)))))
      (:else))))

(event Input|ActionEvents|InputActionFire
  (params (Key :type Key%20Structure :default "None"))
  ;[1 1 1] Try to select an object with a Comp_Select on it, when the fire button is pressed
  (:Pressed
    (bind _hit_result (CallFunction|TraceMouse))
    (CallFunction|TrytoSelect _hit_result)))

(event Input|AxisEvents|InputAxisMoveForward
  (params (AxisValue :type Float%20%28single-precision%29))
  ;[1 1 1] Player Movement
  ;;[1 1 1] Movement for moving forward or backwards
  (Pawn|Input|AddMovementInput (Math|Vector|GetForwardVector (Variables|Default|GetCapsuleComponent)) (* AxisValue (Variables|Settings|GetMovement%20Speed) (Utilities|Time|GetWorldDeltaSeconds)) false))

(event Input|AxisEvents|InputAxisMoveRight
  (params (AxisValue :type Float%20%28single-precision%29))
  ;[1 1 1] Player Movement
  ;;[1 1 1] Movement for moving right and left
  (Pawn|Input|AddMovementInput (Math|Vector|GetRightVector (Variables|Default|GetCapsuleComponent)) (* AxisValue (Variables|Settings|GetMovement%20Speed) (Utilities|Time|GetWorldDeltaSeconds)) false))

(event Input|AxisEvents|InputAxisTurn
  (params (AxisValue :type Float%20%28single-precision%29))
  ;[1 1 1] Player Movement
  ;;[1 1 1] Handle rotation. Only rotate when the right mousebutton is pressed
  (Pawn|Input|AddControllerYawInput (* AxisValue (.x (Variables|Settings|GetMouse%20Sensitivity)) (Utilities|Time|GetWorldDeltaSeconds))))

(event Input|AxisEvents|InputAxisLookUp
  (params (AxisValue :type Float%20%28single-precision%29))
  ;[1 1 1] Player Movement
  ;;[1 1 1] Handle rotation. Only rotate when the right mousebutton is pressed
  (Pawn|Input|AddControllerPitchInput (* AxisValue (.y (Variables|Settings|GetMouse%20Sensitivity)) (Utilities|Time|GetWorldDeltaSeconds))))

(event Input|KeyboardEvents|SpaceBar
  (params (Key :type Key%20Structure :default "None"))
  (:Pressed
    (if (not (Variables|VoiceChat|GetSomeoneIsTalking))
      (CallFunction|SettoServer true)
      (Development|ExecuteConsoleCommand "ToggleSpeaking 1" 0)
      (Variables|VoiceChat|SetIAmTalking true)))
  (:Released
    (if (Variables|VoiceChat|GetIAmTalking)
      (CallFunction|SettoServer false)
      (Variables|VoiceChat|SetIAmTalking false)
      (Development|ExecuteConsoleCommand "ToggleSpeaking 0" 0))))

(fn ConstructionScript
  (|CallParentFunction))

(fn TraceMouse
  (bind _out_hit (CallFunction|TracefromComponent (Variables|Default|GetCamera)))
  (return _out_hit))

(fn HandleInteractionUI
  (params (Current%20Interaction%20Component :type Comp%20Interaction%20Object%20Reference) (Widget%20To%20Show :type WB%20Interaction%20Button%20Object%20Reference) (Hit :type Boolean))
  (bind _returnvalue (Transformation|GetActorLocation))
  (bind (_interaction_code _ui_mode _ui_interaction_description) (Default|GetUISettings Current%20Interaction%20Component))
  (bind (_location _rotation) (Default|GetClosestWidgetLocation Current%20Interaction%20Component _returnvalue))
  ;[1 1 1] Show the widget on the viewport or in world space based on the UI mode from the interaction component.
  (if Hit
    (Utilities|IsValid Current%20Interaction%20Component
      (:Is%20Valid
        (switch Utilities|FlowControl|Switch|SwitchonE_UI_Mode _ui_mode
          (:NewEnumerator2
            (if (Utilities|Enum|NotEqual(Enum) (CallFunction|GetCurrentPlatform) "NewEnumerator2")
              (bind _initial_interaction_widget (Variables|Internal|GetInitial%20Interaction%20Widget :!label _label)
                (:then
                  (Default|SetupWidget _initial_interaction_widget Widget%20To%20Show _ui_interaction_description))
                (:else))
              (else
                ;[1 1 1] Get the location closest location where the widget should teleport, based on the player's location. After that teleport the widget and stop hiding the widget.
                (bind _interaction_widget (Variables|Default|GetInteraction%20Widget :!label _label_2)
                  (:then
                    (Transformation|SetActorLocationAndRotation _interaction_widget _location _rotation)
                    (Default|SetWidget _interaction_widget 0 Widget%20To%20Show)
                    (Rendering|SetActorHiddenInGame _interaction_widget false)
                    (Variables|Internal|SetCurrent%20Button Widget%20To%20Show))
                  (:else)))))
          (:NewEnumerator0
            (goto _label))
          (:NewEnumerator1
            (goto _label_2))))
      (:Is%20Not%20Valid
        ;[1 1 1] Stop showing the widget on the viewport or hide the widget in world space.
        (bind _previous_interaction_component (Variables|Default|GetPrevious%20Interaction%20Component :!label _label_3)
          (:then
            (switch Utilities|FlowControl|Switch|SwitchonE_UI_Mode (.UI%20Mode (Default|GetUISettings _previous_interaction_component))
              (:NewEnumerator2
                (if (Utilities|Enum|NotEqual(Enum) (CallFunction|GetCurrentPlatform) "NewEnumerator2")
                  (bind _initial_interaction_widget_2 (Variables|Internal|GetInitial%20Interaction%20Widget :!label _label_4)
                    (:then
                      (Default|SetupWidget _initial_interaction_widget_2))
                    (:else))
                  (else
                    (bind _interaction_widget_2 (Variables|Default|GetInteraction%20Widget :!label _label_5)
                      (:then
                        (Rendering|SetActorHiddenInGame _interaction_widget_2 true)
                        (Variables|Internal|SetCurrent%20Button 0))
                      (:else)))))
              (:NewEnumerator0
                (goto _label_4))
              (:NewEnumerator1
                (goto _label_5))))
          (:else))))
    (else
      (goto _label_3))))

(fn OnRepSomeoneIsTalking)