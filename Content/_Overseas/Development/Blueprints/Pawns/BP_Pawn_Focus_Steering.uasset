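; BP_Pawn_Focus_Steering is a pawn that lets the player turn a referenced steering wheel with the A and D keys.
; A Handle Input macro turns each held key into a repeating per-frame pulse using a gate and delta-time delay.
; Each pulse rotates the wheel's root by a speed-scaled offset, negated for A.
; CurrentDegrees, exposed through a getter, accumulates signed hold time in seconds rather than actual rotation.
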(event EventBeginPlay
  (|CallParentFunction) ; This node is disabled and will not be called.\nDrag off pins to build functionality.
)

(event Input|KeyboardEvents|D
  (params (Key :type Key%20Structure :default "None"))
  (:Pressed
    (Utilities|HandleInput :!label _label
      (:Exec
        (bind _steering_wheel (Variables|Settings|GetSteering%20Wheel)
          (:then
            (Transformation|AddLocalRotation (Variables|/Script/Engine.Actor|GetRootComponent _steering_wheel) (* (Variables|Settings|GetSteering%20Offset) (* (Variables|Settings|GetSteering%20Speed) (Utilities|Time|GetWorldDeltaSeconds))) false false)
            (Variables|Internal|SetCurrent%20Degrees (+ (Variables|Internal|GetCurrent%20Degrees) (Utilities|Time|GetWorldDeltaSeconds))))
          (:else)))))
  (:Released
    (goto _label Stop)))

(event Input|KeyboardEvents|A
  (params (Key :type Key%20Structure :default "None"))
  (:Pressed
    (Utilities|HandleInput :!label _label
      (:Exec
        (bind _steering_wheel (Variables|Settings|GetSteering%20Wheel)
          (:then
            (Transformation|AddLocalRotation (Variables|/Script/Engine.Actor|GetRootComponent _steering_wheel) (Class|KismetMathLibrary|NegateRotator (* (Variables|Settings|GetSteering%20Offset) (* (Variables|Settings|GetSteering%20Speed) (Utilities|Time|GetWorldDeltaSeconds)))) false false)
            (Variables|Internal|SetCurrent%20Degrees (- (Variables|Internal|GetCurrent%20Degrees) (Utilities|Time|GetWorldDeltaSeconds))))
          (:else)))))
  (:Released
    (goto _label Stop)))

(fn ConstructionScript
  (|CallParentFunction))

(fn GetCurrentDegrees
  (return (Variables|Internal|GetCurrent%20Degrees)))