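; Desktop player pawn with a first-person style camera and the ability to carry an ammunition crate.
; On begin play, the local player's spring arm attaches to the neck bone and the head is hidden to avoid camera clipping.
; Pickup passes through an RPC, RPS, RPM event chain, apparently client to server to multicast, gated on not already holding ammo.
; It spawns a collisionless crate on a mesh socket and flags the AnimBlueprint.
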(event Custom|RPC_PickUpChest
  (params (Target :type Actor%20Object%20Reference))
  (if (not (Variables|Default|GetHoldingAmmo))
    (CallFunction|RPSPickUpChest Target)))

(event Custom|RPM_PickUpChest
  (params (Target :type Actor%20Object%20Reference))
  (bind _returnvalue (Game|SpawnActorfromClass "/Script/Engine.StaticMeshActor" (Math|Transform|MakeTransform "0, 0, 0" "0, 0, 0" "1,1,1") "Undefined" 0 0))
  (Collision|SetCollisionEnabled (Variables|/Script/Engine.StaticMeshActor|GetStaticMeshComponent _returnvalue) "NoCollision")
  (Transformation|SetMobility _returnvalue "Movable")
  (Components|StaticMesh|SetStaticMesh (Variables|/Script/Engine.StaticMeshActor|GetStaticMeshComponent _returnvalue) "/Game/_Overseas/Art/Massi/Fbx/SM_Ammunition_Crate.SM_Ammunition_Crate")
  (Transformation|SetMobility (Variables|/Script/Engine.StaticMeshActor|GetStaticMeshComponent _returnvalue) "Movable")
  (Transformation|AttachComponentToComponent _returnvalue (Variables|Character|GetMesh) "AmmoChestSocket" "SnapToTarget" "SnapToTarget" "SnapToTarget" true)
  (bind _output_get (Variables|Default|SetHoldingAmmo true))
  (bind _asmixamo_base_skeleton_anim_blueprint (Utilities|Casting|CastToMixamo_Base_Skeleton_AnimBlueprint (Components|SkeletalMesh|GetAnimInstance (Variables|Character|GetMesh))))
  (Variables|/Game/_Overseas/Art/Selina/Models/Character_Animations/Mixamo_Base_Skeleton_AnimBlueprint.Mixamo_Base_Skeleton_AnimBlueprint_C|SetHasAmmoChest _asmixamo_base_skeleton_anim_blueprint _output_get))

(event Custom|RPS_PickUpChest
  (params (Target :type Actor%20Object%20Reference))
  (CallFunction|RPMPickUpChest Target))

(event EventBeginPlay
  ;[1 1 1] Attach the camera to the head of the player mesh and hide the head mesh so that the player doesn't clip through the head mesh with the camera.
  (|CallParentFunction)
  (if (== (Game|GetPlayerController 0) (Pawn|GetController))
    (Transformation|AttachComponentToComponent (Variables|Default|GetSpringArm) (Variables|Character|GetMesh) "neck_01" "KeepWorld" "KeepWorld" "KeepWorld" true)
    (CallFunction|HideCharacterHead)))

(fn ConstructionScript
  (|CallParentFunction))