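; Possessable pawn for pushing a torpedo trolley, entered when a player interacts with the trolley and the server switches their controller to it.
; Possession shows the headless body and enables collision, and the trolley attaches to its mesh.
; Forward input steers yaw, side input moves along the trolley's axis, and look input rotates the camera.
; Escape or reaching the torpedo tube returns the previous pawn, with the latter also snapping the trolley into place.
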(event Custom|Interaction%20Pressed
  (params (Pawn :type BP%20Pawn%20Base%20Object%20Reference) (Souce%20Actor :type Actor%20Object%20Reference) (Hit%20Location :type Vector) (Hit%20Distance :type Float%20%28single-precision%29) (Hit%20Component :type Actor%20Component%20Object%20Reference))
  (Networking|SwitchHasAuthority
    (:Authority
      (bind _asbp_player_controller_main (Utilities|Casting|CastToBP_PlayerController_Main (Pawn|GetController Pawn)))
      (Variables|Default|GetPrevious%20Pawn
        (:then)
        (:else
          (Variables|Default|SetPrevious%20Pawn Pawn)
          (EventDispatchers|BindEventtoOnPawnSwitched _asbp_player_controller_main (delegate Custom|Pawn%20Switched%20Initial))
          (Default|SwitchPawn _asbp_player_controller_main self))))))

(event Custom|Hide%20Character%20Head
  ;[1 1 1] Hide the head mesh.
  (Components|SkinnedMesh|HideBonebyName (Variables|Character|GetMesh) "head" "PBO_None"))

(event Custom|Pawn%20Switched
  (params (Player%20Controller :type BP%20Player%20Controller%20Main%20Object%20Reference) (New%20Pawn :type BP%20Pawn%20Base%20Object%20Reference))
  (bind _returnvalue (Transformation|GetActorTransform))
  (EventDispatchers|UnbindEventfromOnPawnSwitched Player%20Controller (delegate Custom|Pawn%20Switched))
  (bind _trolley (Variables|Default|GetTrolley)
    (:then
      (Transformation|DetachFromActor _trolley "KeepWorld" "KeepWorld" "KeepWorld")
      (Transformation|SetActorLocationAndRotation (Variables|Default|GetPrevious%20Pawn) (.location _returnvalue) (.rotation _returnvalue))
      (Variables|Default|SetPrevious%20Pawn 0))
    (:else)))

(event Custom|Torpedo%20Tube%20Reached
  (Utilities|FlowControl|DoOnce false
    (:Completed
      (bind _asbp_player_controller_main (Utilities|Casting|CastToBP_PlayerController_Main (Pawn|GetController)))
      (bind _previous_pawn (Variables|Default|GetPrevious%20Pawn)
        (:then
          (EventDispatchers|AssignOnPawnSwitched _asbp_player_controller_main (delegate Custom|On%20Pawn%20Switched_Event_0))
          (Default|SwitchPawn _asbp_player_controller_main _previous_pawn))
        (:else)))))

(event Custom|Pawn%20Switched%20Initial
  (params (Player%20Controller :type BP%20Player%20Controller%20Main%20Object%20Reference) (New%20Pawn :type BP%20Pawn%20Base%20Object%20Reference))
  (bind _scene (Variables|Default|GetScene))
  (bind _trolley (Variables|Default|GetTrolley))
  (bind _returnvalue (Transformation|GetWorldTransform _scene))
  (EventDispatchers|UnbindEventfromOnPawnSwitched Player%20Controller (delegate Custom|Pawn%20Switched%20Initial))
  (Transformation|SetActorLocationAndRotation _trolley (.location _returnvalue) (.rotation _returnvalue))
  (Transformation|AttachComponentToComponent _trolley (Variables|Character|GetMesh) "None" "KeepWorld" "KeepWorld" "KeepWorld" true))

(event Custom|Switch%20Back%20Pawn
  (bind _returnvalue (Pawn|GetController))
  (if (== (Pawn|GetController (CallFunction|GetMainPlayerPawn self)) _returnvalue)
    (bind _previous_pawn (Variables|Default|GetPrevious%20Pawn)
      (:then
        (bind _asbp_player_controller_main (Utilities|Casting|CastToBP_PlayerController_Main _returnvalue))
        (EventDispatchers|BindEventtoOnPawnSwitched _asbp_player_controller_main (delegate Custom|Pawn%20Switched))
        (Default|SwitchPawn _asbp_player_controller_main _previous_pawn))
      (:else))))

(event Custom|On%20Pawn%20Switched_Event_0
  (params (Player%20Controller :type BP%20Player%20Controller%20Main%20Object%20Reference) (New%20Pawn :type BP%20Pawn%20Base%20Object%20Reference))
  (bind _trolley (Variables|Default|GetTrolley))
  (bind _location_to_snap_to (Variables|/Game/_Overseas/Development/Blueprints/Assets/Ship/Trolley/BP_Torpedo_Trolley.BP_Torpedo_Trolley_C|GetLocation%20To%20Snap%20To _trolley))
  (bind _returnvalue (Transformation|GetActorTransform _location_to_snap_to))
  (EventDispatchers|UnbindEventfromOnPawnSwitched Player%20Controller (delegate Custom|On%20Pawn%20Switched_Event_0))
  (Default|SnaptoTorpedoTubeLocation _trolley (.location _returnvalue) (.rotation _returnvalue))
  (CallFunction|SwitchBackPawn)
  (Utilities|FlowControl|DoOnce false) ; enters at Reset
)

(event EventBeginPlay
  (|CallParentFunction)
  (CallFunction|HideCharacterHead)
  (bind _trolley (Variables|Default|GetTrolley)
    (:then
      (Rendering|SetVisibility (Variables|Character|GetMesh) false false)
      (Collision|SetCollisionEnabled (Variables|Default|GetCapsuleComponent) "NoCollision")
      (EventDispatchers|BindEventtoPressedInteraction (Variables|/Game/_Overseas/Development/Blueprints/Assets/Ship/Trolley/BP_Torpedo_Trolley.BP_Torpedo_Trolley_C|GetComp_Interaction _trolley) (delegate Custom|Interaction%20Pressed))
      (EventDispatchers|BindEventtoTorpedoTubeReached (Variables|Default|GetTrolley) (delegate Custom|Torpedo%20Tube%20Reached)))
    (:else)))

(event EventPossessed
  (params (NewController :type Controller%20Object%20Reference))
  ;[1 1 1] Set the mesh visible or not
  (|CallParentFunction NewController)
  (Rendering|SetVisibility (Variables|Character|GetMesh) true false)
  (Collision|SetCollisionEnabled (Variables|Default|GetCapsuleComponent) "QueryAndPhysics"))

(event EventUnpossessed
  (params (OldController :type Controller%20Object%20Reference))
  ;[1 1 1] Set the mesh visible or not
  (|CallParentFunction OldController)
  (Rendering|SetVisibility (Variables|Character|GetMesh) false false)
  (Collision|SetCollisionEnabled (Variables|Default|GetCapsuleComponent) "NoCollision"))

(event Input|AxisEvents|InputAxisMoveForward
  (params (AxisValue :type Float%20%28single-precision%29))
  ;[1 1 1] Player Movement
  ;;[1 1 1] Movement for moving forward or backwards
  (Pawn|Input|AddControllerYawInput (* AxisValue (Variables|Default|GetMovement%20Speed) (Utilities|Time|GetWorldDeltaSeconds))))

(event Input|AxisEvents|InputAxisMoveRight
  (params (AxisValue :type Float%20%28single-precision%29))
  ;[1 1 1] Player Movement
  ;;[1 1 1] Movement for moving right and left
  (bind _trolley (Variables|Default|GetTrolley)
    (:then
      (Pawn|Input|AddMovementInput (* (Math|Vector|GetForwardVector (Variables|/Script/Engine.Actor|GetRootComponent _trolley)) -1.0) (* AxisValue (Variables|Default|GetMovement%20Speed) (Utilities|Time|GetWorldDeltaSeconds)) false))
    (:else)))

(event Input|AxisEvents|InputAxisTurn
  (params (AxisValue :type Float%20%28single-precision%29))
  ;[1 1 1] Player Movement
  ;;[1 1 1] Turn the camera horizontally
  (Transformation|AddWorldRotation (Variables|Default|GetCamera) (Math|Rotator|MakeRotator 0.0 0.0 (* AxisValue (Variables|Default|GetMovement%20Speed) (Utilities|Time|GetWorldDeltaSeconds))) false false))

(event Input|AxisEvents|InputAxisLookUp
  (params (AxisValue :type Float%20%28single-precision%29))
  ;[1 1 1] Player Movement
  ;;[1 1 1] Turn the camera vertically
  (Transformation|AddLocalRotation (Variables|Default|GetCamera) (Math|Rotator|MakeRotator 0.0 (* (* AxisValue (Variables|Default|GetMovement%20Speed) (Utilities|Time|GetWorldDeltaSeconds)) -1.0) 0.0) false false))

(event Input|KeyboardEvents|Escape
  (params (Key :type Key%20Structure))
  (:Pressed
    (CallFunction|SwitchBackPawn)))

(fn ConstructionScript
  (|CallParentFunction))

(fn OnRepPreviousPawn)