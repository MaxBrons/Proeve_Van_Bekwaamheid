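; Desktop screen player pawn with first-person movement, mouse look, camera-trace selection, highlighting and interaction, plus task popup toggling.
; On BeginPlay the local player builds interaction widgets from a settings data asset, keyed by interaction code.
; Hovering shows them on the viewport or in world space by UI mode and platform, while a gated retriggerable delay handles hold interactions.
; It also socket-attaches a hammer and releases it to a slot through server-to-multicast events.
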(event Custom|Remove%20Widget%20From%20Viewport
  (params (HUD%20Name :type Name))
  (bind _hud_list (Variables|Internal|GetHUD%20List))
  (bind (_value _returnvalue) (Utilities|Map|Find _hud_list HUD%20Name))
  ;[1 1 1] Remove a widget based on a name.
  (if _returnvalue
    (Default|RemoveWidget _value)
    (Utilities|Map|Remove _hud_list HUD%20Name)))

(event Custom|Hide%20Character%20Head
  ;[1 1 1] Hide the head mesh.
  (Components|SkinnedMesh|HideBonebyName (Variables|Character|GetMesh) "head" "PBO_None"))

(event Custom|Multi_Release%20Hammer
  (params (Hammer%20Slot :type BP%20Hammer%20Slot%20Object%20Reference) (Hammer :type BP%20Hammer%20Object%20Reference))
  ;[1 1 1] Server and multi release the hammer.
  (Default|ReleaseHammer Hammer self)
  (Default|OccupySlot Hammer%20Slot Hammer))

(event Custom|Setup%20Interaction%20Widgets
  (bind _interaction_settings (Variables|Default|GetInteraction%20Settings))
  (bind _value (Utilities|Map|Find _interaction_settings "NewEnumerator0"))
  ;[1 1 1] Create the interaction widgets that are shown when you hover over an interactable object. These widgets can be shown in world space or on the viewport of the player.
  (Utilities|IsValid _value
    (:Is%20Valid
      (bind _asda_interaction_settings_simple (Utilities|Casting|CastToDA_Interaction_Settings_Simple _value))
      (for _array_element (Variables|/Game/_Overseas/Development/DataAssets/Interaction/DA_Interaction_Settings_Simple.DA_Interaction_Settings_Simple_C|GetInteraction%20Settings _asda_interaction_settings_simple)
        (if (Utilities|IsValidClass (.interactionwidgetclasstoshow _array_element))
          (bind _returnvalue (UserInterface|CreateWidget (.interactionwidgetclasstoshow _array_element) 0 0 0))
          (Default|SetupWidget _returnvalue (Utilities|String|ToString(Name) (.buttoncontent (.buttonsettings _array_element))) (.buttonimage (.buttonsettings _array_element)) (.holdingbarcolor (.buttonsettings _array_element)) (.backgroundcolor (.buttonsettings _array_element)) (.bordersize (.buttonsettings _array_element)) (.bordercolor (.buttonsettings _array_element)))
          (Utilities|Map|Add (Variables|Internal|GetWidget%20List) (.interactioncode _array_element) _returnvalue))))))

(event Custom|Add%20Widget%20To%20Viewport
  (params (HUD%20Name :type Name) (HUD%20Widget :type WB%20Widget%20Base%20Object%20Reference) (Layer :type Integer))
  (bind _hud_list (Variables|Internal|GetHUD%20List))
  ;[1 1 1] Add a widget to the viewport based on a name, so that ithe name counts as a sort of layer
  (Utilities|IsValid HUD%20Widget
    (:Is%20Valid
      (if (not (.ReturnValue (Utilities|Map|Find _hud_list HUD%20Name)))
        (UserInterface|Viewport|AddtoViewport HUD%20Widget Layer)
        (Utilities|Map|Add _hud_list HUD%20Name HUD%20Widget)))))

(event Custom|Grab%20Hammer
  (params (Hammer :type BP%20Hammer%20Object%20Reference))
  ;[1 1 1] Grab the hammer/ attach it to the hand of the pawn.
  (Utilities|IsValid Hammer
    (:Is%20Valid
      (Variables|Internal|GetCurrent%20Hammer
        (:then)
        (:else
          (bind _output_get (Variables|Internal|SetCurrent%20Hammer Hammer))
          (CallFunction|AttachActortoSocket _output_get "R_Object_Socket" true))))))

(event Custom|Release%20Hammer
  (params (Slot%20To%20Move%20To :type BP%20Hammer%20Slot%20Object%20Reference))
  ;[1 1 1] Release the hammer from the pawn's hand and replicate it to the other clients.
  (Utilities|IsValid Slot%20To%20Move%20To
    (:Is%20Valid
      (bind _current_hammer (Variables|Internal|GetCurrent%20Hammer)
        (:then
          (CallFunction|AttachActortoSocket _current_hammer "R_Object_Socket" false)
          (CallFunction|ServerReleaseHammer Slot%20To%20Move%20To _current_hammer)
          (Variables|Internal|SetCurrent%20Hammer 0))
        (:else)))))

(event Custom|Server_Release%20Hammer
  (params (Hammer%20Slot :type BP%20Hammer%20Slot%20Object%20Reference) (Hammer :type BP%20Hammer%20Object%20Reference))
  ;[1 1 1] Server and multi release the hammer.
  (CallFunction|MultiReleaseHammer Hammer%20Slot Hammer))

(event EventBeginPlay
  ;[1 1 1] Attach the camera to the head of the player mesh and fade in
  (|CallParentFunction)
  (if (== (Pawn|GetController) (Game|GetPlayerController 0))
    (CameraFades|StartCameraFade :self (Game|GetPlayerCameraManager 0) :FromAlpha 1.0 :Duration 0.8)
    (CallFunction|SetupInteractionWidgets)
    (bind _returnvalue (UserInterface|CreateWidget "/Game/_Overseas/Development/Blueprints/Widgets/HUD/Interaction/WB_Interaction_Initial.WB_Interaction_Initial_C" 0 0 self))
    (UserInterface|Viewport|AddtoViewport _returnvalue 99)
    (bind _output_get (Variables|Internal|SetInitial%20Interaction%20Widget _returnvalue))
    (Default|SetupWidget _output_get)
    (CallFunction|SetupInteractionWidget (Math|Transform|MakeTransform "0, 0, 0" "0, 0, 0" "0.100000,0.100000,0.100000") self true 1e+02 "(X=200.000000,Y=200.000000)" "/Game/_Overseas/Art/General/Materials/Widget3DPassThrough_NoDepth_Passthrough_OneSided.Widget3DPassThrough_NoDepth_Passthrough_OneSided")
    (bind _returnvalue_2 (Actor|GetActorOfClass "/Game/_Overseas/Development/Blueprints/Managers/BP_Manager_Popups.BP_Manager_Popups_C"))
    (Variables|Internal|SetPopup%20Manager _returnvalue_2)))

(event EventPossessed
  (params (NewController :type Controller%20Object%20Reference))
  ;[1 1 1] Set the collision of this pawn when the pawn gets possessed or unpossessed.
  (|CallParentFunction NewController)
  (Rendering|SetVisibility (Variables|Character|GetMesh) true false)
  (Collision|SetCollisionEnabled (Variables|Default|GetCapsuleComponent) "QueryAndPhysics"))

(event EventUnpossessed
  (params (OldController :type Controller%20Object%20Reference))
  ;[1 1 1] Set the collision of this pawn when the pawn gets possessed or unpossessed.
  (|CallParentFunction OldController)
  (Rendering|SetVisibility (Variables|Character|GetMesh) false false)
  (Collision|SetCollisionEnabled (Variables|Default|GetCapsuleComponent) "NoCollision"))

(event EventTick
  (params (DeltaSeconds :type Float%20%28single-precision%29))
  ;[1 1 1] Update the highlight, the hud color and the physics handle location;
  (|CallParentFunction DeltaSeconds)
  (if (== (Pawn|GetController) (Game|GetPlayerController 0))
    (bind _hit_result (CallFunction|TraceMouse))
    (CallFunction|TrytoHighlight _hit_result)
    (CallFunction|UpdateHUDColor _hit_result)
    (CallFunction|TrytoHighlightInteract _hit_result)))

(event EventOnInteractionHover
  (params (Interaction%20Command :type Comp%20Interaction%20Object%20Reference))
  (bind _interaction_code (Default|GetUISettings Interaction%20Command))
  (bind _widget_list (Variables|Internal|GetWidget%20List))
  (bind (_value _returnvalue) (Utilities|Map|Find _widget_list _interaction_code))
  ;[1 1 1] Player Interaction is handles here. If a key is pressed the button animation will play and the current interaction component is called. If the player hovers over an interaction component, the right widget will be displayed on the screen.
  ;;[0 0 0] This event fires when a player comes close to an interaction component and aims at it. In this case an UI button is shown when the player comes close enough and aims at the interaction component.
  (Utilities|IsValid Interaction%20Command
    (:Is%20Valid
      (Utilities|FlowControl|DoOnce false :!label _label
        (:Completed
          (Utilities|FlowControl|Sequence
            (:then_0
              (if _returnvalue
                (CallFunction|HandleInteractionUI Interaction%20Command _value true)))
            (:then_1
              (goto _label_2 Reset))
            (:then_2
              (goto _label_3 Reset))))))
    (:Is%20Not%20Valid
      (Utilities|FlowControl|Sequence
        (:then_0
          (goto _label Reset))
        (:then_1
          (Utilities|FlowControl|DoOnce false :!label _label_2
            (:Completed
              (CallFunction|HandleInteractionUI 0 0 false))))
        (:then_2
          (Utilities|FlowControl|DoOnce false :!label _label_3
            (:Completed
              ;;[0 0 0] These events starts and stops the animation from the UI button. When the interaction is stopped it will also stop the execution flow of the interaction functionality that happends after the button is pressed for an amount N of seconds.
              (bind _previous_interaction_component (Variables|Default|GetPrevious%20Interaction%20Component)
                (:then
                  (Utilities|FlowControl|Sequence
                    (:then_0
                      (bind _initial_interaction_widget (Variables|Internal|GetInitial%20Interaction%20Widget)
                        (:then
                          (bind _current_button (Variables|/Game/_Overseas/Development/Blueprints/Widgets/HUD/Interaction/WB_Interaction_Initial.WB_Interaction_Initial_C|GetCurrent%20Button _initial_interaction_widget)
                            (:then
                              (bind _aswb_interaction_button (Utilities|Casting|CastToWB_Interaction_Button _current_button))
                              (Variables|Internal|SetCurrent%20Button _aswb_interaction_button))
                            (:else)))
                        (:else)))
                    (:then_1
                      (bind _current_button_2 (Variables|Internal|GetCurrent%20Button)
                        (:then
                          (Default|StopInteractionAnimation _current_button_2 (Variables|/Game/_Overseas/Development/Blueprints/Components/Core/Comp_Interaction.Comp_Interaction_C|GetInteraction%20Type _previous_interaction_component) (Variables|/Game/_Overseas/Development/Blueprints/Components/Core/Comp_Interaction.Comp_Interaction_C|GetInteraction%20Time _previous_interaction_component))
                          ;;[0 0 0] Handle the interaction when the player pressed the interaction button
                          (Utilities|FlowControl|Gate true) ; enters at Close
                        )
                        (:else)))))
                (:else)))))))))

(event Input|ActionEvents|InputActionInteract
  (params (Key :type Key%20Structure :default "None"))
  ;[1 1 1] Player Interaction is handles here. If a key is pressed the button animation will play and the current interaction component is called. If the player hovers over an interaction component, the right widget will be displayed on the screen.
  ;;[0 0 0] These events starts and stops the animation from the UI button. When the interaction is stopped it will also stop the execution flow of the interaction functionality that happends after the button is pressed for an amount N of seconds.
  (:Pressed
    (bind _previous_interaction_component (Variables|Default|GetPrevious%20Interaction%20Component)
      (:then
        (Utilities|FlowControl|Sequence
          (:then_0
            (bind _initial_interaction_widget (Variables|Internal|GetInitial%20Interaction%20Widget :!label _label)
              (:then
                (bind _current_button (Variables|/Game/_Overseas/Development/Blueprints/Widgets/HUD/Interaction/WB_Interaction_Initial.WB_Interaction_Initial_C|GetCurrent%20Button _initial_interaction_widget)
                  (:then
                    (bind _aswb_interaction_button (Utilities|Casting|CastToWB_Interaction_Button _current_button))
                    (Variables|Internal|SetCurrent%20Button _aswb_interaction_button))
                  (:else)))
              (:else)))
          (:then_1
            (bind _current_button_2 (Variables|Internal|GetCurrent%20Button)
              (:then
                (Default|StartInteractionAnimation _current_button_2 (Variables|/Game/_Overseas/Development/Blueprints/Components/Core/Comp_Interaction.Comp_Interaction_C|GetInteraction%20Type _previous_interaction_component) (Variables|/Game/_Overseas/Development/Blueprints/Components/Core/Comp_Interaction.Comp_Interaction_C|GetInteraction%20Time _previous_interaction_component))
                (switch Utilities|FlowControl|Switch|SwitchonE_Button_Interaction_Type (Variables|/Game/_Overseas/Development/Blueprints/Components/Core/Comp_Interaction.Comp_Interaction_C|GetInteraction%20Type _previous_interaction_component)
                  (:NewEnumerator0
                    _)
                  (:NewEnumerator1
                    ;;[0 0 0] Handle the interaction when the player pressed the interaction button
                    (Utilities|FlowControl|Sequence
                      (:then_0
                        (goto _label_2 Open))
                      (:then_1
                        (Utilities|FlowControl|RetriggerableDelay (Variables|/Game/_Overseas/Development/Blueprints/Components/Core/Comp_Interaction.Comp_Interaction_C|GetInteraction%20Time _previous_interaction_component))
                        (Utilities|FlowControl|Gate true :!label _label_2
                          (:Exit
                            _))))))
                (Variables|Default|GetPrevious%20Interaction%20Component
                  (:then
                    (CallFunction|TrytoInteract (Variables|Default|GetHit%20Result)))
                  (:else)))
              (:else)))))
      (:else)))
  (:Released
    (bind _previous_interaction_component_2 (Variables|Default|GetPrevious%20Interaction%20Component)
      (:then
        (Utilities|FlowControl|Sequence
          (:then_0
            (goto _label))
          (:then_1
            (bind _current_button_3 (Variables|Internal|GetCurrent%20Button)
              (:then
                (Default|StopInteractionAnimation _current_button_3 (Variables|/Game/_Overseas/Development/Blueprints/Components/Core/Comp_Interaction.Comp_Interaction_C|GetInteraction%20Type _previous_interaction_component_2) (Variables|/Game/_Overseas/Development/Blueprints/Components/Core/Comp_Interaction.Comp_Interaction_C|GetInteraction%20Time _previous_interaction_component_2))
                (goto _label_2 Close))
              (:else)))))
      (:else))))

(event Input|ActionEvents|InputActionFire
  (params (Key :type Key%20Structure :default "None"))
  ;[1 1 1] Try to select an object with a Comp_Select on it, when the fire button is pressed
  (:Pressed
    (bind _hit_result (CallFunction|TraceMouse))
    (CallFunction|TrytoSelect _hit_result))
  (:Released
    (bind _current_select_component (Variables|Default|GetCurrent%20Select%20Component)
      (:then
        (CallFunction|ReleaseSelect _current_select_component))
      (:else))))

(event Input|ActionEvents|InputActionToggleTasks
  (params (Key :type Key%20Structure :default "None"))
  ;[1 1 1] Toggle the task window.
  (:Pressed
    (bind _popup_manager (Variables|Internal|GetPopup%20Manager)
      (:then
        (Utilities|FlowControl|FlipFlop
          (:A
            (Default|OpenTaskScreen _popup_manager))
          (:B
            (Default|CloseTaskScreen _popup_manager))))
      (:else))))

(event Input|AxisEvents|InputAxisMoveForward
  (params (AxisValue :type Float%20%28single-precision%29))
  ;[1 1 1] Player Movement
  ;;[1 1 1] Movement for moving forward or backwards
  (Pawn|Input|AddMovementInput (Math|Vector|GetForwardVector (Variables|Default|GetCapsuleComponent)) (* AxisValue (Variables|Settings|GetMovement%20Speed) (Utilities|Time|GetWorldDeltaSeconds)) false))

(event Input|AxisEvents|InputAxisMoveRight
  (params (AxisValue :type Float%20%28single-precision%29))
  ;[1 1 1] Player Movement
  ;;[1 1 1] Movement for moving right and left
  (Pawn|Input|AddMovementInput (Math|Vector|GetRightVector (Variables|Default|GetCapsuleComponent)) (* AxisValue (Variables|Settings|GetMovement%20Speed) (Utilities|Time|GetWorldDeltaSeconds)) false))

(event Input|AxisEvents|InputAxisTurn
  (params (AxisValue :type Float%20%28single-precision%29))
  ;[1 1 1] Player Movement
  ;;[1 1 1] Handle rotation. Only rotate when the right mousebutton is pressed
  (Pawn|Input|AddControllerYawInput (* AxisValue (.x (Variables|Settings|GetMouse%20Sensitivity)) (Utilities|Time|GetWorldDeltaSeconds))))

(event Input|AxisEvents|InputAxisLookUp
  (params (AxisValue :type Float%20%28single-precision%29))
  ;[1 1 1] Player Movement
  ;;[1 1 1] Handle rotation. Only rotate when the right mousebutton is pressed
  (Pawn|Input|AddControllerPitchInput (* AxisValue (.y (Variables|Settings|GetMouse%20Sensitivity)) (Utilities|Time|GetWorldDeltaSeconds))))

(fn ConstructionScript
  (|CallParentFunction))

(fn TraceMouse
  (bind _out_hit (CallFunction|TracefromComponent (Variables|Default|GetCamera)))
  (return _out_hit))

(fn HandleInteractionUI
  (params (Current%20Interaction%20Component :type Comp%20Interaction%20Object%20Reference) (Widget%20To%20Show :type WB%20Interaction%20Button%20Object%20Reference) (Hit :type Boolean))
  (bind _returnvalue (Transformation|GetActorLocation))
  (bind (_interaction_code _ui_mode _ui_interaction_description) (Default|GetUISettings Current%20Interaction%20Component))
  (bind (_location _rotation) (Default|GetClosestWidgetLocation Current%20Interaction%20Component _returnvalue))
  ;[1 1 1] Show the widget on the viewport or in world space based on the UI mode from the interaction component.
  (if Hit
    (Utilities|IsValid Current%20Interaction%20Component
      (:Is%20Valid
        (switch Utilities|FlowControl|Switch|SwitchonE_UI_Mode _ui_mode
          (:NewEnumerator2
            (if (Utilities|Enum|NotEqual(Enum) (CallFunction|GetCurrentPlatform) "NewEnumerator2")
              (bind _initial_interaction_widget (Variables|Internal|GetInitial%20Interaction%20Widget :!label _label)
                (:then
                  (Default|SetupWidget _initial_interaction_widget Widget%20To%20Show _ui_interaction_description))
                (:else))
              (else
                ;[1 1 1] Get the location closest location where the widget should teleport, based on the player's location. After that teleport the widget and stop hiding the widget.
                (bind _interaction_widget (Variables|Default|GetInteraction%20Widget :!label _label_2)
                  (:then
                    (Transformation|SetActorLocationAndRotation _interaction_widget _location _rotation)
                    (Default|SetWidget _interaction_widget 0 Widget%20To%20Show)
                    (Rendering|SetActorHiddenInGame _interaction_widget false)
                    (Variables|Internal|SetCurrent%20Button Widget%20To%20Show))
                  (:else)))))
          (:NewEnumerator0
            (goto _label))
          (:NewEnumerator1
            (goto _label_2))))
      (:Is%20Not%20Valid
        ;[1 1 1] Stop showing the widget on the viewport or hide the widget in world space.
        (bind _previous_interaction_component (Variables|Default|GetPrevious%20Interaction%20Component :!label _label_3)
          (:then
            (switch Utilities|FlowControl|Switch|SwitchonE_UI_Mode (.UI%20Mode (Default|GetUISettings _previous_interaction_component))
              (:NewEnumerator2
                (if (Utilities|Enum|NotEqual(Enum) (CallFunction|GetCurrentPlatform) "NewEnumerator2")
                  (bind _initial_interaction_widget_2 (Variables|Internal|GetInitial%20Interaction%20Widget :!label _label_4)
                    (:then
                      (Default|SetupWidget _initial_interaction_widget_2))
                    (:else))
                  (else
                    (bind _interaction_widget_2 (Variables|Default|GetInteraction%20Widget :!label _label_5)
                      (:then
                        (Rendering|SetActorHiddenInGame _interaction_widget_2 true)
                        (Variables|Internal|SetCurrent%20Button 0))
                      (:else)))))
              (:NewEnumerator0
                (goto _label_4))
              (:NewEnumerator1
                (goto _label_5))))
          (:else))))
    (else
      (goto _label_3))))