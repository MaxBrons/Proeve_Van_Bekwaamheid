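; BP_Pawn_Focus is a pawn for focus views, taking the viewpoint of a target actor and returning to the previous pawn on exit.
; Focusing stores the previous pawn, then has the main player controller transfer this pawn to the target's teleport location, optionally with a fade.
; Escape or a mapped interaction command switches back, firing the unfocus event once the controller validates.
; Key events are broadcast, and the pawn destroys itself shortly after being unpossessed.
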(event Custom|Focus%20Pawn
  (params (Current%20Pawn :type BP%20Pawn%20Base%20Object%20Reference) (Focus%20With%20Fade :type Boolean))
  (Utilities|IsValid Current%20Pawn
    (:Is%20Valid
      (Variables|Internal|GetPrevious%20Pawn
        (:then)
        (:else
          (Variables|Internal|SetPrevious%20Pawn Current%20Pawn)
          (bind _actor_to_focus_from (Variables|Settings|GetActor%20To%20Focus%20From)
            (:then
              (CallFunction|TeleportPawn (.Position (Default|GetTeleportLocation _actor_to_focus_from)) (.Rotation (Default|GetTeleportLocation _actor_to_focus_from)) Focus%20With%20Fade)
              (Default|CallOnPawnFocused self))
            (:else)))))))

(event Custom|Unfocus%20Pawn
  (params (New%20Pawn :type BP%20Pawn%20Base%20Object%20Reference))
  (bind _asbp_player_controller_main (Utilities|Casting|CastToBP_PlayerController_Main (Pawn|GetController)))
  (Default|SwitchPawn _asbp_player_controller_main New%20Pawn)
  (Utilities|WaitforObjecttoValidate (Pawn|GetController New%20Pawn) 0.05
    (:Is%20Valid
      (Variables|Internal|SetPrevious%20Pawn 0)
      (Default|CallOnPawnUnfocused self))))

(event Custom|Teleport%20Pawn
  (params (Location :type Vector) (Rotation :type Rotator) (With%20Fade :type Boolean))
  (bind _asbp_player_controller_main (Utilities|Casting|CastToBP_PlayerController_Main (Pawn|GetController)))
  (Default|TransferPawn _asbp_player_controller_main self Location Rotation With%20Fade))

(event EventBeginPlay
  (|CallParentFunction))

(event EventUnpossessed
  (params (OldController :type Controller%20Object%20Reference))
  (|CallParentFunction OldController)
  (Utilities|FlowControl|Delay 0.2)
  (Actor|DestroyActor))

(event EventPossessed
  (params (NewController :type Controller%20Object%20Reference))
  (|CallParentFunction NewController))

(event Input|KeyboardEvents|Escape
  (params (Key :type Key%20Structure :default "None"))
  (:Pressed
    (bind _previous_pawn (Variables|Internal|GetPrevious%20Pawn)
      (:then
        (CallFunction|UnfocusPawn _previous_pawn))
      (:else))))

(event Input|KeyboardEvents|AnyKey
  (params (Key :type Key%20Structure :default "None"))
  (bind _self self)
  (:Pressed
    (Default|CallOnKeyPressedEvent Key _self)
    (bind _interaction_command (CallFunction|GetValidInteractionSetting Key))
    (switch name _interaction_command
      (:Unfocus
        (bind _previous_pawn (Variables|Internal|GetPrevious%20Pawn)
          (:then
            (CallFunction|UnfocusPawn _previous_pawn))
          (:else)))))
  (:Released
    (Default|CallOnKeyReleasedEvent Key _self)))

(fn ConstructionScript
  (|CallParentFunction))

(fn SetupInteraction
  (params (Interaction%20Settings :type Array%20of%20Struct%20Interaction%20Platform%20Setting%20Key%20Structures))
  (return))