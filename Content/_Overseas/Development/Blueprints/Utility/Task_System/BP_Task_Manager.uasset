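; BP_Task_Manager is a utility that keeps a list of tasks and decides when one should start or stop.
; AddTask stores a valid task and requests a start if no current task exists or the new TaskID is lower.
; RemoveTask drops a task and requests a stop if it is the current one.
; StartTask and StopTask are empty, and nothing here assigns CurrentTask.
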(event Custom|Stop%20Task
  (params (Task%20To%20Stop :type BP%20Task%20Object%20Reference)))

(event Custom|Add%20Task
  (params (Task%20To%20Add :type BP%20Task%20Object%20Reference))
  (Utilities|IsValid Task%20To%20Add
    (:Is%20Valid
      (Utilities|Array|Add (Variables|Internal|GetTask%20List) Task%20To%20Add)
      (bind _current_task (Variables|Internal|GetCurrent%20Task)
        (:then
          (if (< (Variables|/Game/_Overseas/Development/Blueprints/Utility/Task_System/BP_Task.BP_Task_C|GetTask%20ID Task%20To%20Add) (Variables|/Game/_Overseas/Development/Blueprints/Utility/Task_System/BP_Task.BP_Task_C|GetTask%20ID _current_task))
            (CallFunction|StartTask Task%20To%20Add :!label _label)))
        (:else
          (goto _label))))))

(event Custom|Remove%20Task
  (params (Task%20To%20Remove :type BP%20Task%20Object%20Reference))
  (bind _current_task (Variables|Internal|GetCurrent%20Task))
  (Utilities|IsValid Task%20To%20Remove
    (:Is%20Valid
      (Utilities|Array|RemoveItem (Variables|Internal|GetTask%20List) Task%20To%20Remove)
      (if (== Task%20To%20Remove _current_task)
        (CallFunction|StopTask _current_task)))))

(event Custom|Start%20Task
  (params (Task%20To%20Start :type BP%20Task%20Object%20Reference)))

(event EventBeginPlay)

(fn ConstructionScript)