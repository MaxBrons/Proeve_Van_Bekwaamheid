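; BP_Task is a base task actor whose start, stop, pause and unpause events are meant to be overridden by specific tasks.
; On BeginPlay it finds the BP_Task_Manager with a matching TaskManagerID, destroying itself if either ID is negative or no manager is found.
; State changes broadcast through dispatchers for start, update and done.
; StopTask completes only when IsTaskDone passes, otherwise it pauses; the default check prints a warning and returns false.
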(event Custom|Update%20Task%20State
  (params (Task%20State :type E_Task_State%20Enum :default "NewEnumerator0"))
  ;[1 1 1] This event sets the task state variable and calls the On Task Update event.
  (bind _output_get (Variables|Internal|SetTask%20State Task%20State))
  (Default|CallOnTaskUpdate self (Variables|SettingsBase|GetTask%20Name) (Variables|SettingsBase|GetTask%20ID) _output_get))

(event Custom|Start%20Task
  (bind _task_state (Variables|Internal|GetTask%20State))
  ;[1 1 1] This event can only start if the task is not yet in progress. If the task is paused it will be unpaused, else it will call that is starts. This event should be overridden to implement your own functionality. Make sure to call this base event when overriding this event.
  (if (not (Utilities|Enum|Equal(Enum) _task_state "NewEnumerator2"))
    (if (Utilities|Enum|Equal(Enum) _task_state "NewEnumerator3")
      (CallFunction|UnpauseTask)
      (else
        (Default|CallOnTaskStart self (Variables|SettingsBase|GetTask%20Name) (Variables|SettingsBase|GetTask%20ID))
        (CallFunction|UpdateTaskState "NewEnumerator1")
        (CallFunction|UpdateTaskState "NewEnumerator2")))))

(event Custom|Unpause%20Task
  ;[1 1 1] This event updates the task state back to in progress. This event should be overridden to implement your own functionality. Make sure to call this base event when overriding this event.
  (CallFunction|UpdateTaskState "NewEnumerator2"))

(event Custom|Stop%20Task
  ;[1 1 1] This event checks if the task is done, if not, it will pause the task. If the task is done, it will call that it is done. This event should be overridden to implement your own functionality. Make sure to call this base event when overriding this event.
  (if (CallFunction|IsTaskDone)
    (Default|CallOnTaskDone self (Variables|SettingsBase|GetTask%20Name) (Variables|SettingsBase|GetTask%20ID))
    (CallFunction|UpdateTaskState "NewEnumerator4")
    (else
      (CallFunction|PauseTask))))

(event Custom|Pause%20Task
  ;[1 1 1] This event updates the task state to paused. This event should be overridden to implement your own functionality. Make sure to call this base event when overriding this event.
  (CallFunction|UpdateTaskState "NewEnumerator3"))

(event EventBeginPlay
  ;[1 1 1] Check if the Task ID or Task Manager ID are not less than 0 because that would invalidate then and they will be destroyed so they don't interfere with the rest of the system.
  (if (or (< (Variables|SettingsBase|GetTask%20ID) 0) (< (Variables|SettingsBase|GetTask%20Manager%20ID) 0))
    (Actor|DestroyActor :!label _label)
    (else
      (bind _task_manager (CallFunction|GetTaskManager))
      (Utilities|IsValid _task_manager
        (:Is%20Valid
          (Variables|Internal|SetTask%20Manager _task_manager))
        (:Is%20Not%20Valid
          (goto _label))))))

(fn ConstructionScript)

(fn IsTaskDone
  (Development|PrintString "Is Task Done function not yet implemented. Task will automaticaly stop.")
  (return false))

(fn GetTaskManager
  (bind _outactors (Actor|GetAllActorsOfClass "/Game/_Overseas/Development/Blueprints/Utility/Task_System/BP_Task_Manager.BP_Task_Manager_C"))
  (for _array_element _outactors
    (if (== (Variables|/Game/_Overseas/Development/Blueprints/Utility/Task_System/BP_Task_Manager.BP_Task_Manager_C|GetTask%20Manager%20ID _array_element) (Variables|SettingsBase|GetTask%20Manager%20ID))
      (return _array_element)))
  (return 0))