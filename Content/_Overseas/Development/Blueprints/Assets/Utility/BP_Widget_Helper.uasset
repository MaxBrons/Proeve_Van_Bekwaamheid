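; BP_Widget_Helper makes a world-space widget component selectable, relaying presses and hovers to its WB_Widget_Base as 2D coordinates.
; On BeginPlay it retries until the component is valid, then fits a handle and box to its draw size and pivot.
; Comp_Select events supply world hit locations, which a helper scene component converts into widget coordinates via its relative location.
; Hovering also caches WidgetInteraction's last hit when it strikes that widget.
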(event HighlightSelect(Comp_Select)
  (params (Source%20Actor :type Actor%20Object%20Reference) (Hit%20Location :type Vector :default "0, 0, 0") (Hit%20Rotation :type Rotator :default "0, 0, 0") (Hit%20Component :type Actor%20Component%20Object%20Reference))
  (bind _widgetinteraction (Variables|Default|GetWidgetInteraction))
  (bind _returnvalue (Class|WidgetInteractionComponent|GetLastHitResult _widgetinteraction))
  (Variables|Default|SetLast%20Hit%20Vector (CallFunction|Get2DCoordinatesfromHitLocation Hit%20Location))
  (Utilities|FlowControl|Sequence
    (:then_0
      (bind _aswb_widget_base (Utilities|Casting|CastToWB_Widget_Base (UserInterface|GetUserWidgetObject (Variables|Default|GetWidget%20Component))))
      (Default|HoveringOverWidget _aswb_widget_base (Variables|Default|GetLast%20Hit%20Vector)))
    (:then_1
      (if (== (.HitComponent (Collision|BreakHitResult _returnvalue)) (Variables|Default|GetWidget%20Component))
        (Variables|Default|SetHit%20Result _returnvalue)))))

(event PressedSelect(Comp_Select)
  (params (Pawn :type BP%20Pawn%20Base%20Object%20Reference) (Souce%20Actor :type Actor%20Object%20Reference) (Hit%20Location :type Vector :default "0, 0, 0") (Hit%20Component :type Actor%20Component%20Object%20Reference))
  (CallFunction|PressedSelection (CallFunction|Get2DCoordinatesfromHitLocation Hit%20Location) Souce%20Actor Hit%20Location Hit%20Component))

(event Custom|Fit%20To%20Widget
  (bind _widget_component (Variables|Default|GetWidget%20Component))
  (bind _box (Variables|Default|GetBox))
  (bind _returnvalue (Class|WidgetComponent|GetPivot _widget_component))
  (bind _returnvalue_2 (Class|WidgetComponent|GetDrawSize _widget_component))
  (bind _returnvalue_3 (/ (.y _returnvalue_2) 2.0))
  (bind _returnvalue_4 (/ (.x _returnvalue_2) 2.0))
  (Utilities|IsValid _widget_component :!label _label
    (:Is%20Valid
      (Transformation|SetRelativeLocation (Variables|Default|GetHandle) (Math|Vector|MakeVector 0.0 (* (.x _returnvalue) (.x _returnvalue_2)) (* (.y _returnvalue) (.y _returnvalue_2))) false false)
      (Components|Box|SetBoxExtent _box (Math|Vector|MakeVector 1e+01 _returnvalue_4 _returnvalue_3) true)
      (Transformation|SetRelativeLocation _box (Math|Vector|MakeVector 0.0 (* _returnvalue_4 -1.0) (* _returnvalue_3 -1.0)) false false))
    (:Is%20Not%20Valid
      (Utilities|FlowControl|Delay 0.05)
      (goto _label))))

(event Custom|Pressed%20Selection
  (params (Absolute%20Hit%20Coordinate :type Vector%202D%20Structure) (Source%20Actor :type Actor%20Object%20Reference) (Hit%20Location :type Vector) (Hit%20Component :type Actor%20Component%20Object%20Reference))
  (bind _aswb_widget_base (Utilities|Casting|CastToWB_Widget_Base (UserInterface|GetUserWidgetObject (Variables|Default|GetWidget%20Component))))
  (Default|PressedatLocation _aswb_widget_base Absolute%20Hit%20Coordinate Source%20Actor Hit%20Location Hit%20Component))

(event EventBeginPlay
  (CallFunction|FittoWidget))

(fn ConstructionScript)

(fn Get2DCoordinatesfromHitLocation
  (params (Hit%20Location :type Vector))
  (bind _helper_scene (Variables|Default|GetHelper%20Scene))
  (bind _relativelocation (Variables|/Script/Engine.SceneComponent|GetRelativeLocation _helper_scene))
  (Transformation|SetWorldLocation _helper_scene Hit%20Location false false)
  (return (Math|Vector2D|MakeVector2D (* (.y _relativelocation) -1.0) (* -1.0 (.z _relativelocation)))))