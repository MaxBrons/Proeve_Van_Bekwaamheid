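; Torpedo rack that players interact with to transfer a torpedo, requiring two players in multiplayer or one when solo.
; Interaction switches the player's input to the rack and updates an interacting-player count through server-to-multicast events.
; At the threshold, a DoOnce-gated multicast checks LoadTorpedoManager, fades the interacting player's camera around the transfer, then unfocuses.
; Escape also unfocuses and decrements the count, while failed transfer checks reset the gate.
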(event PressedInteraction(Comp_Interaction)
  (params (Pawn :type BP%20Pawn%20Base%20Object%20Reference) (Souce%20Actor :type Actor%20Object%20Reference) (Hit%20Location :type Vector :default "0, 0, 0") (Hit%20Distance :type Float%20%28single-precision%29) (Hit%20Component :type Actor%20Component%20Object%20Reference))
  ;[1 1 1] Check if it is allowed to interact with the object and switch the input to this object.
  (if (not (Utilities|Array|ContainsItem (Variables|Internal|GetInteracted%20Actors) Pawn))
    (Utilities|Array|Add (Variables|Internal|GetInteracted%20Actors) Pawn)
    (bind _asbp_player_controller_main (Utilities|Casting|CastToBP_PlayerController_Main (Pawn|GetController Pawn)))
    (Default|SwitchInput _asbp_player_controller_main Pawn self true)
    (Networking|SwitchHasAuthority
      (:Authority
        ;[1 1 1] Increase the index for checking how many players are currently interacting with this obejct and spawn in a torpedo if at least one player is interacting, if mulitplayer there have to be two players minimum.
        (CallFunction|IncreasePlayerAmount true)
        (bind _asbp_game_mode_main (Utilities|Casting|CastToBP_GameMode_Main (Game|GetGameMode)))
        (if (>= (Variables|Internal|GetPlayers%20Interacted) (Math|Integer|SelectInt 1 2 (<= (Utilities|Map|Length (Variables|/Game/_Overseas/Development/Game/BP_GameMode_Main.BP_GameMode_Main_C|GetPlayer%20List _asbp_game_mode_main)) 1)))
          (Utilities|FlowControl|DoOnce false
            (:Completed
              (CallFunction|ServerTransferTorpedo))))))))

(event Custom|MultiTransfer%20Torpedo
  ;[1 1 1] Do a fade in and out. In between the fade, spawn in the new torpedo and place it in on the location that is set in the editor.
  (if (Utilities|Array|ContainsItem (Variables|Internal|GetInteracted%20Actors) (Game|Player|GetPlayerPawn 0))
    (bind _load_torpedo_manager (Variables|Settings|GetLoad%20Torpedo%20Manager)
      (:then
        (if (Default|AllowedtoLoadTorpedoin _load_torpedo_manager)
          (CameraFades|StartCameraFade :self (Game|GetPlayerCameraManager 0) :ToAlpha 1.0 :Duration 1.0 :bHoldWhenFinished true)
          (Utilities|FlowControl|Delay 1.5)
          (Default|TransferTorpedo _load_torpedo_manager true)
          (CameraFades|StartCameraFade :self (Game|GetPlayerCameraManager 0) :FromAlpha 1.0 :Duration 1.0)
          (CallFunction|Unfocus)
          (else
            (CallFunction|Reset :!label _label))))
      (:else
        (goto _label)))
    (else
      (goto _label))))

(event Custom|Server_Transfer%20Torpedo
  ;[1 1 1] Do a fade in and out. In between the fade, spawn in the new torpedo and place it in on the location that is set in the editor.
  (CallFunction|MultiTransferTorpedo))

(event Custom|Multi_Increase%20Player%20Amount
  (params (Increase :type Boolean))
  (bind _players_interacted (Variables|Internal|GetPlayers%20Interacted))
  (if Increase
    (Math|Integer|IncrementInt _players_interacted)
    (else
      (Math|Integer|DecrementInt _players_interacted))))

(event Custom|Unfocus
  (bind _self self)
  (bind _player_pawn (CallFunction|GetMainPlayerPawn _self))
  ;[1 1 1] Unfocus from the object and decrease the index for checking how many players are currently interacting
  (bind _returnvalue (Utilities|Array|RemoveItem (Variables|Internal|GetInteracted%20Actors) _player_pawn))
  (if _returnvalue
    (bind _asbp_player_controller_main (Utilities|Casting|CastToBP_PlayerController_Main (Pawn|GetController _player_pawn)))
    (Default|SwitchInput _asbp_player_controller_main _player_pawn self false)
    (CallFunction|IncreasePlayerAmount false)))

(event Custom|Reset
  ;[1 1 1] Increase the index for checking how many players are currently interacting with this obejct and spawn in a torpedo if at least one player is interacting, if mulitplayer there have to be two players minimum.
  (Utilities|FlowControl|DoOnce false) ; enters at Reset
)

(event Custom|Increase%20Player%20Amount
  (params (Increase :type Boolean))
  (CallFunction|ServerIncreasePlayerAmount Increase))

(event Custom|Server_Increase%20Player%20Amount
  (params (Increase :type Boolean))
  (CallFunction|MultiIncreasePlayerAmount Increase))

(event Input|KeyboardEvents|Escape
  (params (Key :type Key%20Structure :default "None"))
  (bind _self self)
  (bind _player_pawn (CallFunction|GetMainPlayerPawn _self))
  ;[1 1 1] Unfocus from the object and decrease the index for checking how many players are currently interacting
  (:Pressed
    (bind _returnvalue (Utilities|Array|RemoveItem (Variables|Internal|GetInteracted%20Actors) _player_pawn))
    (if _returnvalue
      (bind _asbp_player_controller_main (Utilities|Casting|CastToBP_PlayerController_Main (Pawn|GetController _player_pawn)))
      (Default|SwitchInput _asbp_player_controller_main _player_pawn self false)
      (CallFunction|IncreasePlayerAmount false))))

(fn ConstructionScript)

(fn OnRepPlayersInteracted)