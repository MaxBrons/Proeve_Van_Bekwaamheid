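; Launch button that fires a torpedo through the level's BP_Manager_LaunchTorpedo when pressed.
; On BeginPlay it finds the manager, binds to its launch-keys-turned event and starts disabled, so its interaction is enabled only while all keys are turned.
; A press checks that the manager is valid and can fire, then launches with a boolean mapped from the torpedo room direction.
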(event PressedInteraction(Comp_Interaction)
  (params (Pawn :type BP%20Pawn%20Base%20Object%20Reference) (Souce%20Actor :type Actor%20Object%20Reference) (Hit%20Location :type Vector :default "0, 0, 0") (Hit%20Distance :type Float%20%28single-precision%29) (Hit%20Component :type Actor%20Component%20Object%20Reference))
  (bind _launch_torpedo_manager (Variables|Internal|GetLaunch%20Torpedo%20Manager)
    (:then
      (if (Default|CanFireTorpedo _launch_torpedo_manager)
        (Default|LaunchTorpedo _launch_torpedo_manager (Utilities|Select :Index (Variables|Settings|GetTorpedo%20Room%20Direction) :NewEnumerator0 false :NewEnumerator1 true :NewEnumerator2 false :NewEnumerator3 true))))
    (:else)))

(event Custom|On%20Keys%20Turned
  (params (All%20Turned :type Boolean))
  (Default|SetInteractionEnabled (Variables|Default|GetComp_Interaction) All%20Turned))

(event EventBeginPlay
  (bind _returnvalue (Actor|GetActorOfClass "/Game/_Overseas/Development/Blueprints/Managers/BP_Manager_LaunchTorpedo.BP_Manager_LaunchTorpedo_C"))
  (bind _output_get (Variables|Internal|SetLaunch%20Torpedo%20Manager _returnvalue))
  (EventDispatchers|BindEventtoLaunchKeysTurned _output_get (delegate Custom|On%20Keys%20Turned))
  (CallFunction|OnKeysTurned false))

(fn ConstructionScript)