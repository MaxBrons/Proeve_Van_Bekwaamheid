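; BP_Torpedo_Launch_Lamp is an indicator lamp that shows whether all torpedo launch keys are turned.
; On BeginPlay it creates a dynamic ready-lamp material, and on authority only binds to the key-turn event of BP_Manager_LaunchTorpedo.
; Key changes pass through server and multi events, which switch the material's "Torpedo Ready Licht" scalar on or off.
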(event Custom|Multi_Keys%20Turned
  (params (All%20Turned :type Boolean))
  (Rendering|Material|SetScalarParameterValue (Variables|Internal|GetLamp%20Material) "Torpedo Ready Licht" (select All%20Turned 1.0 0.0) :!class /Script/Engine.MaterialInstanceDynamic))

(event Custom|Keys%20Turned
  (params (All%20Turned :type Boolean))
  (CallFunction|ServerKeysTurned All%20Turned))

(event Custom|Server_Keys%20Turned
  (params (All%20Turned :type Boolean))
  (CallFunction|MultiKeysTurned All%20Turned))

(event EventBeginPlay
  (bind _returnvalue (Rendering|Material|CreateDynamicMaterialInstance (Variables|Default|GetStaticMesh) 0 "/Game/_Overseas/Art/Saskia/Materials/M_TorpedoReadyKnop.M_TorpedoReadyKnop" "ReadyLamp" :!class /Script/Engine.PrimitiveComponent))
  (Variables|Internal|SetLamp%20Material _returnvalue)
  (Networking|SwitchHasAuthority
    (:Authority
      (bind _returnvalue_2 (Actor|GetActorOfClass "/Game/_Overseas/Development/Blueprints/Managers/BP_Manager_LaunchTorpedo.BP_Manager_LaunchTorpedo_C"))
      (bind _output_get (Variables|Default|SetTorpedo%20Launch%20Manager _returnvalue_2))
      (Utilities|IsValid _output_get
        (:Is%20Valid
          (EventDispatchers|BindEventtoLaunchKeysTurned _output_get (delegate Custom|Keys%20Turned)))))))

(fn ConstructionScript)