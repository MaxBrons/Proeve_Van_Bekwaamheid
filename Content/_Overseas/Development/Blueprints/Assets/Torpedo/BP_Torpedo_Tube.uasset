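; A torpedo tube Blueprint that tracks whether it is occupied and shows or hides its Torpedo component to match, starting empty on BeginPlay.
; OccupyTorpedo calls a server event and sets Occupied on the caller, and the server event relays to a multicast that toggles the torpedo's visibility.
; IsOccupied exposes the flag, while its OnRep handler is empty, so visuals rely on the multicast.
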(event Custom|Multi_Occupy%20Torpedo
  (params (Occupy :type Boolean))
  (Development|SetHiddeninGame (Variables|Default|GetTorpedo) (not Occupy) false))

(event Custom|Occupy%20Torpedo
  (params (Occupy :type Boolean))
  (CallFunction|ServerOccupyTorpedo Occupy)
  (Variables|Internal|SetOccupied Occupy))

(event Custom|Server_Occupy%20Torpedo
  (params (Occupy :type Boolean))
  (CallFunction|MultiOccupyTorpedo Occupy))

(event EventBeginPlay
  (CallFunction|OccupyTorpedo false))

(fn ConstructionScript)

(fn IsOccupied
  (return (Variables|Internal|GetOccupied)))

(fn OnRepOccupied)