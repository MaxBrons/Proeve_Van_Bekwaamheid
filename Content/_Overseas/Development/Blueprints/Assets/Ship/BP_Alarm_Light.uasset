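; BP_Alarm_Light is a ship emergency lamp that runs a light and sound alarm when StartAlarm is called.
; StartAlarm plays the audio and loops an Actor Sequence until the sound finishes.
; It then stops the sequence and, after a short delay, zeroes the spotlight intensity and the lamp material's NoodLamp parameter.
; The construction script creates that dynamic material instance on the static mesh.
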(event Custom|Start%20Alarm
  (bind _audio (Variables|Default|GetAudio))
  (Audio|Components|Audio|Play _audio 0.0)
  (Class|MovieSceneSequencePlayer|PlayLooping (Variables|/Script/ActorSequence.ActorSequenceComponent|GetSequencePlayer (Variables|Default|GetActorSequence)) -1)
  (EventDispatchers|BindEventtoOnAudioFinished _audio (delegate Custom|Audio%20Finished)))

(event Custom|Audio%20Finished
  (Sequencer|Player|Stop (Variables|/Script/ActorSequence.ActorSequenceComponent|GetSequencePlayer (Variables|Default|GetActorSequence)) :!class /Script/MovieScene.MovieSceneSequencePlayer)
  (Utilities|FlowControl|Delay 0.2)
  (Rendering|Components|Light|SetIntensity (Variables|Default|GetSpotLight) 0.0)
  (Rendering|Material|SetScalarParameterValue (Variables|Default|GetEmergency%20Lamp%20Material) "NoodLamp" 0.0 :!class /Script/Engine.MaterialInstanceDynamic))

(fn ConstructionScript
  (bind _returnvalue (Rendering|Material|CreateDynamicMaterialInstance (Variables|Default|GetStaticMesh) 0 "/Game/_Overseas/Art/Saskia/Materials/Lampjes/Control_Noodlamp.Control_Noodlamp" "None" :!class /Script/Engine.PrimitiveComponent))
  (Variables|Default|SetEmergency%20Lamp%20Material _returnvalue))