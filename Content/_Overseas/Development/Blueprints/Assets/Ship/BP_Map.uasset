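; Ship status map with a lamp for each compartment, colored to show it as working, needing investigation or broken.
; On BeginPlay it gives each lamp mesh a dynamic material, stores it in a map and requests the Working state.
; SetLampState finds lamps by component object name, broadcasts the update and recolors them, but only while the active component is on.
; Changes to that component's active state switch every lamp's light value on or off.
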(event ActiveStateChanged(Comp_Active)
  (params (Pawn :type BP%20Pawn%20Base%20Object%20Reference) (Comp%20Active :type Comp%20Active%20Object%20Reference) (New%20Active :type Boolean))
  (bind _values (Utilities|Map|Values (Variables|Internal|GetLights)))
  (for _array_element _values
    (Rendering|Material|SetScalarParameterValue _array_element (Variables|Internal|GetLamp%20Light%20value%20Paramater%20Name) (select New%20Active 1e+02 0.0) :!class /Script/Engine.MaterialInstanceDynamic)))

(event Custom|Set%20Lamp%20State
  (params (Name :type Name) (State :type E_Map_Light_State%20Enum :default "NewEnumerator0"))
  (if (Default|IsActive (Variables|Default|GetComp_Active))
    (bind _lamp (CallFunction|GetLampbyName Name))
    (Utilities|IsValid _lamp
      (:Is%20Valid
        (Default|CallMapUpdated Name State self)
        (Rendering|Material|SetVectorParameterValue (.Value (Utilities|Map|Find (Variables|Internal|GetLights) _lamp)) (Variables|Internal|GetLamp%20Color%20Paramater%20Name) (Utilities|Select :Index State :NewEnumerator0 (Variables|Internal|GetWorking%20Color) :NewEnumerator1 (Variables|Internal|GetInvestigate) :NewEnumerator2 (Variables|Internal|GetBroken%20Color)) :!class /Script/Engine.MaterialInstanceDynamic)))))

(event EventBeginPlay
  (for _array_element (Utilities|Array|MakeArray (Variables|Default|GetCommando%20Centrale) (Variables|Default|GetMunition) (Variables|Default|GetTorpedo%20Right) (Variables|Default|GetTorpedo%20Left) (Variables|Default|GetBrug) (Variables|Default|GetCommunications) (Variables|Default|GetCannon) (Variables|Default|GetElectrical) (Variables|Default|GetEngine))
    (bind _returnvalue (Rendering|Material|CreateDynamicMaterialInstance _array_element 0 (Rendering|Material|GetMaterial _array_element 0) "None" :!class /Script/Engine.PrimitiveComponent))
    (Utilities|Map|Add (Variables|Internal|GetLights) _array_element _returnvalue)
    (CallFunction|SetLampState (Utilities|String|StringToName (Utilities|GetObjectName _array_element)) "NewEnumerator0"))
  (Default|SetActive (Variables|Default|GetComp_Active) 0 true))

(fn ConstructionScript)

(fn GetLampbyName
  (params (Name :type Name))
  (bind _keys (Utilities|Map|Keys (Variables|Internal|GetLights)))
  (for _array_element _keys
    (if (Utilities|Name|Equal(Name) Name (Utilities|String|StringToName (Utilities|GetObjectName _array_element)))
      (return _array_element))))