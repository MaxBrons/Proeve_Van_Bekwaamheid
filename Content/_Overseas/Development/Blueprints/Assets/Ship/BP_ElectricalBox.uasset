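; BP_ElectricalBox is a ship electrical box with ten switch meshes that the player flips by interacting.
; Pressing a switch changes its pitch and broadcasts the GetAllSwitchesOn result, which currently always returns false because its loop is unconnected.
; Active-state changes toggle interaction: active disables it and zeroes switch pitches, while inactive enables it and randomizes them.
; The Switches map starts all true and is never updated on press.
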(event PressedInteraction(Comp_Interaction)
  (params (Pawn :type BP%20Pawn%20Base%20Object%20Reference) (Souce%20Actor :type Actor%20Object%20Reference) (Hit%20Location :type Vector :default "0, 0, 0") (Hit%20Distance :type Float%20%28single-precision%29) (Hit%20Component :type Actor%20Component%20Object%20Reference))
  (bind _asstatic_mesh_component (Utilities|Casting|CastToStaticMeshComponent Hit%20Component))
  (bind _keys (Utilities|Map|Keys (Variables|Internal|GetSwitches)))
  (Utilities|IsValid (Utilities|Array|Get(acopy) _keys (Utilities|Array|FindItem _keys _asstatic_mesh_component))
    (:Is%20Valid
      (Transformation|SetRelativeRotation (Utilities|Array|Get(acopy) _keys (Utilities|Array|FindItem _keys _asstatic_mesh_component)) (Math|Rotator|MakeRotator (.roll (Variables|/Script/Engine.SceneComponent|GetRelativeRotation (Utilities|Array|Get(acopy) _keys (Utilities|Array|FindItem _keys _asstatic_mesh_component)))) (select (== (.pitch (Variables|/Script/Engine.SceneComponent|GetRelativeRotation (Utilities|Array|Get(acopy) _keys (Utilities|Array|FindItem _keys _asstatic_mesh_component)))) 0.0) -1.8e+02 179.0) (.yaw (Variables|/Script/Engine.SceneComponent|GetRelativeRotation (Utilities|Array|Get(acopy) _keys (Utilities|Array|FindItem _keys _asstatic_mesh_component))))) false true)
      (bind _all_switches_on (CallFunction|GetAllSwitcheson))
      (Default|CallOnSwitchesUpdated _all_switches_on))))

(event ActiveStateChanged(Comp_Active)
  (params (Pawn :type BP%20Pawn%20Base%20Object%20Reference) (Comp%20Active :type Comp%20Active%20Object%20Reference) (New%20Active :type Boolean))
  (Default|SetInteractionEnabled (Variables|Default|GetComp_Interaction) (not New%20Active))
  (for _array_element 0
    (Transformation|SetRelativeRotation _array_element (Math|Rotator|MakeRotator (.roll (Variables|/Script/Engine.SceneComponent|GetRelativeRotation _array_element)) (CallFunction|GetRandomRotation New%20Active) (.yaw (Variables|/Script/Engine.SceneComponent|GetRelativeRotation _array_element))) false true)))

(event EventBeginPlay
  (Variables|Internal|SetSwitches (Utilities|Map|MakeMap (Variables|Default|GetStaticMesh1) true (Variables|Default|GetStaticMesh2) true (Variables|Default|GetStaticMesh3) true (Variables|Default|GetStaticMesh4) true (Variables|Default|GetStaticMesh5) true (Variables|Default|GetStaticMesh6) true (Variables|Default|GetStaticMesh7) true (Variables|Default|GetStaticMesh8) true (Variables|Default|GetStaticMesh9) true (Variables|Default|GetStaticMesh10) true)))

(fn ConstructionScript)

(fn GetAllSwitcheson
  (return false))

(fn GetRandomRotation
  (params (Index :type Boolean))
  (return (select Index 0.0 (select (Math|Random|RandomBool) -1.8e+02 0.0))))