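; Torpedo loading hole on a ship, with a hinged hatch (Klep) that players toggle open and closed by interaction.
; A DoOnce-guarded Delay loop eases the hatch rotation with RInterpTo, then sets Opened and calls the door opened or closed event, alongside matching audio.
; Active-state changes show or hide the torpedo, update Occupied, announce it and play a loading sound when filled.
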(event PressedInteraction(Comp_Interaction)
  (params (Pawn :type BP%20Pawn%20Base%20Object%20Reference) (Souce%20Actor :type Actor%20Object%20Reference) (Hit%20Location :type Vector :default "0, 0, 0") (Hit%20Distance :type Float%20%28single-precision%29) (Hit%20Component :type Actor%20Component%20Object%20Reference))
  (bind _door_open_sound (Variables|Settings|GetDoor%20Open%20Sound))
  (bind _audio (Variables|Default|GetAudio))
  (bind _audio_2 (Variables|Default|GetAudio))
  (Utilities|FlowControl|DoOnce false :!label _label
    (:Completed
      (Utilities|FlowControl|Sequence
        (:then_0
          (bind _isa (Utilities|FlowControl|FlipFlop)
            (:A
              _)
            (:B
              _))
          (Transformation|SetRelativeRotation (Variables|Default|GetKlep) (Math|Interpolation|RInterpTo (Variables|/Script/Engine.SceneComponent|GetRelativeRotation (Variables|Default|GetKlep)) (Math|Rotator|SelectRotator (Math|Rotator|MakeRotator 0.0 0.0 (.yaw (Variables|Internal|GetOpen%20Rotation))) (Variables|Internal|GetStart%20Rotation) _isa) (Utilities|Time|GetWorldDeltaSeconds) 5.0) false false :!label _label_2)
          (if (Math|Rotator|Equal(Rotator) (Math|Interpolation|RInterpTo (Variables|/Script/Engine.SceneComponent|GetRelativeRotation (Variables|Default|GetKlep)) (Math|Rotator|SelectRotator (Math|Rotator|MakeRotator 0.0 0.0 (.yaw (Variables|Internal|GetOpen%20Rotation))) (Variables|Internal|GetStart%20Rotation) _isa) (Utilities|Time|GetWorldDeltaSeconds) 5.0) (Math|Rotator|SelectRotator (Math|Rotator|MakeRotator 0.0 0.0 (.yaw (Variables|Internal|GetOpen%20Rotation))) (Variables|Internal|GetStart%20Rotation) _isa) 0.1)
            (bind _output_get (Variables|Internal|SetOpened (not (Math|Rotator|Equal(Rotator) (Variables|/Script/Engine.SceneComponent|GetRelativeRotation (Variables|Default|GetKlep)) (Variables|Internal|GetStart%20Rotation) 1.0))))
            (Utilities|FlowControl|Sequence
              (:then_0
                (if _output_get
                  (Default|CallTorpedoDoorOpened)
                  (else
                    (Default|CallTorpedoDoorClosed))))
              (:then_1
                (goto _label Reset)))
            (else
              (Utilities|FlowControl|Delay (Utilities|Time|GetWorldDeltaSeconds))
              (goto _label_2))))
        (:then_1
          (Utilities|FlowControl|FlipFlop
            (:A
              (Audio|Components|Audio|SetSound _audio_2 _door_open_sound)
              (Audio|Components|Audio|Play _audio_2 (* (Variables|/Script/Engine.SoundBase|GetDuration _door_open_sound) 0.25)))
            (:B
              (Audio|Components|Audio|SetSound _audio (Variables|Settings|GetDoor%20Close%20Sound))
              (Utilities|FlowControl|Delay 1.0)
              (Audio|Components|Audio|Play _audio 0.0))))))))

(event ActiveStateChanged(Comp_Active)
  (params (Pawn :type BP%20Pawn%20Base%20Object%20Reference) (Comp%20Active :type Comp%20Active%20Object%20Reference) (New%20Active :type Boolean))
  (bind _audio (Variables|Default|GetAudio))
  (Development|SetHiddeninGame (Variables|Default|GetTorpedo) (not New%20Active) false)
  (bind _output_get (Variables|Internal|SetOccupied New%20Active))
  (Default|CallTorpedoHoleOccupied)
  (if _output_get
    (Audio|Components|Audio|SetSound _audio (Variables|Settings|GetLoading%20Torpedo%20Sound))
    (Audio|Components|Audio|Play _audio 0.0)))

(event EventBeginPlay
  (Variables|Internal|SetStart%20Rotation (Variables|/Script/Engine.SceneComponent|GetRelativeRotation (Variables|Default|GetKlep)))
  (Variables|Internal|SetOpen%20Rotation "0,150.000000, 0"))

(fn ConstructionScript)

(fn GetKlepLocalRotation
  (return (- (+ (* (.yaw (Transformation|GetWorldRotation (Variables|Default|GetDefaultSceneRoot))) -1.0) (.yaw (Variables|/Script/Engine.SceneComponent|GetRelativeRotation (Variables|Default|GetKlep)))) 9e+01)))

(fn IsOpened
  (return (Variables|Internal|GetOpened)))

(fn IsOccupied
  (return (Variables|Internal|GetOccupied)))

(fn OnRepOccupied)

(fn OnRepOpened)