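; BP_Torpedo_Hole_Out is a ship munition actor that acts as a docking point between a torpedo cart and a torpedo tube.
; A cart-tagged component overlapping its box snaps the torpedo cart to the scene anchor's transform.
; Setting torpedo visibility clears Occupied, updates the tube's occupancy, and runs through server and multicast events to show or hide the spawned torpedo and disable interaction.
; The interaction press is empty, and the cart-loading logic is disconnected.
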(event PressedInteraction(Comp_Interaction)
  (params (Pawn :type BP%20Pawn%20Base%20Object%20Reference) (Souce%20Actor :type Actor%20Object%20Reference) (Hit%20Location :type Vector :default "0, 0, 0") (Hit%20Distance :type Float%20%28single-precision%29) (Hit%20Component :type Actor%20Component%20Object%20Reference)))

(event OnComponentBeginOverlap(Box)
  (params (OverlappedComponent :type Primitive%20Component%20Object%20Reference) (OtherActor :type Actor%20Object%20Reference) (OtherComp :type Primitive%20Component%20Object%20Reference) (OtherBodyIndex :type Integer) (bFromSweep :type Boolean) (SweepResult :type Hit%20Result%20Structure%20%28by%20ref%29))
  (bind _scene1 (Variables|Default|GetScene1))
  (bind _returnvalue (Transformation|GetWorldTransform _scene1))
  (if (Components|ComponentHasTag OtherComp (Variables|Settings|GetTorpedo%20Cart%20Tag))
    (bind _torpedo_cart (Variables|Settings|GetTorpedo%20Cart)
      (:then
        (Default|SnaptoTorpedoTubeLocation _torpedo_cart (.location _returnvalue) (.rotation _returnvalue)))
      (:else))))

(event Custom|Multi_Set%20Torpedo%20Visible
  (params (Set :type Boolean))
  (bind _spawned_torpedo (Variables|Internal|GetSpawned%20Torpedo)
    (:then
      (Rendering|SetActorHiddenInGame _spawned_torpedo (not Set)))
    (:else)))

(event Custom|Set%20Torpedo%20Visible
  (params (Set :type Boolean))
  (CallFunction|ServerSetTorpedoVisible Set)
  (Variables|Internal|SetOccupied false)
  (bind _torpedo_tube (Variables|Settings|GetTorpedo%20Tube)
    (:then
      (Default|OccupyTorpedo _torpedo_tube Set))
    (:else)))

(event Custom|Server_Set%20Torpedo%20Visible
  (params (Set :type Boolean))
  (CallFunction|MultiSetTorpedoVisible Set)
  (Default|SetInteractionEnabled (Variables|Default|GetComp_Interaction) false))

(event EventBeginPlay)

(fn ConstructionScript)

(fn IsOccupied
  (return (Variables|Internal|GetOccupied)))

(fn OnRepOccupied)

(fn OnRepOpened)

(fn OnRepSpawnedTorpedo)