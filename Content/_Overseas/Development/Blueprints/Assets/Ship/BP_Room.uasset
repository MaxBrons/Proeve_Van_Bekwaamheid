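; BP_Room is a ship room volume that tracks the doors touching it and the player pawns inside it.
; One second after BeginPlay, it gathers every BP_Door overlapping its Box component into the DoorsToRoom array.
; GetPlayerCountInsideRoom returns how many BP_Pawn_Base actors currently overlap the same box.
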(event EventBeginPlay
  (Utilities|FlowControl|Delay 1.0)
  (for _array_element (Collision|GetOverlappingActors (Variables|Default|GetBox) "/Game/_Overseas/Development/Blueprints/Assets/Ship/BP_Door.BP_Door_C" :!class /Script/Engine.PrimitiveComponent)
    (bind _asbp_door (Utilities|Casting|CastToBP_Door _array_element))
    (Utilities|Array|Add (Variables|Internal|GetDoors%20To%20Room) _asbp_door)))

(fn ConstructionScript)

(fn GetPlayerCountInsideRoom
  (return (Utilities|Array|Length (Collision|GetOverlappingActors (Variables|Default|GetBox) "/Game/_Overseas/Development/Blueprints/Pawns/BP_Pawn_Base.BP_Pawn_Base_C" :!class /Script/Engine.PrimitiveComponent))))