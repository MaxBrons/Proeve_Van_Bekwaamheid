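; Interactable electrical handle on a ship that flips a replicated Turned state when used.
; A press passes a DoOnce gate, and a FlipFlop alternates the pitch direction as a per-frame Delay loop rotates the mesh until a pitch check ends it.
; Completion toggles Turned and reopens the gate; its OnRep updates the active component and calls HandleTurned.
; BeginPlay simulates a press if Turned starts true.
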(event PressedInteraction(Comp_Interaction)
  (params (Pawn :type BP%20Pawn%20Base%20Object%20Reference) (Souce%20Actor :type Actor%20Object%20Reference) (Hit%20Location :type Vector :default "0, 0, 0") (Hit%20Distance :type Float%20%28single-precision%29) (Hit%20Component :type Actor%20Component%20Object%20Reference))
  (bind _hendel (Variables|Default|GetHendel))
  (Utilities|FlowControl|DoOnce false :!label _label
    (:Completed
      (bind _isa (Utilities|FlowControl|FlipFlop)
        (:A
          _)
        (:B
          _))
      (Transformation|SetWorldRotation _hendel (Math|Transform|TransformRotation (Transformation|GetWorldTransform _hendel) (Math|Rotator|MakeRotator 0.0 (* (Variables|Settings|GetRotation%20Speed) (Utilities|Time|GetWorldDeltaSeconds) (select _isa -1.0 1.0) 1.8e+02) 0.0)) false false :!label _label_2)
      (if (<= (.pitch (Variables|/Script/Engine.SceneComponent|GetRelativeRotation (Variables|Default|GetHendel))) (* (Variables|Settings|GetRotation%20Speed) -1.0))
        (Utilities|FlowControl|Delay (Utilities|Time|GetWorldDeltaSeconds))
        (goto _label_2)
        (else
          (Variables|Internal|SetTurned (not (Variables|Internal|GetTurned)))
          (goto _label Reset))))))

(event EventBeginPlay
  (if (Variables|Internal|GetTurned)
    (Default|InteractionPressed (Variables|Default|GetComp_Interaction) 0 0 "0, 0, 0" 0.0)))

(fn ConstructionScript)

(fn OnRepTurned
  (bind _turned (Variables|Internal|GetTurned))
  (Default|SetActive (Variables|Default|GetComp_Active) (CallFunction|GetMainPlayerPawn self) _turned)
  (Default|CallHandleTurned _turned))