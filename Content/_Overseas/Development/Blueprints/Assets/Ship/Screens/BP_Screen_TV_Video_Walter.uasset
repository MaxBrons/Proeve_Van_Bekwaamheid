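; Ship TV screen actor that plays a configured video through a screen-loop widget.
; On BeginPlay it hands the screen material to the WB_Screen_Loop widget, then opens the video source on the media player.
; A failed media open deactivates the active component.
; That component's state change drives widget visibility, hiding the widget when active and showing it when inactive.
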(event ActiveStateChanged(Comp_Active)
  (params (Pawn :type BP%20Pawn%20Base%20Object%20Reference) (Comp%20Active :type Comp%20Active%20Object%20Reference) (New%20Active :type Boolean))
  (Development|SetHiddeninGame (Variables|Default|GetComp_Widget) New%20Active false))

(event Custom|OnMediaOpenFailed_Event_0
  (params (FailedUrl :type String))
  (Default|SetActive (Variables|Default|GetComp_Active) 0 false))

(event EventBeginPlay
  (bind _aswb_screen_loop (Utilities|Casting|CastToWB_Screen_Loop (UserInterface|GetUserWidgetObject (Variables|Default|GetComp_Widget))))
  (bind _output_get (Variables|Default|SetScreen%20Widget _aswb_screen_loop))
  (bind _screen_material_to_show (Variables|Settings|GetScreen%20Material%20To%20Show)
    (:then
      (Default|SetupWidget _output_get _screen_material_to_show)
      (bind _mediaplayer_to_show (Variables|Settings|GetMediaplayer%20To%20Show)
        (:then
          (EventDispatchers|AssignOnMediaOpenFailed _mediaplayer_to_show (delegate Custom|OnMediaOpenFailed_Event_0))
          (bind _mediaplayer_to_show_2 (Variables|Settings|GetMediaplayer%20To%20Show)
            (:then
              (bind _video_to_show (Variables|Settings|GetVideo%20To%20Show)
                (:then
                  (Media|MediaPlayer|OpenSource _mediaplayer_to_show_2 _video_to_show))
                (:else)))
            (:else)))
        (:else)))
    (:else)))

(fn ConstructionScript)