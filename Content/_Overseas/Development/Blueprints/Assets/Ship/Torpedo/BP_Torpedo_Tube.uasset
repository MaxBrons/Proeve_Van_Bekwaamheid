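; BP_Torpedo_Tube is a ship torpedo tube with an interactive door, torpedo loading and launching.
; Interaction toggles the door through a per-frame interpolated rotation loop, with sounds and open/closed notifications; active state enables interaction.
; On authority, loading lerps the torpedo inside via timeline and marks the tube occupied; launching destroys it.
; Launching also plays audio and asks the enemy ship manager to attempt a hit along the ship's current course.
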(event PressedInteraction(Comp_Interaction)
  (params (Pawn :type BP%20Pawn%20Base%20Object%20Reference) (Souce%20Actor :type Actor%20Object%20Reference) (Hit%20Location :type Vector :default "0, 0, 0") (Hit%20Distance :type Float%20%28single-precision%29) (Hit%20Component :type Actor%20Component%20Object%20Reference))
  (bind _self self)
  (bind _opening_door_sound (Variables|Settings|GetOpening%20Door%20Sound))
  (bind _audio (Variables|Default|GetAudio))
  (bind _audio_2 (Variables|Default|GetAudio))
  ;[1 1 1] Open and close the tube door, when the door is closed or opened it also will play a sound.
  (Utilities|FlowControl|DoOnce false :!label _label
    (:Completed
      (Utilities|FlowControl|Sequence
        (:then_0
          (bind _isa (Utilities|FlowControl|FlipFlop)
            (:A
              _)
            (:B
              _))
          (Transformation|SetRelativeRotation (Variables|Default|GetKlep) (Math|Interpolation|RInterpTo (Variables|/Script/Engine.SceneComponent|GetRelativeRotation (Variables|Default|GetKlep)) (Math|Rotator|SelectRotator (Math|Rotator|MakeRotator 0.0 0.0 (Variables|Settings|GetOpen%20Rotation)) (Variables|Internal|GetStart%20Rotation) _isa) (Utilities|Time|GetWorldDeltaSeconds) 5.0) false false :!label _label_2)
          (if (Math|Rotator|Equal(Rotator) (Math|Interpolation|RInterpTo (Variables|/Script/Engine.SceneComponent|GetRelativeRotation (Variables|Default|GetKlep)) (Math|Rotator|SelectRotator (Math|Rotator|MakeRotator 0.0 0.0 (Variables|Settings|GetOpen%20Rotation)) (Variables|Internal|GetStart%20Rotation) _isa) (Utilities|Time|GetWorldDeltaSeconds) 5.0) (Math|Rotator|SelectRotator (Math|Rotator|MakeRotator 0.0 0.0 (Variables|Settings|GetOpen%20Rotation)) (Variables|Internal|GetStart%20Rotation) _isa) 0.1)
            (bind _output_get (Variables|Internal|SetClosed (Math|Rotator|Equal(Rotator) (Variables|/Script/Engine.SceneComponent|GetRelativeRotation (Variables|Default|GetKlep)) (Variables|Internal|GetStart%20Rotation) 1.0)))
            (Utilities|FlowControl|Sequence
              (:then_0
                (if _output_get
                  (Default|CallTubeDoorClosed _self)
                  (else
                    (Default|CallTubeDoorOpened _self))))
              (:then_1
                (goto _label Reset)))
            (else
              (Utilities|FlowControl|Delay (Utilities|Time|GetWorldDeltaSeconds))
              (goto _label_2))))
        (:then_1
          (Utilities|FlowControl|FlipFlop
            (:A
              (Audio|Components|Audio|SetSound _audio_2 _opening_door_sound)
              (Audio|Components|Audio|Play _audio_2 (* (Variables|/Script/Engine.SoundBase|GetDuration _opening_door_sound) 0.25)))
            (:B
              (Audio|Components|Audio|SetSound _audio (Variables|Settings|GetClosing%20Door%20Sound))
              (Utilities|FlowControl|Delay 1.0)
              (Audio|Components|Audio|Play _audio 0.0))))))))

(event ActiveStateChanged(Comp_Active)
  (params (Pawn :type BP%20Pawn%20Base%20Object%20Reference) (Comp%20Active :type Comp%20Active%20Object%20Reference) (New%20Active :type Boolean))
  ;[1 1 1] Disable the interaction with the door when the active state changes.
  (Default|SetInteractionEnabled (Variables|Default|GetComp_Interaction) New%20Active))

(event Custom|Load%20Torpedo
  (params (Torpedo%20To%20Load :type BP%20Torpedo%20Object%20Reference))
  ;[1 1 1] Lerp the torpedo to the inside of the tube.
  (Networking|SwitchHasAuthority
    (:Authority
      (Utilities|IsValid Torpedo%20To%20Load
        (:Is%20Valid
          (Transformation|DetachFromActor Torpedo%20To%20Load "KeepWorld" "KeepWorld" "KeepWorld")
          (bind _output_get (Variables|Internal|SetCurrent%20Torpedo Torpedo%20To%20Load))
          (Variables|Internal|SetLerp%20Start%20Transform (Transformation|GetActorTransform _output_get))
          (bind _alpha (Timeline|Torpedo%20Loading PlayFromStart)
            (:Update
              (Transformation|SetActorTransform (Variables|Internal|GetCurrent%20Torpedo) (Math|Transform|Lerp(Transform) (Variables|Internal|GetLerp%20Start%20Transform) (Transformation|GetWorldTransform (Variables|Default|GetScene)) _alpha)))
            (:Finished
              (Variables|Internal|SetOccupied true)
              (Default|CallTubeOccupied))))))))

(event Custom|Launch%20Torpedo
  (bind _torpedo_launch (Variables|Default|GetTorpedo%20Launch))
  ;[1 1 1] Launch a torpedo in the current direction of the ship and destroy the torpedo actor.
  (Audio|Components|Audio|SetSound _torpedo_launch (Variables|Settings|GetFire%20Torpedo%20Sound))
  (Audio|Components|Audio|Play _torpedo_launch 0.0)
  (Networking|SwitchHasAuthority
    (:Authority
      (bind _current_torpedo (Variables|Internal|GetCurrent%20Torpedo)
        (:then
          (Actor|DestroyActor _current_torpedo))
        (:else
          _))
      (Variables|Internal|SetCurrent%20Torpedo 0)
      (Variables|Internal|SetOccupied false))
    (:Remote
      _))
  (bind _ship (Variables|Default|GetShip)
    (:then
      (bind _enemy_ship_manager (Variables|Default|GetEnemy%20Ship%20Manager)
        (:then
          (Default|TrytoHitShipwithTorpedo _enemy_ship_manager (Variables|/Game/_Overseas/Development/Blueprints/Systems/Ship/BP_Ship.BP_Ship_C|GetCurrent%20Course _ship) "NewEnumerator0")
          (Default|CallTorpedoLaunched))
        (:else)))
    (:else)))

(event EventBeginPlay
  ;[1 1 1] Store the start rotation of the door and set the ship manager and the ship variable to use for firing the torpedo and getting the course to fire the torpedo from.
  (Variables|Internal|SetStart%20Rotation (Variables|/Script/Engine.SceneComponent|GetRelativeRotation (Variables|Default|GetKlep)))
  (bind _returnvalue (Actor|GetActorOfClass "/Game/_Overseas/Development/Blueprints/Systems/Enemy_Ship/BP_Enemy_Ship_Manager.BP_Enemy_Ship_Manager_C"))
  (Utilities|WaitforObjecttoValidate _returnvalue 0.05
    (:Is%20Valid
      (Variables|Default|SetEnemy%20Ship%20Manager _returnvalue)
      (bind _returnvalue_2 (Actor|GetActorOfClass "/Game/_Overseas/Development/Blueprints/Systems/Ship/BP_Ship.BP_Ship_C"))
      (Utilities|WaitforObjecttoValidate _returnvalue_2 0.05
        (:Is%20Valid
          (Variables|Default|SetShip _returnvalue_2))))))

(fn ConstructionScript)

(fn IsOccupied
  (return (Variables|Internal|GetOccupied)))

(fn IsClosed
  (return (Variables|Internal|GetClosed)))