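; Ship torpedo loading rack that holds one torpedo and animates it moving onto and off the rack.
; Load accepts a torpedo only when empty; on authority it detaches it and timeline-lerps it to the in or out location chosen by TorpedoDirection.
; Unload, also authority-driven, lerps the torpedo to a supplied component's transform, then attaches it to the given parent.
; Multicast events announce each completed move, with unload also clearing the current torpedo.
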(event Custom|Unload%20Torpedo
  (params (Component%20To%20Attach%20To :type Primitive%20Component%20Object%20Reference) (Scene%20Component%20To%20Move%20To :type Scene%20Component%20Object%20Reference))
  (Networking|SwitchHasAuthority
    (:Authority
      (Utilities|IsValid Component%20To%20Attach%20To
        (:Is%20Valid
          (bind _current_torpedo (Variables|Internal|GetCurrent%20Torpedo)
            (:then
              (Variables|Internal|SetLerp%20Start%20Transform (Transformation|GetActorTransform _current_torpedo))
              (Transformation|DetachFromActor _current_torpedo "KeepWorld" "KeepWorld" "KeepWorld")
              (bind _alpha (Timeline|Timeline_1 PlayFromStart)
                (:Update
                  (Transformation|SetActorTransform (Variables|Internal|GetCurrent%20Torpedo) (Math|Transform|Lerp(Transform) (Variables|Internal|GetLerp%20Start%20Transform) (Transformation|GetWorldTransform Scene%20Component%20To%20Move%20To) _alpha)))
                (:Finished
                  (Transformation|AttachComponentToComponent (Variables|Internal|GetCurrent%20Torpedo) Component%20To%20Attach%20To "None" "KeepWorld" "KeepWorld" "KeepWorld" true)
                  (CallFunction|MultiUnloadTorpedo))))
            (:else)))))))

(event Custom|Load%20Torpedo
  (params (Torpedo%20To%20Load :type BP%20Torpedo%20Object%20Reference))
  (Variables|Internal|GetCurrent%20Torpedo
    (:then)
    (:else
      (Utilities|IsValid Torpedo%20To%20Load
        (:Is%20Valid
          (bind _output_get (Variables|Internal|SetCurrent%20Torpedo Torpedo%20To%20Load))
          (Networking|SwitchHasAuthority
            (:Authority
              (Transformation|DetachFromActor _output_get "KeepWorld" "KeepWorld" "KeepWorld")
              (Variables|Internal|SetLerp%20Start%20Transform (Transformation|GetActorTransform _output_get))
              (bind _alpha (Timeline|Timeline_0 PlayFromStart)
                (:Update
                  (Transformation|SetActorTransform (Variables|Internal|GetCurrent%20Torpedo) (Math|Transform|Lerp(Transform) (Variables|Internal|GetLerp%20Start%20Transform) (Transformation|GetWorldTransform (Utilities|Select :Index (Variables|Settings|GetTorpedo%20Direction) :NewEnumerator0 (Variables|Default|GetTorpedo%20Out%20Location) :NewEnumerator1 (Variables|Default|GetTorpedo%20In%20Location))) _alpha)))
                (:Finished
                  (CallFunction|MultiLoadTorpedo))))))))))

(event Custom|Multi_Unload%20Torpedo
  (Variables|Internal|SetCurrent%20Torpedo 0)
  (Default|CallTorpedoUnloadedfromRack))

(event Custom|Multi_Load%20Torpedo
  (Default|CallTorpedoLoadedonRack))

(fn ConstructionScript)