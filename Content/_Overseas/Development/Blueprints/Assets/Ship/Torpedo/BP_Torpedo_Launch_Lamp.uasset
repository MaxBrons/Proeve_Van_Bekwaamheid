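; Ship torpedo launch lamp that lights up to show when all launch keys are turned.
; On BeginPlay it creates a dynamic material for the lamp, and the authority binds to the TorpedoLaunchManager's launch-keys-turned event.
; That event is relayed through a server event to a multicast, which switches the material's ready-light parameter on or off.
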(event Custom|Multi_Keys%20Turned
  (params (All%20Turned :type Boolean))
  (bind _lamp_material (Variables|Internal|GetLamp%20Material)
    (:then
      (Rendering|Material|SetScalarParameterValue _lamp_material "Torpedo Ready Licht" (select All%20Turned 1.0 0.0) :!class /Script/Engine.MaterialInstanceDynamic))
    (:else)))

(event Custom|Keys%20Turned
  (params (All%20Turned :type Boolean))
  (CallFunction|ServerKeysTurned All%20Turned))

(event Custom|Server_Keys%20Turned
  (params (All%20Turned :type Boolean))
  (CallFunction|MultiKeysTurned All%20Turned))

(event EventBeginPlay
  (bind _returnvalue (Rendering|Material|CreateDynamicMaterialInstance (Variables|Default|GetStaticMesh) 0 "/Game/_Overseas/Art/Saskia/Materials/M_TorpedoReadyKnop.M_TorpedoReadyKnop" "ReadyLamp" :!class /Script/Engine.PrimitiveComponent))
  (Variables|Internal|SetLamp%20Material _returnvalue)
  (Networking|SwitchHasAuthority
    (:Authority
      (bind _torpedo_launch_manager (Variables|Settings|GetTorpedo%20Launch%20Manager)
        (:then
          (EventDispatchers|BindEventtoLaunchKeysTurned _torpedo_launch_manager (delegate Custom|Keys%20Turned)))
        (:else)))))

(fn ConstructionScript)