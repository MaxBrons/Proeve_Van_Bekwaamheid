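; Torpedo launch key that fires an OnKeyTurned event on interaction, then plays an animated turn and return.
; A FlipFlop chains the two phases, rotating the key to 90 degrees yaw, then easing it back to its start rotation with FInterpTo.
; Frame-length Delay loops drive the motion instead of Tick, with DoOnce-gated sounds near each end.
; Further presses are blocked until the key is back at rest.
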(event PressedInteraction(Comp_Interaction)
  (params (Pawn :type BP%20Pawn%20Base%20Object%20Reference) (Souce%20Actor :type Actor%20Object%20Reference) (Hit%20Location :type Vector :default "0, 0, 0") (Hit%20Distance :type Float%20%28single-precision%29) (Hit%20Component :type Actor%20Component%20Object%20Reference))
  (bind _returnvalue (Utilities|Time|GetWorldDeltaSeconds))
  (bind _key (Variables|Default|GetKey))
  (bind _start_rotation (Variables|Internal|GetStart%20Rotation))
  (bind _turn_speed (Variables|Settings|GetTurn%20Speed))
  (bind _key_2 (Variables|Default|GetKey))
  (bind _key_3 (Variables|Default|GetKey))
  (bind _returnvalue_2 (CallFunction|GetLocalRotation _key_3 "0.000000,0.000000,0.000000"))
  (bind _relativerotation (Variables|/Script/Engine.SceneComponent|GetRelativeRotation _key_2))
  (bind _returnvalue_3 (Math|Interpolation|FInterpTo (.yaw _relativerotation) (.yaw _start_rotation) _returnvalue _turn_speed))
  (bind _returnvalue_4 (- _returnvalue_3 (.yaw _start_rotation)))
  (Utilities|FlowControl|DoOnce false
    (:Completed
      (Utilities|FlowControl|Sequence
        (:then_0
          (Default|CallOnKeyTurned self)
          (goto _label_3 Reset))
        (:then_1
          (goto _label_6 Reset))
        (:then_2
          (Utilities|FlowControl|FlipFlop :!label _label
            (:A
              (if (>= (.yaw _returnvalue_2) 9e+01) :!label _label_2
                (goto _label)
                (elif (>= (.yaw _returnvalue_2) 6e+01)
                  (Utilities|FlowControl|Sequence
                    (:then_0
                      (Utilities|FlowControl|DoOnce false :!label _label_3
                        (:Completed
                          (Audio|Components|Audio|Play (Variables|Default|GetAudio) 0.0))))
                    (:then_1
                      (Utilities|FlowControl|Sequence :!label _label_4
                        (:then_0
                          (Transformation|SetWorldRotation _key (Math|Transform|TransformRotation (Transformation|GetWorldTransform _key) (Math|Rotator|MakeRotator 0.0 0.0 (/ (Variables|Settings|GetTurn%20Speed) 2.0))) false false))
                        (:then_1
                          (Utilities|FlowControl|Delay (Utilities|Time|GetWorldDeltaSeconds))
                          (goto _label_2)))))
                  (else
                    (goto _label_4)))))
            (:B
              (if (Math|Float|NearlyEqual(Float) _returnvalue_4 0.0 1.0) :!label _label_5
                (CallFunction|ResetInteractionBlock)
                (else
                  (Utilities|FlowControl|Sequence
                    (:then_0
                      (if (Math|Float|NearlyEqual(Float) _returnvalue_4 0.0 5.0)
                        (Utilities|FlowControl|Sequence
                          (:then_0
                            (Utilities|FlowControl|DoOnce false :!label _label_6
                              (:Completed
                                (Audio|Components|Audio|Play (Variables|Default|GetAudio) 0.0))))
                          (:then_1
                            (Transformation|SetRelativeRotation (Variables|Default|GetKey) (Math|Rotator|MakeRotator 0.0 0.0 _returnvalue_3) false false :!label _label_7)))
                        (else
                          (goto _label_7))))
                    (:then_1
                      (Utilities|FlowControl|Delay (Utilities|Time|GetWorldDeltaSeconds))
                      (goto _label_5))))))))))))

(event Custom|Reset%20Interaction%20Block
  (bind _returnvalue (Utilities|Time|GetWorldDeltaSeconds))
  (bind _key (Variables|Default|GetKey))
  (bind _start_rotation (Variables|Internal|GetStart%20Rotation))
  (bind _turn_speed (Variables|Settings|GetTurn%20Speed))
  (bind _key_2 (Variables|Default|GetKey))
  (bind _key_3 (Variables|Default|GetKey))
  (bind _returnvalue_2 (CallFunction|GetLocalRotation _key_3 "0.000000,0.000000,0.000000"))
  (bind _relativerotation (Variables|/Script/Engine.SceneComponent|GetRelativeRotation _key_2))
  (bind _returnvalue_3 (Math|Interpolation|FInterpTo (.yaw _relativerotation) (.yaw _start_rotation) _returnvalue _turn_speed))
  (bind _returnvalue_4 (- _returnvalue_3 (.yaw _start_rotation)))
  (Utilities|FlowControl|DoOnce false) ; enters at Reset
)

(event EventBeginPlay
  (Variables|Internal|SetStart%20Rotation (Variables|/Script/Engine.SceneComponent|GetRelativeRotation (Variables|Default|GetKey)))
  (bind _turn_key_sound (Variables|Settings|GetTurn%20Key%20Sound)
    (:then
      (Audio|Components|Audio|SetSound (Variables|Default|GetAudio) _turn_key_sound))
    (:else)))

(fn ConstructionScript)