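; Player-operated torpedo crane that moves torpedoes to and from loading racks, with a controls widget and cyclable cameras.
; Key presses are forwarded through the player's pawn for replication and set axis values that Tick turns into clamped offsets.
; Vertical travel is spread across stacked beam meshes by cumulative bounds, and movement fades a sound blend parameter.
; The beam rotates based on distance to a target rack, and interacting loads or unloads the overlapped rack's torpedo.
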(event ActiveStateChanged(Comp_Active)
  (params (Pawn :type BP%20Pawn%20Base%20Object%20Reference) (Comp%20Active :type Comp%20Active%20Object%20Reference) (New%20Active :type Boolean))
  ;[1 1 1] Prevent another player from taking control of the crane when a player is currently controlling the crane.
  (Default|SetInteractionEnabled (Variables|Default|GetComp_Focus) New%20Active))

(event PressedInteraction(Comp_Focus)
  (params (Pawn :type BP%20Pawn%20Base%20Object%20Reference) (Souce%20Actor :type Actor%20Object%20Reference) (Hit%20Location :type Vector :default "0, 0, 0") (Hit%20Distance :type Float%20%28single-precision%29) (Hit%20Component :type Actor%20Component%20Object%20Reference))
  ;[1 1 1] Switch the input to the interacting player
  (Variables|Internal|Input|SetCurrent%20Pawn (CallFunction|GetMainPlayerPawn self))
  (Utilities|IsReplicatedOwner Pawn
    (:Owner
      (bind _asbp_pawn_screen (Utilities|Casting|CastToBP_Pawn_Screen Pawn))
      (bind _crane_widget (Variables|Internal|General|GetCrane%20Widget)
        (:then
          (Default|AddWidgettoViewport _asbp_pawn_screen "Crane" _crane_widget)
          (bind _images (UI|GetWidgetInputs))
          (Default|SetupWidgetInput _crane_widget _images)
          (Variables|Internal|General|SetCurrent%20Camera%20Index -1)
          (CallFunction|SwitchCamera true))
        (:else)))
    (:Not%20Owner
      _))
  (Actor|Tick|SetActorTickEnabled true)
  (CallFunction|PlayMovingSound true)
  (Networking|SwitchHasAuthority
    (:Authority
      (Default|SetInteractionEnabled (Variables|Default|GetComp_Focus) false))))

(event Custom|Switch%20Camera
  (params (First :type Boolean))
  (bind _comp_focus (Variables|Default|GetComp_Focus))
  ;[1 1 1] Switch the camera that is used to view the crane when controlling it.
  (bind _result (Math|Integer|IncrementInt (Variables|Internal|General|GetCurrent%20Camera%20Index))
    (:%20%20
      (if (Utilities|Array|IsValidIndex (Variables|Internal|General|GetCamera's%20To%20Switch%20To) _result)
        _
        (else
          (Variables|Internal|General|SetCurrent%20Camera%20Index 0)))
      (Game|Player|SetViewTargetwithBlend (Game|GetPlayerController 0) (Utilities|Array|Get(acopy) (Variables|Internal|General|GetCamera's%20To%20Switch%20To) (Variables|Internal|General|GetCurrent%20Camera%20Index)) (select First (Variables|/Game/_Overseas/Development/Blueprints/Components/Comp_Focus.Comp_Focus_C|GetFocus%20Time _comp_focus) 0.5) (Variables|/Game/_Overseas/Development/Blueprints/Components/Comp_Focus.Comp_Focus_C|GetFocus%20Motion%20Type _comp_focus) 2.0 false)
      (bind _crane_widget (Variables|Internal|General|GetCrane%20Widget)
        (:then
          (Default|UpdateMovementTexts _crane_widget (select (== (Variables|Internal|General|GetCurrent%20Camera%20Index) 0) "Voorwaards / Achterwaards" "Links / Rechts") (select (== (Variables|Internal|General|GetCurrent%20Camera%20Index) 0) "Rechts / Links" "Voorwaards / Achterwaards") "Omhoog / Omlaag"))
        (:else)))))

(event Custom|Play%20Moving%20Sound
  (params (Play :type Boolean))
  (bind _crane_moving_sound (Variables|Default|GetCrane_Moving_Sound))
  ;[1 1 1] Play the sound and replicate it.
  (if Play
    (Audio|Components|Audio|Play _crane_moving_sound 0.0)
    (else
      (Audio|Components|Audio|Stop _crane_moving_sound))))

(event Custom|Toggle%20Attach%20Torpedo
  ;[1 1 1] Attach or detach the torpedo to the Z mesh to let it move with the mesh. When releasing it will turn on the physics of the torpedo to let it naturally fall to the ground. Upon hitting something except for the player it will disable the physics again.
  (bind _asbp_loading_rack (Utilities|Casting|CastToBP_LoadingRack (Utilities|Array|Get(acopy) (Collision|GetOverlappingActors (Variables|Default|GetBox) "/Game/_Overseas/Development/Blueprints/Assets/Ship/Torpedo/BP_LoadingRack.BP_LoadingRack_C" :!class /Script/Engine.PrimitiveComponent))))
  (Variables|Internal|General|GetAttached%20Torpedo
    (:then
      (Default|LoadTorpedo _asbp_loading_rack (Variables|Internal|General|GetAttached%20Torpedo))
      (Variables|Internal|General|SetAttached%20Torpedo 0))
    (:else
      (bind _current_torpedo (Variables|/Game/_Overseas/Development/Blueprints/Assets/Ship/Torpedo/BP_LoadingRack.BP_LoadingRack_C|GetCurrent%20Torpedo _asbp_loading_rack)
        (:then
          (Variables|Internal|General|SetAttached%20Torpedo _current_torpedo)
          (Default|UnloadTorpedo _asbp_loading_rack (Variables|Default|GetZ) (Variables|Default|GetTorpedo%20Location)))
        (:else))))
  (Audio|Components|Audio|Play (Variables|Default|GetCrane_Decopple_Sound) 0.0))

(event EventBeginPlay
  (bind _crane_moving_sound (Variables|Default|GetCrane_Moving_Sound))
  (bind _crane_decopple_sound (Variables|Default|GetCrane_Decopple_Sound))
  ;[1 1 1] Ignore the overlap with meshes from this actor and create the widget that is shown when you controll the crane. Also set the audio files and stop the sound components.
  (Collision|IgnoreActorwhenMoving (Variables|Default|GetBox) self true)
  (bind _returnvalue (UserInterface|CreateWidget "/Game/_Overseas/Development/Blueprints/Widgets/HUD/Task_Screens/WB_Screen_Crane.WB_Screen_Crane_C" 0 0 0))
  (Variables|Internal|General|SetCrane%20Widget _returnvalue)
  (Audio|Components|Audio|Stop _crane_moving_sound)
  (bind _crane_moving_sound_2 (Variables|Settings|GetCrane%20Moving%20Sound)
    (:then
      (Audio|Components|Audio|SetSound _crane_moving_sound _crane_moving_sound_2))
    (:else
      _))
  (Audio|Components|Audio|Stop _crane_decopple_sound)
  (bind _torpedo_lock_sound (Variables|Settings|GetTorpedo%20Lock%20Sound)
    (:then
      (Audio|Components|Audio|SetSound _crane_decopple_sound _torpedo_lock_sound)
      ;[1 1 1] Set the child actor array that is used for the different camera's.
      (Variables|Internal|General|SetCamera's%20To%20Switch%20To (Utilities|Array|MakeArray (Variables|/Script/Engine.ChildActorComponent|GetChildActor (Variables|Default|GetChildActor)) (Variables|/Script/Engine.ChildActorComponent|GetChildActor (Variables|Default|GetChildActor1)) (Variables|/Script/Engine.ChildActorComponent|GetChildActor (Variables|Default|GetChildActor2)) (Variables|/Script/Engine.ChildActorComponent|GetChildActor (Variables|Default|GetChildActor3))))
      ;[1 1 1] Set the max height to use for the lift it's z axis.
      (bind _output_get (Variables|Internal|Movement|SetHeight%20Meshes (Utilities|Array|MakeArray (Variables|Default|GetBalk4) (Variables|Default|GetBalk3) (Variables|Default|GetBalk2))))
      (for _array_element _output_get
        (bind _output_get_2 (Variables|Internal|Movement|SetMax%20Height (+ (Variables|Internal|Movement|GetMax%20Height) (.z (.Max (Components|StaticMesh|GetLocalBounds _array_element))))))
        (Utilities|Array|Add (Variables|Internal|Movement|GetHeight%20Meshes%20Bounds) _output_get_2)))
    (:else)))

(event EventInteractionReleased
  (params (Key%20Code :type Name :default "None"))
  ;[1 1 1] Reset the the axis value to 0 to stop moving in the direction
  (switch name Key%20Code
    (:Forward
      (Variables|Internal|Input|SetInput%20Y 0.0 :!label _label))
    (:Backwards
      (goto _label))
    (:Left
      (Variables|Internal|Input|SetInput%20X 0.0 :!label _label_2))
    (:Right
      (goto _label_2))
    (:Up
      (Variables|Internal|Input|SetInput%20Z 0.0 :!label _label_3))
    (:Down
      (goto _label_3))))

(event EventInteractionPressed
  (params (Key%20Code :type Name :default "None"))
  ;[1 1 1] Set the axis value to eather increase or decrease in the axis you want to move.
  (Utilities|FlowControl|Sequence
    (:then_0
      (switch name Key%20Code
        (:Forward
          (Variables|Internal|Input|SetInput%20Y 1.0))
        (:Backwards
          (Variables|Internal|Input|SetInput%20Y -1.0))))
    (:then_1
      (switch name Key%20Code
        (:Left
          (Variables|Internal|Input|SetInput%20X -1.0))
        (:Right
          (Variables|Internal|Input|SetInput%20X 1.0))))
    (:then_2
      (switch name Key%20Code
        (:Up
          (Variables|Internal|Input|SetInput%20Z -1.0))
        (:Down
          (Variables|Internal|Input|SetInput%20Z 1.0))))
    (:then_3
      (switch name Key%20Code
        (:Interact
          (CallFunction|ToggleAttachTorpedo))
        (:Esc
          (Default|SetInteractionEnabled (Variables|Default|GetComp_Focus) true)
          (CallFunction|PlayMovingSound false)
          (Actor|Tick|SetActorTickEnabled false)
          (Variables|Internal|Input|SetInput%20X 0.0)
          (Variables|Internal|Input|SetInput%20Y 0.0)
          (Variables|Internal|Input|SetInput%20Z 0.0))
        (:Confirm
          (CallFunction|SwitchCamera false))))))

(event EventTick
  (params (DeltaSeconds :type Float%20%28single-precision%29))
  (bind _springarm (Variables|Default|GetSpringArm))
  (bind _returnvalue (Transformation|GetWorldLocation _springarm))
  ;[1 1 1] Move the crane meshes in the direction they have to move based on their input values.
  (|CraneMovement DeltaSeconds
    (:Output
      (Transformation|SetWorldLocation _springarm (Math|Vector|MakeVector (.x _returnvalue) (.y _returnvalue) (.z (Transformation|GetWorldLocation (Variables|Default|GetZ)))) false false)
      (Utilities|RotateCrane 1.5))))

(event Input|ActionEvents|InputActionConfirm
  (params (Key :type Key%20Structure :default "None"))
  ;[1 1 1] Handle all the input. Forward the input to the controller so that it can be replicated from the client to the server.
  (:Pressed
    (CallFunction|InteractionPressed "Confirm")
    (bind _crane_widget (Variables|Internal|General|GetCrane%20Widget)
      (:then
        (Default|UpdateInput _crane_widget "Confirm" "Confirm" "Clicked"))
      (:else)))
  (:Released
    (CallFunction|InteractionReleased "Confirm")
    (bind _crane_widget_2 (Variables|Internal|General|GetCrane%20Widget)
      (:then
        (Default|UpdateInput _crane_widget_2 "Confirm" "Confirm"))
      (:else))))

(event Input|ActionEvents|InputActionUp
  (params (Key :type Key%20Structure :default "None"))
  (bind _self self)
  (bind _current_pawn (Variables|Internal|Input|GetCurrent%20Pawn))
  ;[1 1 1] Handle all the input. Forward the input to the controller so that it can be replicated from the client to the server.
  (:Pressed
    (Default|PressKey _current_pawn _self "Up")
    (UI|UpdateInputUI "NewEnumerator0" true))
  (:Released
    (Default|ReleaseKey _current_pawn _self "Up")
    (UI|UpdateInputUI "NewEnumerator0" false)))

(event Input|ActionEvents|InputActionDown
  (params (Key :type Key%20Structure :default "None"))
  (bind _self self)
  (bind _current_pawn (Variables|Internal|Input|GetCurrent%20Pawn))
  ;[1 1 1] Handle all the input. Forward the input to the controller so that it can be replicated from the client to the server.
  (:Pressed
    (Default|PressKey _current_pawn _self "Down")
    (UI|UpdateInputUI "NewEnumerator1" true))
  (:Released
    (Default|ReleaseKey _current_pawn _self "Down")
    (UI|UpdateInputUI "NewEnumerator1" false)))

(event Input|ActionEvents|InputActionLeft
  (params (Key :type Key%20Structure :default "None"))
  (bind _self self)
  (bind _current_pawn (Variables|Internal|Input|GetCurrent%20Pawn))
  ;[1 1 1] Handle all the input. Forward the input to the controller so that it can be replicated from the client to the server.
  (:Pressed
    (Default|PressKey _current_pawn _self "Left")
    (UI|UpdateInputUI "NewEnumerator2" true))
  (:Released
    (Default|ReleaseKey _current_pawn _self "Left")
    (UI|UpdateInputUI "NewEnumerator2" false)))

(event Input|ActionEvents|InputActionRight
  (params (Key :type Key%20Structure :default "None"))
  (bind _self self)
  (bind _current_pawn (Variables|Internal|Input|GetCurrent%20Pawn))
  ;[1 1 1] Handle all the input. Forward the input to the controller so that it can be replicated from the client to the server.
  (:Pressed
    (Default|PressKey _current_pawn _self "Right")
    (UI|UpdateInputUI "NewEnumerator3" true))
  (:Released
    (Default|ReleaseKey _current_pawn _self "Right")
    (UI|UpdateInputUI "NewEnumerator3" false)))

(event Input|ActionEvents|InputActionForward
  (params (Key :type Key%20Structure :default "None"))
  (bind _self self)
  (bind _current_pawn (Variables|Internal|Input|GetCurrent%20Pawn))
  ;[1 1 1] Handle all the input. Forward the input to the controller so that it can be replicated from the client to the server.
  (:Pressed
    (Default|PressKey _current_pawn _self "Forward")
    (UI|UpdateInputUI "NewEnumerator4" true))
  (:Released
    (Default|ReleaseKey _current_pawn _self "Forward")
    (UI|UpdateInputUI "NewEnumerator4" false)))

(event Input|ActionEvents|InputActionBackwards
  (params (Key :type Key%20Structure :default "None"))
  (bind _self self)
  (bind _current_pawn (Variables|Internal|Input|GetCurrent%20Pawn))
  ;[1 1 1] Handle all the input. Forward the input to the controller so that it can be replicated from the client to the server.
  (:Pressed
    (Default|PressKey _current_pawn _self "Backwards")
    (UI|UpdateInputUI "NewEnumerator5" true))
  (:Released
    (Default|ReleaseKey _current_pawn _self "Backwards")
    (UI|UpdateInputUI "NewEnumerator5" false)))

(event Input|ActionEvents|InputActionReturn
  (params (Key :type Key%20Structure :default "None"))
  (bind _self self)
  (bind _comp_focus (Variables|Default|GetComp_Focus))
  (bind _player_controller (CallFunction|GetMainPlayerController _self))
  ;[1 1 1] Handle all the input. Forward the input to the controller so that it can be replicated from the client to the server.
  ;;[0 0 0] Switch the input back to the original pawn and remove the widget from the HUD of the interacting pawn.
  (:Pressed
    (Default|PressKey (Variables|Internal|Input|GetCurrent%20Pawn) self "Esc")
    (bind _crane_widget (Variables|Internal|General|GetCrane%20Widget)
      (:then
        (Default|UpdateInput _crane_widget "Back" "Back" "Clicked")
        (Utilities|FlowControl|Delay 0.2)
        (Default|Unfocus (Variables|Default|GetComp_Focus))
        (bind _asbp_pawn_screen (Utilities|Casting|CastToBP_Pawn_Screen (CallFunction|GetMainPlayerPawn _self))
          (:then
            (Default|RemoveWidgetfromViewport _asbp_pawn_screen "Crane"))
          (:CastFailed
            _))
        (Game|Player|SetViewTargetwithBlend _player_controller (Variables|/Game/_Overseas/Development/Game/BP_PlayerController_Main.BP_PlayerController_Main_C|GetPlayer%20Pawn _player_controller) (Variables|/Game/_Overseas/Development/Blueprints/Components/Comp_Focus.Comp_Focus_C|GetFocus%20Time _comp_focus) (Variables|/Game/_Overseas/Development/Blueprints/Components/Comp_Focus.Comp_Focus_C|GetFocus%20Motion%20Type _comp_focus) 2.0 false))
      (:else))))

(event Input|ActionEvents|InputActionJump
  (params (Key :type Key%20Structure :default "None"))
  ;[1 1 1] Handle all the input. Forward the input to the controller so that it can be replicated from the client to the server.
  (:Pressed
    (Default|PressKey (Variables|Internal|Input|GetCurrent%20Pawn) self "Interact")
    (bind _crane_widget (Variables|Internal|General|GetCrane%20Widget)
      (:then
        (Default|UpdateInput _crane_widget "Toggle Torpedo" "Toggle Torpedo" "Clicked"))
      (:else)))
  (:Released
    (bind _crane_widget_2 (Variables|Internal|General|GetCrane%20Widget)
      (:then
        (Default|UpdateInput _crane_widget_2 "Toggle Torpedo" "Toggle Torpedo"))
      (:else))))

(fn ConstructionScript)

(fn AddOffsettoCranePart
  (params (Component :type Primitive%20Component%20Object%20Reference) (Amount :type Vector) (Min :type Float%20%28single-precision%29) (Max :type Float%20%28single-precision%29) (Value%20To%20Clamp :type Float%20%28single-precision%29) (X :type Boolean) (Y :type Boolean) (Z :type Boolean))
  (bind _returnvalue (+ Amount Value%20To%20Clamp))
  (bind _returnvalue_2 (select Z (.z _returnvalue) 0.0))
  (bind _returnvalue_3 (select Y (.y _returnvalue) _returnvalue_2))
  (bind _returnvalue_4 (select X (.x _returnvalue) _returnvalue_3))
  (bind _returnvalue_5 (Math|Float|InRange(Float) _returnvalue_4 Min Max))
  (if (Math|Vector|NotEqual(Vector) Amount "0, 0, 0" 0.1)
    (if _returnvalue_5
      (Transformation|AddLocalOffset Component Amount false false)
      (return true false)
      (else
        (return false true)))
    (else
      (return false _returnvalue_5))))

(fn UpdateZComponenttoUse
  (params (Movement%20Value :type Float%20%28single-precision%29))
  (if (Math|Boolean|NORBoolean (> (+ Movement%20Value (Variables|Internal|Movement|GetCurrent%20Height)) 0.0) (< (+ Movement%20Value (Variables|Internal|Movement|GetCurrent%20Height)) (* (+ (Variables|Internal|Movement|GetMax%20Height) (Variables|Settings|GetCrane%20Max%20Height%20Offset)) -1.0)))
    (bind _output_get (Variables|Internal|Movement|SetCurrent%20Height (+ Movement%20Value (Variables|Internal|Movement|GetCurrent%20Height))))
    (for (_array_element _array_index) (Variables|Internal|Movement|GetHeight%20Meshes%20Bounds)
      (if (> _output_get (* _array_element -1.0))
        (return (Utilities|Array|Get(acopy) (Variables|Internal|Movement|GetHeight%20Meshes) _array_index))))
    (else
      (return 0))))

(fn GetFinalOverrideforSound
  (if true
    (return (<= (+ (Math|Float|Absolute(Float) (Variables|Internal|Input|GetInput%20X)) (Math|Float|Absolute(Float) (Variables|Internal|Input|GetInput%20Y)) (Math|Float|Absolute(Float) (Variables|Internal|Input|GetInput%20Z))) 1.0))
    (else
      (return false))))

(fn SetOverrideSound
  (params (Should%20Override :type Boolean))
  (if true
    _))

(fn GetWidgetInputs
  (switch Utilities|FlowControl|Switch|SwitchonE_Platform (CallFunction|GetCurrentPlatform)
    (:NewEnumerator0
      (return (Utilities|Map|MakeMap "Up" (Utilities|Struct|MakeStruct_Image_Set "/Game/_Overseas/Art/Saskia/Meshes/2D/Q_Knop.Q_Knop" "/Game/_Overseas/Art/Saskia/Meshes/2D/Q_Pressed_Knop.Q_Pressed_Knop") "Down" (Utilities|Struct|MakeStruct_Image_Set "/Game/_Overseas/Art/Saskia/Meshes/2D/E_Knop.E_Knop" "/Game/_Overseas/Art/Saskia/Meshes/2D/E_Pressed_Knop.E_Pressed_Knop") "Left" (Utilities|Struct|MakeStruct_Image_Set "/Game/_Overseas/Art/Saskia/Meshes/2D/A_Knop.A_Knop" "/Game/_Overseas/Art/Saskia/Meshes/2D/A_Pressed_Knop.A_Pressed_Knop") "Right" (Utilities|Struct|MakeStruct_Image_Set "/Game/_Overseas/Art/Saskia/Meshes/2D/D_Knop.D_Knop" "/Game/_Overseas/Art/Saskia/Meshes/2D/D_Pressed_Knop.D_Pressed_Knop") "Forward" (Utilities|Struct|MakeStruct_Image_Set "/Game/_Overseas/Art/Saskia/Meshes/2D/W_Knop.W_Knop" "/Game/_Overseas/Art/Saskia/Meshes/2D/W_Pressed_Knop.W_Pressed_Knop") "Backwards" (Utilities|Struct|MakeStruct_Image_Set "/Game/_Overseas/Art/Saskia/Meshes/2D/S_Knop.S_Knop" "/Game/_Overseas/Art/Saskia/Meshes/2D/S_Pressed_Knop.S_Pressed_Knop") "Toggle Torpedo" (Utilities|Struct|MakeStruct_Image_Set "/Game/_Overseas/Art/Saskia/Meshes/2D/Spatie_Knop.Spatie_Knop" "/Game/_Overseas/Art/Saskia/Meshes/2D/Spatie_Pressed_Knop.Spatie_Pressed_Knop") "Back" (Utilities|Struct|MakeStruct_Image_Set "/Game/_Overseas/Art/Saskia/Meshes/2D/Esc_Knop.Esc_Knop" "/Game/_Overseas/Art/Saskia/Meshes/2D/Esc_Pressed_Knop.Esc_Pressed_Knop") "Confirm" (Utilities|Struct|MakeStruct_Image_Set "/Game/_Overseas/Art/Saskia/Meshes/2D/Enter_Knop.Enter_Knop" "/Game/_Overseas/Art/Saskia/Meshes/2D/Enter_Pressed_Knop.Enter_Pressed_Knop"))))
    (:NewEnumerator1
      (return (Utilities|Map|MakeMap "Up" "" "Down" "" "Left" "" "Right" "" "Forward" "" "Backwards" "" "Toggle Torpedo" "" "Back" "")))))

(fn UpdateInputUI
  (params (Direction :type E_Direction%20Enum :default "NewEnumerator0") (Clicked :type Boolean))
  (bind _returnvalue (Utilities|Select :Index Direction :NewEnumerator0 "Up" :NewEnumerator1 "Down" :NewEnumerator2 "Left" :NewEnumerator3 "Right" :NewEnumerator4 "Forward" :NewEnumerator5 "Backwards"))
  (bind _crane_widget (Variables|Internal|General|GetCrane%20Widget)
    (:then
      (Default|UpdateInput _crane_widget _returnvalue _returnvalue (select Clicked "Clicked" "")))
    (:else)))