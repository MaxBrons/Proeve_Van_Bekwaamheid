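; Interactable ship torpedo rack that triggers a torpedo transfer once enough players use it: one when solo, two in multiplayer.
; The authority tracks interacting players, while a lone owning player may see the rack widget.
; The transfer calls TorpedoTransfered, wrapped in a camera fade for participants, then unfocuses them and resets its DoOnce.
; Unfocusing sends the player's list index as a key name for server removal, and Comp_Active toggles interaction.
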(event ActiveStateChanged(Comp_Active)
  (params (Pawn :type BP%20Pawn%20Base%20Object%20Reference) (Comp%20Active :type Comp%20Active%20Object%20Reference) (New%20Active :type Boolean))
  ;[1 1 1] Set the interaction enabled or disabled, so that the player can or can't interact with the rack.
  (Default|SetInteractionEnabled (Variables|Default|GetComp_Interaction) New%20Active))

(event PressedInteraction(Comp_Interaction)
  (params (Pawn :type BP%20Pawn%20Base%20Object%20Reference) (Souce%20Actor :type Actor%20Object%20Reference) (Hit%20Location :type Vector :default "0, 0, 0") (Hit%20Distance :type Float%20%28single-precision%29) (Hit%20Component :type Actor%20Component%20Object%20Reference))
  (bind _self self)
  (bind _players_interacted (Variables|Internal|GetPlayers%20Interacted))
  ;[1 1 1] Check if it is allowed to interact with the object and switch the input to this object.
  (Utilities|IsReplicatedOwner Pawn
    (:Owner
      (Default|SwitchInput (CallFunction|GetMainPlayerController _self) _self true false))
    (:Not%20Owner
      _))
  ;[1 1 1] Increase the index for checking how many players are currently interacting with this obejct and spawn in a torpedo if at least one player is interacting, if mulitplayer there have to be two players minimum.
  (Networking|SwitchHasAuthority
    (:Authority
      (Math|Integer|IncrementInt _players_interacted
        (:%20%20
          (Utilities|Array|Add (Variables|Internal|GetInteracted%20Players) Pawn)
          (bind _asbp_game_mode_main (Utilities|Casting|CastToBP_GameMode_Main (Game|GetGameMode)))
          (if (>= _players_interacted (Math|Integer|SelectInt 1 2 (<= (Utilities|Map|Length (Variables|/Game/_Overseas/Development/Game/BP_GameMode_Main.BP_GameMode_Main_C|GetPlayer%20List _asbp_game_mode_main)) 1)))
            (Utilities|FlowControl|DoOnce false
              (:Completed
                (CallFunction|TransferTorpedo)))
            (else
              (Utilities|IsReplicatedOwner Pawn :!label _label
                (:Owner
                  (if (not (>= (Variables|Internal|GetPlayers%20Interacted) 2))
                    (bind _asbp_pawn_screen (Utilities|Casting|CastToBP_Pawn_Screen Pawn))
                    (Default|AddWidgettoViewport _asbp_pawn_screen "Torpedo Rack" (Variables|Internal|GetTorpedo%20Rack%20Widget))))))))))
    (:Remote
      (goto _label))))

(event Custom|Transfer%20Torpedo
  (bind _self self)
  ;[1 1 1] Do a fade in and out. In between the fade, spawn in the new torpedo and place it in on the location that is set in the editor.
  (if (Utilities|Array|ContainsItem (Variables|Internal|GetInteracted%20Players) (CallFunction|GetMainPlayerPawn self))
    (CameraFades|StartCameraFade :self (Game|GetPlayerCameraManager 0) :ToAlpha 1.0 :Duration 1.0 :bHoldWhenFinished true)
    (Utilities|FlowControl|Delay 0.75)
    (Default|CallTorpedoTransfered _self)
    (Utilities|FlowControl|Delay 0.75)
    (CameraFades|StartCameraFade :self (Game|GetPlayerCameraManager 0) :FromAlpha 1.0 :Duration 1.0)
    (CallFunction|Unfocus)
    (else
      (Utilities|FlowControl|Delay 0.75)
      (Default|CallTorpedoTransfered _self)))
  (CallFunction|Reset))

(event Custom|Unfocus
  (bind _self self)
  (bind _player_pawn (CallFunction|GetMainPlayerPawn _self))
  ;[1 1 1] Unfocus from the object and decrease the index for checking how many players are currently interacting
  (Default|SwitchInput (CallFunction|GetMainPlayerController _self) _self false false)
  (bind _asbp_pawn_screen (Utilities|Casting|CastToBP_Pawn_Screen _player_pawn))
  (Default|RemoveWidgetfromViewport _asbp_pawn_screen "Torpedo Rack")
  (Default|PressKey _asbp_pawn_screen self (Utilities|String|StringToName (Utilities|String|ToString(Integer) (Utilities|Array|FindItem (Variables|Internal|GetInteracted%20Players) _player_pawn)))))

(event Custom|Reset
  ;[1 1 1] Increase the index for checking how many players are currently interacting with this obejct and spawn in a torpedo if at least one player is interacting, if mulitplayer there have to be two players minimum.
  (Utilities|FlowControl|DoOnce false) ; enters at Reset
)

(event EventBeginPlay
  (bind _returnvalue (UserInterface|CreateWidget "/Game/_Overseas/Development/Blueprints/Widgets/HUD/Task_Screens/WB_Screen_Torpedo_Rack.WB_Screen_Torpedo_Rack_C" 0 0 0))
  (Variables|Internal|SetTorpedo%20Rack%20Widget _returnvalue))

(event EventInteractionPressed
  (params (Key%20Code :type Name :default "None"))
  ;[1 1 1] Remove the player from the list on the server
  (Networking|SwitchHasAuthority
    (:Authority
      (Utilities|Array|RemoveIndex (Variables|Internal|GetInteracted%20Players) (Math|Conversions|ToInteger(Byte) (Utilities|String|ToString(Name) Key%20Code)))
      (Math|Integer|DecrementInt (Variables|Internal|GetPlayers%20Interacted)))))

(event Input|ActionEvents|InputActionReturn
  (params (Key :type Key%20Structure :default "None"))
  (bind _self self)
  (bind _player_pawn (CallFunction|GetMainPlayerPawn _self))
  ;[1 1 1] Unfocus from the object and decrease the index for checking how many players are currently interacting
  (:Pressed
    (Default|SwitchInput (CallFunction|GetMainPlayerController _self) _self false false)
    (bind _asbp_pawn_screen (Utilities|Casting|CastToBP_Pawn_Screen _player_pawn))
    (Default|RemoveWidgetfromViewport _asbp_pawn_screen "Torpedo Rack")
    (Default|PressKey _asbp_pawn_screen self (Utilities|String|StringToName (Utilities|String|ToString(Integer) (Utilities|Array|FindItem (Variables|Internal|GetInteracted%20Players) _player_pawn))))))

(fn ConstructionScript)

(fn OnRepPlayersInteracted)

(fn GetPlayerbyName
  (params (Object%20Name :type Name))
  (for _array_element (Variables|Internal|GetPlayer%20List)
    (if (Utilities|Enum|Equal(Enum) (Utilities|GetObjectName _array_element) (Utilities|String|ToString(Name) Object%20Name))
      (return _array_element)))
  (return 0))