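; Ship door that fade-transfers the interacting pawn to a linked door's teleport position and can be locked as part of a two-door code puzzle.
; DisableDoor has authority block interaction and generate a random code, then shows either that code or an out-of-order sign, depending on CompActive.
; Keypad input is compared against the corresponding door's code, and a match re-enables both doors.
; The code display polls with a short delay until the code is non-empty.
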(event PressedInteraction(Comp_Interaction)
  (params (Pawn :type BP%20Pawn%20Base%20Object%20Reference) (Souce%20Actor :type Actor%20Object%20Reference) (Hit%20Location :type Vector :default "0, 0, 0") (Hit%20Distance :type Float%20%28single-precision%29) (Hit%20Component :type Actor%20Component%20Object%20Reference))
  (bind _self self)
  ;[1 1 1] Transfer the player to the new location.
  (Utilities|IsReplicatedOwner Pawn
    (:Owner
      (bind _door_to_transfer_to (Variables|Settings|GetDoor%20To%20Transfer%20To)
        (:then
          (Default|TransferPawn (CallFunction|GetMainPlayerController self) Pawn (.Location (CallFunction|GetTeleportLocation _door_to_transfer_to)) (.Rotation (CallFunction|GetTeleportLocation _door_to_transfer_to)) true))
        (:else)))
    (:Not%20Owner
      _))
  (Variables|/Game/_Overseas/Development/Game/BP_PlayerController_Main.BP_PlayerController_Main_C|SetLast%20Entered%20Door (CallFunction|GetMainPlayerController _self) _self)
  (Default|CallDoorEntered Pawn Souce%20Actor))

(event WidgetFunctionality(Comp_Widget_Keypad)
  (params (Command :type Name :default "None") (Object%20Reference :type Object%20Object%20Reference) (Options :type String))
  (bind _returnvalue (Math|Conversions|ToInteger(Byte) Options))
  ;[1 1 1] Set the current keycode that the player has entered in the keypad.
  (Utilities|FlowControl|Sequence
    (:then_0
      (if (Variables|Internal|GetLocked)
        (switch name Command
          (:Enter
            (Variables|Internal|SetCurrent%20Keypad%20Sequence _returnvalue)
            (bind _corresponding_door (Variables|Internal|GetCorresponding%20Door)
              (:then
                (if (CallFunction|CompareCodeSequence _corresponding_door _returnvalue)
                  (CallFunction|EnableDoor)
                  (CallFunction|EnableDoor (Variables|Internal|GetCorresponding%20Door))
                  (bind _keypad_widget (Variables|Default|GetKeypad%20Widget)
                    (:then
                      (Default|SetupWidget _keypad_widget 10))
                    (:else))))
              (:else))))))
    (:then_1
      (switch name Command
        (:Add%20Number
          (bind _keypad_widget_2 (Variables|Default|GetKeypad%20Widget)
            (:then
              (Default|AddNumbertoSequence _keypad_widget_2 Options))
            (:else)))
        (:Remove%20Number
          (bind _keypad_widget_3 (Variables|Default|GetKeypad%20Widget)
            (:then
              (Default|RemoveNumber _keypad_widget_3))
            (:else)))
        (:Enter
          (bind _keypad_widget_4 (Variables|Default|GetKeypad%20Widget)
            (:then
              (Default|SetupWidget _keypad_widget_4 10))
            (:else)))))))

(event Custom|Disable%20Door
  (params (Corresponding%20Door :type BP%20Door%20Object%20Reference))
  ;[1 1 1] Disable the door. Depending on the active state of the comp active it will display a code or a disabled sign. The code has to be entered in the other door's keypad.
  (Rendering|SetVisibility (Variables|Default|GetComp_Widget_Front) true false)
  (Variables|Internal|SetCorresponding%20Door Corresponding%20Door)
  (Variables|Internal|SetLocked true)
  (Default|CallOnDoorLocked)
  (bind _aswb_door_front (Utilities|Casting|CastToWB_Door_Front (UserInterface|GetUserWidgetObject (Variables|Default|GetComp_Widget_Front))))
  (Networking|SwitchHasAuthority
    (:Authority
      (Default|SetInteractionEnabled (Variables|Default|GetComp_Interaction) false)
      (Variables|Internal|SetCurrent%20Code%20Sequence (CallFunction|GenerateRandomCode)))
    (:Remote
      _))
  (if (Variables|/Game/_Overseas/Development/Blueprints/Components/Core/Comp_Active.Comp_Active_C|GetActive (Variables|Default|GetComp_Active))
    (if (> (Utilities|String|Len (Variables|Internal|GetCurrent%20Code%20Sequence)) 0) :!label _label
      (Default|SetupWidget _aswb_door_front (Variables|Internal|GetCurrent%20Code%20Sequence) true)
      (Rendering|SetVisibility (Variables|Default|GetComp_Widget_Keypad) false false)
      (else
        (Utilities|FlowControl|Delay 0.05)
        (goto _label)))
    (else
      (Default|SetupWidget _aswb_door_front "Buiten Gebruik" false "(R=1.000000,G=0.000000,B=0.000000,A=1.000000)")
      (Rendering|SetVisibility (Variables|Default|GetComp_Widget_Keypad) true false))))

(event Custom|Enable%20Door
  ;[1 1 1] Reset the door to a normal state.
  (Rendering|SetVisibility (Variables|Default|GetComp_Widget_Front) false false)
  (Variables|Internal|SetCorresponding%20Door 0)
  (Rendering|SetVisibility (Variables|Default|GetComp_Widget_Keypad) true false)
  (Variables|Internal|SetLocked false)
  (Default|CallOnDoorUnlocked)
  (Networking|SwitchHasAuthority
    (:Authority
      (Variables|Internal|SetCurrent%20Code%20Sequence "")
      (Default|SetInteractionEnabled (Variables|Default|GetComp_Interaction) true))))

(event EventBeginPlay
  ;[1 1 1] Setup the keypad widget and enable the door.
  (bind _aswb_keypad (Utilities|Casting|CastToWB_Keypad (UserInterface|GetUserWidgetObject (Variables|Default|GetComp_Widget_Keypad))))
  (bind _output_get (Variables|Default|SetKeypad%20Widget _aswb_keypad))
  (Default|SetupWidget _output_get 10)
  (CallFunction|EnableDoor)
  (Default|OnDestroyedEvent0 (Variables|Default|GetComp_Widget_Front)))

(fn ConstructionScript)

(fn GetTeleportLocation
  (bind _player_teleport_position (Variables|Default|GetPlayer%20Teleport%20Position))
  (return (Transformation|GetWorldLocation _player_teleport_position) (Transformation|GetWorldRotation _player_teleport_position)))

(fn GenerateRandomCode
  (for _index (range 0 3)
    (LocalVariables|SetCode (Utilities|String|Append (LocalVariables|GetCode) (Utilities|String|ToString(Integer) (Math|Random|RandomInteger 9)))))
  (return (LocalVariables|GetCode)))

(fn CompareCodeSequence
  (params (Code%20To%20Compare :type Integer))
  (return (== Code%20To%20Compare (Math|Conversions|ToInteger(Byte) (Variables|Internal|GetCurrent%20Code%20Sequence)))))