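; Torpedo trolley actor that carries a torpedo and can be snapped to a torpedo tube.
; LoadTorpedo attaches the torpedo through server-to-multicast events, then eases it onto the TorpedoLocation point with a VInterpTo and Delay loop.
; An overlap box checks for tagged components, with a DoOnce gating the TorpedoTubeReached call.
; Snapping passes a location and rotation to a server event that moves the trolley.
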(event OnComponentBeginOverlap(TorepdoBuisBox)
  (params (OverlappedComponent :type Primitive%20Component%20Object%20Reference) (OtherActor :type Actor%20Object%20Reference) (OtherComp :type Primitive%20Component%20Object%20Reference) (OtherBodyIndex :type Integer) (bFromSweep :type Boolean) (SweepResult :type Hit%20Result%20Structure%20%28by%20ref%29))
  (if (Components|ComponentHasTag OtherComp (Variables|Settings|GetTorpedo%20Buis%20Tag))
    _))

(event OnComponentEndOverlap(TorepdoBuisBox)
  (params (OverlappedComponent :type Primitive%20Component%20Object%20Reference) (OtherActor :type Actor%20Object%20Reference) (OtherComp :type Primitive%20Component%20Object%20Reference) (OtherBodyIndex :type Integer))
  (if (Components|ComponentHasTag OtherComp (Variables|Settings|GetTorpedo%20Buis%20Tag))
    (Utilities|FlowControl|DoOnce false ; enters at Reset
      (:Completed
        (Default|CallTorpedoTubeReached)))))

(event Custom|Snap%20To%20Torpedo%20Tube%20Location
  (params (Location :type Vector) (Rotation :type Rotator))
  (CallFunction|ServerSnaptoTorpedoTubeLocation Location Rotation))

(event Custom|Server_Snap%20To%20Torpedo%20Tube%20Location
  (params (Location :type Vector) (Rotation :type Rotator))
  (Transformation|SetActorLocationAndRotation Location Rotation))

(event Custom|Multi_Load%20Torpedo
  (params (Torpedo :type BP%20Torpedo%20Object%20Reference))
  (Transformation|AttachActorToActor Torpedo self "None" "KeepWorld" "KeepWorld" "KeepWorld" true))

(event Custom|Load%20Torpedo
  (params (Torpedo :type BP%20Torpedo%20Object%20Reference))
  (bind _returnvalue (Transformation|GetActorLocation Torpedo))
  (bind _torpedo_location (Variables|Default|GetTorpedo%20Location))
  (bind _returnvalue_2 (Transformation|GetWorldLocation _torpedo_location))
  (Utilities|IsValid Torpedo
    (:Is%20Valid
      (bind _output_get (Variables|Internal|SetTorpedo Torpedo))
      (CallFunction|ServerLoadTorpedo _output_get)
      (if (not (Math|Float|NearlyEqual(Float) (Math|Vector|VectorLength (- _returnvalue _returnvalue_2)) 0.0 1.0)) :!label _label
        (Transformation|SetActorLocation (Variables|Internal|GetTorpedo) (Math|Interpolation|VInterpTo _returnvalue _returnvalue_2 (Utilities|Time|GetWorldDeltaSeconds) 1.0) false false)
        (Utilities|FlowControl|Delay 0.01)
        (goto _label)))))

(event Custom|Server_Load%20Torpedo
  (params (Torpedo :type BP%20Torpedo%20Object%20Reference))
  (CallFunction|MultiLoadTorpedo Torpedo))

(event EventBeginPlay
  (|CallParentFunction) ; This node is disabled and will not be called.\nDrag off pins to build functionality.
)

(fn ConstructionScript)