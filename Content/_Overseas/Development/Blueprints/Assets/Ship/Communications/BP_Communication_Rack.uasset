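; Ship communication rack with a radio that players focus on and tune with Left/Right, turning a knob and updating the frequency widget.
; The server picks a random start frequency, and key presses reach everyone via the player controller and multicast events.
; While focused, Tick lets only the server change the frequency, wrapping at the limits, as all machines animate the knob.
; Clients refresh the display again once tuning stops.
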(event PressedInteraction(Comp_Focus)
  (params (Pawn :type BP%20Pawn%20Base%20Object%20Reference) (Souce%20Actor :type Actor%20Object%20Reference) (Hit%20Location :type Vector :default "0, 0, 0") (Hit%20Distance :type Float%20%28single-precision%29) (Hit%20Component :type Actor%20Component%20Object%20Reference))
  ;[1 1 1] Enable the tick of the actor on server and client.
  (Networking|SwitchHasAuthority
    (:Authority
      (Default|SetInteractionEnabled (Variables|Default|GetComp_Focus) false))
    (:Remote
      _))
  (Actor|Tick|SetActorTickEnabled true))

(event Custom|Multi_Interaction%20Released
  (params (Selection :type Name))
  ;[1 1 1] Handle the input.
  (CallFunction|InteractionReleased Selection))

(event Custom|Multi_Interaction%20Pressed
  (params (Selection :type Name))
  ;[1 1 1] Handle the input.
  (CallFunction|InteractionPressed Selection))

(event EventBeginPlay
  ;[1 1 1] Set the radio widget and set the start frequency.
  (bind _aswb_radio_frequency (Utilities|Casting|CastToWB_Radio_Frequency (UserInterface|GetUserWidgetObject (Variables|Default|GetComp_Widget))))
  (bind _output_get (Variables|Internal|SetRadio%20Widget _aswb_radio_frequency))
  (Networking|SwitchHasAuthority
    (:Authority
      (Variables|Internal|SetCurrent%20Frequency (Math|Random|RandomFloatinRange (Variables|Settings|GetMin%20Frequency) (Variables|Settings|GetMax%20Frequency))))
    (:Remote
      (Utilities|FlowControl|Delay 0.5)))
  (Default|SetupWidget _output_get (Variables|Internal|GetCurrent%20Frequency)))

(event EventTick
  (params (DeltaSeconds :type Float%20%28single-precision%29))
  ;[1 1 1] Handle the rotation from the knob and set the frequency accordingly.
  (if (!= (Variables|Internal|GetCurrent%20Axis) 0.0)
    (Utilities|FlowControl|Sequence
      (:then_0
        (goto _label Reset))
      (:then_1
        (Networking|SwitchHasAuthority
          (:Authority
            (Variables|Internal|SetCurrent%20Frequency (select (> (+ (Variables|Internal|GetCurrent%20Frequency) (* (Variables|Internal|GetCurrent%20Axis) DeltaSeconds (Variables|Internal|GetFrequency%20Change%20Speed))) (Variables|Settings|GetMax%20Frequency)) (Variables|Settings|GetMin%20Frequency) (select (< (+ (Variables|Internal|GetCurrent%20Frequency) (* (Variables|Internal|GetCurrent%20Axis) DeltaSeconds (Variables|Internal|GetFrequency%20Change%20Speed))) (Variables|Settings|GetMin%20Frequency)) (Variables|Settings|GetMax%20Frequency) (+ (Variables|Internal|GetCurrent%20Frequency) (* (Variables|Internal|GetCurrent%20Axis) DeltaSeconds (Variables|Internal|GetFrequency%20Change%20Speed)))))))
          (:Remote
            _))
        (bind _radio_widget (Variables|Internal|GetRadio%20Widget)
          (:then
            (Default|SetupWidget _radio_widget (Variables|Internal|GetCurrent%20Frequency))
            (Transformation|AddLocalRotation (Variables|Default|GetKnop) (Math|Rotator|MakeRotator 0.0 (* (* (Variables|Internal|GetCurrent%20Axis) (Variables|Internal|GetFrequency%20Change%20Speed)) -1.0) 0.0) false false))
          (:else))))
    (else
      (Utilities|FlowControl|DoOnce false :!label _label
        (:Completed
          (Networking|SwitchHasAuthority
            (:Remote
              (bind _radio_widget_2 (Variables|Internal|GetRadio%20Widget)
                (:then
                  (Default|SetupWidget _radio_widget_2 (Variables|Internal|GetCurrent%20Frequency)))
                (:else)))))))))

(event EventInteractionPressed
  (params (Key%20Code :type Name :default "None"))
  ;[1 1 1] Handle the input.
  (switch name Key%20Code
    (:Left
      (Variables|Internal|SetCurrent%20Axis -1.0))
    (:Right
      (Variables|Internal|SetCurrent%20Axis 1.0))
    (:Esc
      (Actor|Tick|SetActorTickEnabled false))))

(event EventInteractionReleased
  (params (Key%20Code :type Name :default "None"))
  ;[1 1 1] Handle the input.
  (switch name Key%20Code
    (:Left
      _)
    (:Right
      _))
  (Variables|Internal|SetCurrent%20Axis 0.0))

(event Input|ActionEvents|InputActionLeft
  (params (Key :type Key%20Structure :default "None"))
  ;[1 1 1] Handle the input.
  (:Pressed
    (Utilities|HandleInteraction "Left" :!label _label))
  (:Released
    (goto _label Released)))

(event Input|ActionEvents|InputActionRight
  (params (Key :type Key%20Structure :default "None"))
  ;[1 1 1] Handle the input.
  (:Pressed
    (Utilities|HandleInteraction "Right" :!label _label))
  (:Released
    (goto _label Released)))

(event Input|ActionEvents|InputActionReturn
  (params (Key :type Key%20Structure :default "None"))
  ;[1 1 1] Handle the input.
  (:Pressed
    (Default|Unfocus (Variables|Default|GetComp_Focus))
    (Utilities|HandleInteraction "Esc")))

(fn ConstructionScript)