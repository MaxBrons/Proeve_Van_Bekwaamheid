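; Torpedo trolley actor that detects arrival at a torpedo tube and can snap into place there.
; An overlap with a TorpedoBuisTag component fires TorpedoTubeReached once, provided LocationToSnapTo is valid, and re-arms when that overlap ends.
; A separate snap event relays through server and multicast events to set the trolley's location and rotation to that target actor's transform.
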(event OnComponentBeginOverlap(TorepdoBuisBox)
  (params (OverlappedComponent :type Primitive%20Component%20Object%20Reference) (OtherActor :type Actor%20Object%20Reference) (OtherComp :type Primitive%20Component%20Object%20Reference) (OtherBodyIndex :type Integer) (bFromSweep :type Boolean) (SweepResult :type Hit%20Result%20Structure%20%28by%20ref%29))
  (if (Components|ComponentHasTag OtherComp (Variables|Settings|GetTorpedo%20Buis%20Tag))
    (Variables|Settings|GetLocation%20To%20Snap%20To
      (:then
        (Utilities|FlowControl|DoOnce false
          (:Completed
            (Default|CallTorpedoTubeReached))))
      (:else))
    (else
      (for _array_element (Variables|/Script/Engine.ActorComponent|GetComponentTags OtherComp)
        _))))

(event OnComponentEndOverlap(TorepdoBuisBox)
  (params (OverlappedComponent :type Primitive%20Component%20Object%20Reference) (OtherActor :type Actor%20Object%20Reference) (OtherComp :type Primitive%20Component%20Object%20Reference) (OtherBodyIndex :type Integer))
  (if (Components|ComponentHasTag OtherComp (Variables|Settings|GetTorpedo%20Buis%20Tag))
    (Utilities|FlowControl|DoOnce false) ; enters at Reset
  ))

(event Custom|Multi_Snap%20To%20Torpedo%20Tube%20Location
  (bind _location_to_snap_to (Variables|Settings|GetLocation%20To%20Snap%20To)
    (:then
      (Transformation|SetActorLocationAndRotation (.location (Transformation|GetActorTransform _location_to_snap_to)) (.rotation (Transformation|GetActorTransform _location_to_snap_to))))
    (:else)))

(event Custom|Snap%20To%20Torpedo%20Tube%20Location
  (CallFunction|ServerSnaptoTorpedoTubeLocation))

(event Custom|Server_Snap%20To%20Torpedo%20Tube%20Location
  (CallFunction|MultiSnaptoTorpedoTubeLocation))

(event EventBeginPlay
  (|CallParentFunction) ; This node is disabled and will not be called.\nDrag off pins to build functionality.
)

(fn ConstructionScript)