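; Cannon ammo deposit where players store and take cannon ammo.
; On interaction, a held crate adds its capacity if it fits, held ammo adds one, and empty hands spawn and pick up one if available.
; The count drives visibility of three crate meshes, roughly one per six rounds.
; Authority gates interactions with a delayed DoOnce reset while remotes run ungated; the active component toggles interactability.
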(event PressedInteraction(Comp_Interaction)
  (params (Pawn :type BP%20Pawn%20Base%20Object%20Reference) (Souce%20Actor :type Actor%20Object%20Reference) (Hit%20Location :type Vector :default "0, 0, 0") (Hit%20Distance :type Float%20%28single-precision%29) (Hit%20Component :type Actor%20Component%20Object%20Reference))
  (bind _asbp_pawn_desktop (Utilities|Casting|CastToBP_Pawn_Desktop Pawn))
  (Variables|Default|SetPlayerPawn _asbp_pawn_desktop)
  (Networking|SwitchHasAuthority
    (:Authority
      (Utilities|FlowControl|DoOnce false :!label _label
        (:Completed
          _)))
    (:Remote
      _))
  (Utilities|IsValid (Variables|/Game/_Overseas/Development/Blueprints/Pawns/BP_Pawn_Desktop.BP_Pawn_Desktop_C|GetItemInHands (Variables|Default|GetPlayerPawn))
    (:Is%20Valid
      (bind _asbp_ammo_crate (Utilities|Casting|CastToBP_AmmoCrate (Variables|/Game/_Overseas/Development/Blueprints/Pawns/BP_Pawn_Desktop.BP_Pawn_Desktop_C|GetItemInHands (Variables|Default|GetPlayerPawn)))
        (:then
          (CallFunction|AddAmmoChest _asbp_ammo_crate)
          (Default|CallOnAmmoAdded)
          (Networking|SwitchHasAuthority
            (:Authority
              (Utilities|FlowControl|Delay 0.1)
              (goto _label Reset))))
        (:CastFailed
          (bind _asbp_cannon_ammo (Utilities|Casting|CastToBP_CannonAmmo (Variables|/Game/_Overseas/Development/Blueprints/Pawns/BP_Pawn_Desktop.BP_Pawn_Desktop_C|GetItemInHands (Variables|Default|GetPlayerPawn))))
          (Default|ItemDropDown _asbp_cannon_ammo (Variables|Default|GetPlayerPawn))
          (CallFunction|IncreaseAmmo)
          (Networking|SwitchHasAuthority
            (:Authority
              (Utilities|FlowControl|Delay 0.1)
              (goto _label Reset))))))
    (:Is%20Not%20Valid
      (if (> (Variables|Default|GetAmmoCount) 0)
        (Variables|/Game/_Overseas/Development/Blueprints/Pawns/BP_Pawn_Desktop.BP_Pawn_Desktop_C|SetHoldingObjectInHands (Variables|Default|GetPlayerPawn) true)
        (bind _returnvalue (Game|SpawnActorfromClass "/Game/_Overseas/Development/Blueprints/Assets/Cannon/BP_CannonAmmo.BP_CannonAmmo_C" (Math|Transform|MakeTransform "0, 0, 0" "0, 0, 0" "1,1,1") "Undefined" 0 0))
        (Default|ItemPickedUp _returnvalue (Variables|Default|GetPlayerPawn) (Variables|Default|GetSocket%20Name))
        (CallFunction|DecreaseAmmo)
        (Networking|SwitchHasAuthority
          (:Authority
            (Utilities|FlowControl|Delay 0.1)
            (goto _label Reset)))
        (else
          (Networking|SwitchHasAuthority
            (:Authority
              (Utilities|FlowControl|Delay 0.2)
              (goto _label Reset))))))))

(event ActiveStateChanged(Comp_Active)
  (params (Pawn :type BP%20Pawn%20Base%20Object%20Reference) (Comp%20Active :type Comp%20Active%20Object%20Reference) (New%20Active :type Boolean))
  (Default|SetInteractionEnabled (Variables|Default|GetComp_Interaction) New%20Active))

(event EventBeginPlay
  (for _array_element (Components|GetChildrenComponents (Variables|Default|GetDepositMesh) false)
    (Rendering|SetVisibility _array_element false true)))

(event Collision|EventActorBeginOverlap
  (params (OtherActor :type Actor%20Object%20Reference)))

(event EventTick
  (params (DeltaSeconds :type Float%20%28single-precision%29)))

(fn ConstructionScript
  (Variables|Default|SetAmmoCrates (Utilities|Array|MakeArray (Variables|Default|GetSM_AmmoCrateHalfOpen) (Variables|Default|GetSM_AmmoCrateHalfOpen1) (Variables|Default|GetSM_AmmoCrateHalfOpen2))))

(fn AddAmmoChest
  (params (AmmoCrate :type BP%20Ammo%20Crate%20Object%20Reference))
  (bind _ammocapicity (Variables|/Game/_Overseas/Development/Blueprints/Assets/Cannon/BP_AmmoCrate.BP_AmmoCrate_C|GetAmmoCapicity AmmoCrate))
  (bind _playerpawn (Variables|Default|GetPlayerPawn))
  (if (<= (+ (Variables|Default|GetAmmoCount) _ammocapicity) (Variables|Default|GetMaxAmmo))
    (Rendering|SetVisibility (Utilities|Array|Get(acopy) (Variables|Default|GetAmmoCrates) (Variables|Default|GetCrateCount)) true true)
    (Math|Integer|IncrementInt (Variables|Default|GetCrateCount)
      (:%20%20
        (Variables|Default|SetAmmoCount (+ (Variables|Default|GetAmmoCount) _ammocapicity))
        (Default|ItemDropDown (Variables|/Game/_Overseas/Development/Blueprints/Pawns/BP_Pawn_Desktop.BP_Pawn_Desktop_C|GetItemInHands _playerpawn) _playerpawn)
        (return)))))

(fn DecreaseAmmo
  (bind _cratecount (Variables|Default|GetCrateCount))
  (bind _output_get (Variables|Default|SetAmmoCount (- (Variables|Default|GetAmmoCount) 1)))
  (if (or (== (- (* (Variables|Default|GetCrateCount) 6) 1) 0) (< (Math|Float|Ceil (/ (Math|Conversions|ToFloat(Integer) _output_get) 6.0)) (Variables|Default|GetCrateCount)))
    (Math|Integer|DecrementInt _cratecount
      (:%20%20
        (Rendering|SetVisibility (Utilities|Array|Get(acopy) (Variables|Default|GetAmmoCrates) _cratecount) false true))))
  (return))

(fn IncreaseAmmo
  (bind _cratecount (Variables|Default|GetCrateCount))
  (bind _output_get (Variables|Default|SetAmmoCount (+ (Variables|Default|GetAmmoCount) 1)))
  (if (< (Variables|Default|GetCrateCount) (Math|Float|Ceil (/ (Math|Conversions|ToFloat(Integer) _output_get) 6.0)))
    (Rendering|SetVisibility (Utilities|Array|Get(acopy) (Variables|Default|GetAmmoCrates) _cratecount) true true)
    (Math|Integer|IncrementInt _cratecount
      (:%20%20
        _)))
  (return))