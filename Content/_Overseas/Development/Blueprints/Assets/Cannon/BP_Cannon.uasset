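; Cannon actor that players load by interacting while holding a BP_CannonAmmo item, and that spends one round per CannonShoot call.
; The construction script collects TurningGear's child meshes as hidden bullets and sets ammo capacity from the child count.
; Loading drops the held item, reveals a bullet and rotates the Scene component by timeline, while shooting hides one and rotates back.
; Ammo changes fire the OnSetAmmo dispatcher.
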(event PressedInteraction(Comp_Interaction)
  (params (Pawn :type BP%20Pawn%20Base%20Object%20Reference) (Souce%20Actor :type Actor%20Object%20Reference) (Hit%20Location :type Vector :default "0, 0, 0") (Hit%20Distance :type Float%20%28single-precision%29) (Hit%20Component :type Actor%20Component%20Object%20Reference))
  (bind _asbp_pawn_desktop (Utilities|Casting|CastToBP_Pawn_Desktop Pawn))
  (bind _output_get (Variables|Default|SetPlayerPawn _asbp_pawn_desktop))
  (Variables|/Game/_Overseas/Development/Blueprints/Pawns/BP_Pawn_Desktop.BP_Pawn_Desktop_C|GetItemInHands _output_get
    (:then
      (if (<= (+ (Variables|Default|GetAmmo) 1) (Variables|Default|GetMaxAmmo))
        (Networking|SwitchHasAuthority
          (:Authority
            (Utilities|FlowControl|DoOnce false :!label _label
              (:Completed
                _)))
          (:Remote
            _))
        (Utilities|Casting|CastToBP_CannonAmmo (Variables|/Game/_Overseas/Development/Blueprints/Pawns/BP_Pawn_Desktop.BP_Pawn_Desktop_C|GetItemInHands (Variables|Default|GetPlayerPawn))
          (:then
            (CallFunction|LoadCannon)
            (goto _label Reset))
          (:CastFailed
            (goto _label Reset)))))
    (:else)))

(event Custom|LoadCannon
  (bind _scene (Variables|Default|GetScene))
  (bind _ammo (Variables|Default|GetAmmo))
  (bind _playerpawn (Variables|Default|GetPlayerPawn))
  (Variables|Default|SetStartRotation (Variables|/Script/Engine.SceneComponent|GetRelativeRotation _scene))
  (Rendering|SetVisibility (Utilities|Array|Get(acopy) (Variables|Default|GetBullets) _ammo) true false)
  (Default|ItemDropDown (Variables|/Game/_Overseas/Development/Blueprints/Pawns/BP_Pawn_Desktop.BP_Pawn_Desktop_C|GetItemInHands _playerpawn) _playerpawn)
  (CallFunction|SetAmmo (+ _ammo 1))
  (bind _newtrack_0 (Timeline|Timeline_0 PlayFromStart)
    (:Update
      (Transformation|SetRelativeRotation _scene (Math|Rotator|MakeRotator 0.0 0.0 (+ (.yaw (Variables|Default|GetStartRotation)) _newtrack_0)) false false))))

(event Custom|CannonShoot
  (bind _scene (Variables|Default|GetScene))
  (bind _ammo (Variables|Default|GetAmmo))
  (bind _returnvalue (- _ammo 1))
  (if (>= (- (Variables|Default|GetAmmo) 1) 0)
    (Variables|Default|SetStartRotation (Variables|/Script/Engine.SceneComponent|GetRelativeRotation _scene))
    (Rendering|SetVisibility (Utilities|Array|Get(acopy) (Variables|Default|GetBullets) _returnvalue) false false)
    (CallFunction|SetAmmo _returnvalue)
    (bind _newtrack_0 (Timeline|Timeline_1 PlayFromStart)
      (:Update
        (Transformation|SetRelativeRotation _scene (Math|Rotator|MakeRotator 0.0 0.0 (- (.yaw (Variables|Default|GetStartRotation)) _newtrack_0)) false false))
      (:Finished
        (if (== _returnvalue 0)
          (Transformation|SetRelativeRotation (Variables|Default|GetScene) "0, 0, 0" false false))))))

(event Custom|SetAmmo
  (params (New%20Ammo :type Integer))
  (bind _output_get (Variables|Default|SetAmmo New%20Ammo))
  (Default|CallOnSetAmmo _output_get))

(event EventBeginPlay)

(event Collision|EventActorBeginOverlap
  (params (OtherActor :type Actor%20Object%20Reference)))

(event EventTick
  (params (DeltaSeconds :type Float%20%28single-precision%29)))

(fn ConstructionScript
  (bind _turninggear (Variables|Default|GetTurningGear))
  (bind _children (Components|GetChildrenComponents _turninggear false))
  (for _array_element _children
    (bind _asstatic_mesh_component (Utilities|Casting|CastToStaticMeshComponent _array_element))
    (Utilities|Array|Add (Variables|Default|GetBullets) _asstatic_mesh_component)
    (Rendering|SetVisibility _asstatic_mesh_component false false))
  (Variables|Default|SetMaxAmmo (Utilities|Array|Length _children)))

(fn HasAnoughAmmo
  (return (> (Variables|Default|GetAmmo) 0)))