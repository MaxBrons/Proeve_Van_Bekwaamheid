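; Interactable cannon station that plays a targeting minigame against enemy cannon ships on the ship's course.
; Focusing it enables input and shows a key-hint HUD; course and ammo updates feed the screen widget.
; Input routes through the pawn's PressKey into InteractionPressed, which moves the cursor, randomizes target spawns and fires hits or misses.
; Shots call BP_Cannon; hits damage the current enemy and, on destruction, notify EnemyShipHandler and recheck the course.
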(event ActiveStateChanged(Comp_Active)
  (params (Pawn :type BP%20Pawn%20Base%20Object%20Reference) (Comp%20Active :type Comp%20Active%20Object%20Reference) (New%20Active :type Boolean))
  (bind _canoninterfacewidget (Variables|Default|GetCanonInterFaceWidget))
  (Utilities|WaitforObjecttoValidate _canoninterfacewidget 0.05
    (:Is%20Valid
      (Default|SetCanonInterfaceEnabled _canoninterfacewidget New%20Active)
      (Networking|SwitchHasAuthority
        (:Authority
          (Default|SetInteractionEnabled (Variables|Default|GetComp_Focus) New%20Active))))))

(event PressedInteraction(Comp_Focus)
  (params (Pawn :type BP%20Pawn%20Base%20Object%20Reference) (Souce%20Actor :type Actor%20Object%20Reference) (Hit%20Location :type Vector :default "0, 0, 0") (Hit%20Distance :type Float%20%28single-precision%29) (Hit%20Component :type Actor%20Component%20Object%20Reference))
  (Variables|Default|SetCurrent%20Pawn (CallFunction|GetMainPlayerPawn self))
  (Networking|SwitchHasAuthority
    (:Authority
      (Default|SetInteractionEnabled (Variables|Default|GetComp_Focus) false))
    (:Remote
      _))
  (Actor|Tick|SetActorTickEnabled true)
  (Utilities|IsReplicatedOwner Pawn
    (:Owner
      (bind _asbp_pawn_screen (Utilities|Casting|CastToBP_Pawn_Screen Pawn))
      (bind _cannon_widget (Variables|Default|GetCannon%20Widget)
        (:then
          (Default|AddWidgettoViewport _asbp_pawn_screen "Cannon" _cannon_widget)
          (bind _cannon_widget_2 (Variables|Default|GetCannon%20Widget)
            (:then
              (bind _images (CallFunction|GetInputWidgets))
              (Default|SetupWidgetInput _cannon_widget_2 _images))
            (:else)))
        (:else)))))

(event Custom|CheckIfEnemyCannonShipIsInCourse
  (params (Course :type Float%20%28single-precision%29))
  (bind _canoninterfacewidget (Variables|Default|GetCanonInterFaceWidget))
  (bind (_hit _enemyship) (Default|CannonShipinRange (Variables|Default|GetEnemyShipHandler) Course))
  (if _hit
    (Default|EnemyFound _canoninterfacewidget)
    (Utilities|IsValid _enemyship
      (:Is%20Valid
        (bind _asbp_enemy_canon_ship (Utilities|Casting|CastToBP_Enemy_CanonShip _enemyship))
        (Variables|Default|SetCurrentEnemy _asbp_enemy_canon_ship)))
    (else
      (Default|EnemyNotFound _canoninterfacewidget))))

(event Custom|AmmoAmountChanged
  (params (Ammo :type Integer))
  (Default|SetAmmo (Variables|Default|GetCanonInterFaceWidget) Ammo))

(event Custom|ShootMis
  (Utilities|FlowControl|DoOnce false :!label _label
    (:Completed
      (Default|CannonShoot (Variables|Default|GetCannonAmmo))
      (Utilities|FlowControl|Delay 0.2)
      (goto _label Reset))))

(event Custom|StartGame
  (bind _current_pawn (Variables|Default|GetCurrent%20Pawn))
  (Utilities|WaitforObjecttoValidate _current_pawn 0.05
    (:Is%20Valid
      (Default|PressKey _current_pawn self "StartGame"))))

(event Custom|ServerRandom
  (Variables|Default|SetRandomInt (Utilities|Select :Index (Math|Random|RandomIntegerinRange 0 1) :Option%200 0 :Option%201 1))
  (Variables|Default|SetRandom%20Float (Math|Random|RandomFloatinRange -5.5e+02 5.5e+02)))

(event Custom|Shoot%20Hit
  (bind _this_ship (Variables|Default|GetThis%20Ship))
  (bind _current_course (Variables|/Game/_Overseas/Development/Blueprints/Systems/Ship/BP_Ship.BP_Ship_C|GetCurrent%20Course _this_ship))
  (Default|CannonShoot (Variables|Default|GetCannonAmmo))
  (bind _is_death (Default|DoDamage (Variables|Default|GetCurrentEnemy)))
  (if _is_death
    (Default|TrytoHitShipwithTorpedo (Variables|Default|GetEnemyShipHandler) _current_course "NewEnumerator1")
    (Default|CallEnemyDestroyed)
    (CallFunction|CheckifEnemyCannonShipIsinCourse _current_course))
  (Networking|SwitchHasAuthority
    (:Authority
      (bind _current_pawn (Variables|Default|GetCurrent%20Pawn)
        (:then
          (Default|PressKey _current_pawn self "StartGame"))
        (:else)))))

(event EventInteractionPressed
  (params (Key%20Code :type Name :default "None"))
  (bind _canoninterfacewidget (Variables|Default|GetCanonInterFaceWidget))
  (switch name Key%20Code
    (:W
      (Default|CursorMoveUpDown _canoninterfacewidget -1.0))
    (:S
      (Default|CursorMoveUpDown _canoninterfacewidget 1.0))
    (:D
      (Default|CursorLeftRight _canoninterfacewidget 1.0))
    (:A
      (Default|CursorLeftRight _canoninterfacewidget -1.0))
    (:StartGame
      (CallFunction|ServerRandom)
      (Default|RandomSpawnandMoveDirection (Variables|Default|GetCanonInterFaceWidget) (Variables|Default|GetRandomInt) (Variables|Default|GetRandom%20Float)))
    (:Shoot%20Hit
      (CallFunction|ShootHit))
    (:Shoot%20Mis
      (CallFunction|ShootMis))
    (:Esc
      (Default|SetInteractionEnabled (Variables|Default|GetComp_Focus) true)
      (Actor|Tick|SetActorTickEnabled false)
      (Development|PrintString "Hello"))))

(event Collision|EventActorBeginOverlap
  (params (OtherActor :type Actor%20Object%20Reference)))

(event EventBeginPlay
  (Audio|Components|Audio|Stop (Variables|Default|GetAudio))
  (EventDispatchers|BindEventtoCourseUpdate (Variables|Default|GetThis%20Ship) (delegate Custom|CheckIfEnemyCannonShipIsInCourse))
  (bind _returnvalue (UserInterface|CreateWidget "/Game/_Overseas/Development/Blueprints/Widgets/HUD/Task_Screens/WB_Screen_Cannon.WB_Screen_Cannon_C" 0 0 0))
  (Variables|Default|SetCannon%20Widget _returnvalue)
  (bind _aswb_cannon_interface (Utilities|Casting|CastToWB_CannonInterface (UserInterface|GetWidget (Variables|Default|GetComp_Widget))))
  (Variables|Default|SetCanonInterFaceWidget _aswb_cannon_interface)
  (bind _returnvalue_2 (Actor|GetActorOfClass "/Game/_Overseas/Development/Blueprints/Assets/Cannon/BP_Cannon.BP_Cannon_C"))
  (bind _output_get (Variables|Default|SetCannonAmmo _returnvalue_2))
  (EventDispatchers|BindEventtoOnSetAmmo _output_get (delegate Custom|AmmoAmountChanged))
  (EventDispatchers|BindEventtoCloseDone (Variables|/Game/_Overseas/Development/Blueprints/Widgets/Systems/CanonWidget/WB_CannonInterface.WB_CannonInterface_C|GetWB_CannonStartScreen_C_1 _aswb_cannon_interface) (delegate Custom|StartGame))
  (Variables|/Game/_Overseas/Development/Blueprints/Widgets/Systems/CanonWidget/WB_CannonInterface.WB_CannonInterface_C|SetCanon _aswb_cannon_interface self))

(event Input|ActionEvents|InputActionReturn
  (params (Key :type Key%20Structure :default "None"))
  (:Pressed
    (bind _cannon_widget (Variables|Default|GetCannon%20Widget)
      (:then
        (Default|UpdateInput _cannon_widget "Back" "Back" "Clicked")
        (Utilities|FlowControl|Delay 0.2))
      (:else
        _))
    (Default|Unfocus (Variables|Default|GetComp_Focus))
    (Default|PressKey (Variables|Default|GetCurrent%20Pawn) self "Esc")
    (bind _asbp_pawn_screen (Utilities|Casting|CastToBP_Pawn_Screen (CallFunction|GetMainPlayerPawn self)))
    (Variables|Default|GetCannon%20Widget
      (:then
        (Default|RemoveWidgetfromViewport _asbp_pawn_screen "Cannon"))
      (:else))))

(event Input|ActionEvents|InputActionDown
  (params (Key :type Key%20Structure :default "None"))
  (bind _self self)
  (bind _current_pawn (Variables|Default|GetCurrent%20Pawn))
  (:Pressed
    (bind _cannon_widget (Variables|Default|GetCannon%20Widget)
      (:then
        (Default|UpdateInput _cannon_widget "Shoot" "Shoot" "Clicked"))
      (:else
        _))
    (Variables|Default|GetCurrentEnemy
      (:then
        (bind _anoughammo (Default|HasAnoughAmmo (Variables|Default|GetCannonAmmo)))
        (if _anoughammo
          (bind _enemyinrange (Default|CheckifEnemyIsinRange (Variables|Default|GetCanonInterFaceWidget)))
          (if _enemyinrange
            (Default|PressKey _current_pawn _self "Shoot Hit")
            (else
              (Default|PressKey _current_pawn _self "Shoot Mis")))
          (Audio|Components|Audio|Play (Variables|Default|GetAudio) 0.0)))
      (:else)))
  (:Released
    (bind _cannon_widget_2 (Variables|Default|GetCannon%20Widget)
      (:then
        (Default|UpdateInput _cannon_widget_2 "Shoot" "Shoot"))
      (:else))))

(event Input|ActionEvents|InputActionLeft
  (params (Key :type Key%20Structure :default "None"))
  (:Pressed
    (CallFunction|UpdateInputUI "Left" true))
  (:Released
    (CallFunction|UpdateInputUI "Left" false)))

(event Input|ActionEvents|InputActionRight
  (params (Key :type Key%20Structure :default "None"))
  (:Pressed
    (CallFunction|UpdateInputUI "Right" true))
  (:Released
    (CallFunction|UpdateInputUI "Right" false)))

(event Input|ActionEvents|InputActionForward
  (params (Key :type Key%20Structure :default "None"))
  (:Pressed
    (CallFunction|UpdateInputUI "Up" true))
  (:Released
    (CallFunction|UpdateInputUI "Up" false)))

(event Input|ActionEvents|InputActionBackwards
  (params (Key :type Key%20Structure :default "None"))
  (:Pressed
    (CallFunction|UpdateInputUI "Down" true))
  (:Released
    (CallFunction|UpdateInputUI "Down" false)))

(event Input|AxisEvents|InputAxisMoveForward
  (params (AxisValue :type Float%20%28single-precision%29))
  (bind _returnvalue (> AxisValue 0.1))
  (bind _self self)
  (bind _current_pawn (Variables|Default|GetCurrent%20Pawn))
  (if (or (< AxisValue -0.1) _returnvalue)
    (if _returnvalue
      (Default|PressKey _current_pawn _self "W")
      (else
        (Default|PressKey _current_pawn _self "S")))))

(event Input|AxisEvents|InputAxisMoveRight
  (params (AxisValue :type Float%20%28single-precision%29))
  (bind _returnvalue (> AxisValue 0.1))
  (bind _self self)
  (bind _current_pawn (Variables|Default|GetCurrent%20Pawn))
  (if (or (< AxisValue -0.1) _returnvalue)
    (if _returnvalue
      (Default|PressKey _current_pawn _self "D")
      (else
        (Default|PressKey _current_pawn _self "A")))))

(fn ConstructionScript)

(fn GetInputWidgets
  (switch Utilities|FlowControl|Switch|SwitchonE_Platform (CallFunction|GetCurrentPlatform)
    (:NewEnumerator0
      (return (Utilities|Map|MakeMap "Up" (Utilities|Struct|MakeStruct_Image_Set "/Game/_Overseas/Art/Saskia/Meshes/2D/W_Knop.W_Knop" "/Game/_Overseas/Art/Saskia/Meshes/2D/W_Pressed_Knop.W_Pressed_Knop") "Down" (Utilities|Struct|MakeStruct_Image_Set "/Game/_Overseas/Art/Saskia/Meshes/2D/S_Knop.S_Knop" "/Game/_Overseas/Art/Saskia/Meshes/2D/S_Pressed_Knop.S_Pressed_Knop") "Left" (Utilities|Struct|MakeStruct_Image_Set "/Game/_Overseas/Art/Saskia/Meshes/2D/A_Knop.A_Knop" "/Game/_Overseas/Art/Saskia/Meshes/2D/A_Pressed_Knop.A_Pressed_Knop") "Right" (Utilities|Struct|MakeStruct_Image_Set "/Game/_Overseas/Art/Saskia/Meshes/2D/D_Knop.D_Knop" "/Game/_Overseas/Art/Saskia/Meshes/2D/D_Pressed_Knop.D_Pressed_Knop") "Shoot" (Utilities|Struct|MakeStruct_Image_Set "/Game/_Overseas/Art/Saskia/Meshes/2D/E_Knop.E_Knop" "/Game/_Overseas/Art/Saskia/Meshes/2D/E_Pressed_Knop.E_Pressed_Knop") "Back" (Utilities|Struct|MakeStruct_Image_Set "/Game/_Overseas/Art/Saskia/Meshes/2D/Esc_Knop.Esc_Knop" "/Game/_Overseas/Art/Saskia/Meshes/2D/Esc_Pressed_Knop.Esc_Pressed_Knop"))))
    (:NewEnumerator1
      (return (Utilities|Map|MakeMap "Up" (Utilities|Struct|MakeStruct_Image_Set "/Game/_Overseas/Art/Saskia/Meshes/2D/W_Knop.W_Knop" "/Game/_Overseas/Art/Saskia/Meshes/2D/W_Pressed_Knop.W_Pressed_Knop") "Down" (Utilities|Struct|MakeStruct_Image_Set "/Game/_Overseas/Art/Saskia/Meshes/2D/S_Knop.S_Knop" "/Game/_Overseas/Art/Saskia/Meshes/2D/S_Pressed_Knop.S_Pressed_Knop") "Left" (Utilities|Struct|MakeStruct_Image_Set "/Game/_Overseas/Art/Saskia/Meshes/2D/A_Knop.A_Knop" "/Game/_Overseas/Art/Saskia/Meshes/2D/A_Pressed_Knop.A_Pressed_Knop") "Right" (Utilities|Struct|MakeStruct_Image_Set "/Game/_Overseas/Art/Saskia/Meshes/2D/D_Knop.D_Knop" "/Game/_Overseas/Art/Saskia/Meshes/2D/D_Pressed_Knop.D_Pressed_Knop") "Shoot" (Utilities|Struct|MakeStruct_Image_Set "/Game/_Overseas/Art/Saskia/Meshes/2D/E_Knop.E_Knop" "/Game/_Overseas/Art/Saskia/Meshes/2D/E_Pressed_Knop.E_Pressed_Knop") "Back" (Utilities|Struct|MakeStruct_Image_Set "/Game/_Overseas/Art/Saskia/Meshes/2D/Esc_Knop.Esc_Knop" "/Game/_Overseas/Art/Saskia/Meshes/2D/Esc_Pressed_Knop.Esc_Pressed_Knop"))))))

(fn UpdateInputUI
  (params (Input%20Name :type Name) (Clicked :type Boolean))
  (bind _cannon_widget (Variables|Default|GetCannon%20Widget)
    (:then
      (Default|UpdateInput _cannon_widget Input%20Name Input%20Name (Utilities|String|SelectString "Clicked" "" Clicked)))
    (:else)))