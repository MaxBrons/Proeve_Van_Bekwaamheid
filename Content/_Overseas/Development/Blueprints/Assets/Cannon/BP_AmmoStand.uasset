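; Ammo stand, filed with cannon assets, where desktop players pick up or return ammo crates.
; The interaction component stores the pawn and calls PressKey on the main player controller, targeting the stand.
; InteractionPressed spawns and attaches a crate when hands are empty, or drops a held crate.
; It runs on authority and remote, with a briefly delayed DoOnce reset debouncing the authority side.
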(event PressedInteraction(Comp_Interaction)
  (params (Pawn :type BP%20Pawn%20Base%20Object%20Reference) (Souce%20Actor :type Actor%20Object%20Reference) (Hit%20Location :type Vector :default "0, 0, 0") (Hit%20Distance :type Float%20%28single-precision%29) (Hit%20Component :type Actor%20Component%20Object%20Reference))
  (bind _asbp_pawn_desktop (Utilities|Casting|CastToBP_Pawn_Desktop Pawn))
  (Variables|Default|SetPlayerPawn _asbp_pawn_desktop)
  (bind _asbp_player_controller_main (Utilities|Casting|CastToBP_PlayerController_Main (Game|GetPlayerController 0)))
  (Default|PressKey _asbp_player_controller_main self "None"))

(event EventBeginPlay)

(event Collision|EventActorBeginOverlap
  (params (OtherActor :type Actor%20Object%20Reference)))

(event EventTick
  (params (DeltaSeconds :type Float%20%28single-precision%29)))

(event EventInteractionPressed
  (params (Key%20Code :type Name :default "None"))
  (bind _playerpawn (Variables|Default|GetPlayerPawn))
  (Variables|Default|GetPlayerPawn
    (:then
      (Networking|SwitchHasAuthority
        (:Authority
          (Utilities|FlowControl|DoOnce false :!label _label
            (:Completed
              _)))
        (:Remote
          _))
      (if (Variables|/Game/_Overseas/Development/Blueprints/Pawns/BP_Pawn_Desktop.BP_Pawn_Desktop_C|GetHoldingObjectInHands (Variables|Default|GetPlayerPawn))
        (bind _asbp_ammo_crate (Utilities|Casting|CastToBP_AmmoCrate (Variables|/Game/_Overseas/Development/Blueprints/Pawns/BP_Pawn_Desktop.BP_Pawn_Desktop_C|GetItemInHands (Variables|Default|GetPlayerPawn))))
        (Utilities|IsValid _asbp_ammo_crate
          (:Is%20Valid
            (Default|ItemDropDown (Variables|/Game/_Overseas/Development/Blueprints/Pawns/BP_Pawn_Desktop.BP_Pawn_Desktop_C|GetItemInHands _playerpawn) _playerpawn)
            (Default|CallOnItemDropped)
            (Networking|SwitchHasAuthority
              (:Authority
                (Utilities|FlowControl|Delay 0.1)
                (goto _label Reset)))))
        (else
          (Variables|/Game/_Overseas/Development/Blueprints/Pawns/BP_Pawn_Desktop.BP_Pawn_Desktop_C|SetHoldingObjectInHands (Variables|Default|GetPlayerPawn) true)
          (bind _returnvalue (Game|SpawnActorfromClass "/Game/_Overseas/Development/Blueprints/Assets/Cannon/BP_AmmoCrate.BP_AmmoCrate_C" (Math|Transform|MakeTransform "0, 0, 0" "0, 0, 0" "1,1,1") "Undefined" 0 0))
          (Default|ItemPickedUp _returnvalue (Variables|Default|GetPlayerPawn) (Variables|Default|GetSocketAmmoName))
          (Default|CallOnItemPickedUp)
          (Networking|SwitchHasAuthority
            (:Authority
              (Utilities|FlowControl|Delay 0.1)
              (goto _label Reset))))))
    (:else)))

(fn ConstructionScript)