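; BP_Item is a carriable item, apparently a cannon ammo chest, that a player holds in their hands.
; On pickup it snaps to a given socket on the player mesh, registers as the held item and sets the player's holding and animation Blueprint's ammo-chest flags.
; On drop it clears both flags and destroys itself rather than detaching, provided the animation Blueprint cast succeeds.
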(event Custom|ItemPickedUp
  (params (player :type BP%20Pawn%20Desktop%20Object%20Reference) (SocketName :type Name))
  (Transformation|AttachComponentToComponent (Variables|/Script/Engine.Character|GetMesh player) SocketName "SnapToTarget" "SnapToTarget" "SnapToTarget" true)
  (Variables|/Game/_Overseas/Development/Blueprints/Pawns/BP_Pawn_Desktop.BP_Pawn_Desktop_C|SetItemInHands player self)
  (bind _asmixamo_base_skeleton_anim_blueprint (Utilities|Casting|CastToMixamo_Base_Skeleton_AnimBlueprint (Components|SkeletalMesh|GetAnimInstance (Variables|/Script/Engine.Character|GetMesh player))))
  (Variables|/Game/_Overseas/Art/Selina/Models/Character_Animations/Mixamo_Base_Skeleton_AnimBlueprint.Mixamo_Base_Skeleton_AnimBlueprint_C|SetHasAmmoChest _asmixamo_base_skeleton_anim_blueprint true)
  (Variables|/Game/_Overseas/Development/Blueprints/Pawns/BP_Pawn_Desktop.BP_Pawn_Desktop_C|SetHoldingObjectInHands player true))

(event Custom|ItemDropDown
  (params (Player :type BP%20Pawn%20Desktop%20Object%20Reference))
  (bind _asmixamo_base_skeleton_anim_blueprint (Utilities|Casting|CastToMixamo_Base_Skeleton_AnimBlueprint (Components|SkeletalMesh|GetAnimInstance (Variables|/Script/Engine.Character|GetMesh Player))))
  (Variables|/Game/_Overseas/Art/Selina/Models/Character_Animations/Mixamo_Base_Skeleton_AnimBlueprint.Mixamo_Base_Skeleton_AnimBlueprint_C|SetHasAmmoChest _asmixamo_base_skeleton_anim_blueprint false)
  (Variables|/Game/_Overseas/Development/Blueprints/Pawns/BP_Pawn_Desktop.BP_Pawn_Desktop_C|SetHoldingObjectInHands Player false)
  (Actor|DestroyActor))

(event EventBeginPlay)

(event Collision|EventActorBeginOverlap
  (params (OtherActor :type Actor%20Object%20Reference)))

(event EventTick
  (params (DeltaSeconds :type Float%20%28single-precision%29)))

(fn ConstructionScript)