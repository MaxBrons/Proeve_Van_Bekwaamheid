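; BP_Survival_Timer is a clock actor that counts how long players survive and shows it on a WB_AlarmClock widget component.
; On authority, the enemy ship manager's first spawn event starts a one-second looping timer, and the GameIsOver event stops it.
; Each tick saves the time to the game instance and calls RPM_SetGameTimer to update the widget.
; An IsLobbyClock instance also displays the saved time on BeginPlay.
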(event Custom|StartGameTimer
  (params (Ship%20Reference :type BP%20Enemy%20Ship%20Object%20Reference) (Spawn%20Location :type Vector))
  (bind _returnvalue (Actor|GetActorOfClass "/Game/_Overseas/Development/Blueprints/Systems/Enemy_Ship/BP_Enemy_Ship_Manager.BP_Enemy_Ship_Manager_C"))
  (EventDispatchers|UnbindEventfromOnShipSpawned (stale EventBeginPlay _returnvalue) (delegate Custom|StartGameTimer))
  (bind _returnvalue_2 (Utilities|Time|SetTimerbyEvent (delegate Custom|RPS_StartGameTimer) 1.0 true))
  (Variables|Default|SetTimerHandle _returnvalue_2))

(event Custom|RPM_SetGameTimer
  (Variables|/Game/_Overseas/Development/Blueprints/Widgets/Systems/Clock/WB_AlarmClock.WB_AlarmClock_C|SetTimeInSeconds (Variables|Default|GetClockWidget) (Variables|Default|GetTimeInSeconds)))

(event Custom|RPS_StartGameTimer
  (Variables|Default|SetTimeInSeconds (+ (Variables|Default|GetTimeInSeconds) 1.0))
  (Variables|/Game/_Overseas/Development/Game/BP_GameInstance_Main.BP_GameInstance_Main_C|SetTimePlayersSurvived (Variables|Default|GetGameMode) (Variables|Default|GetTimeInSeconds))
  (CallFunction|RPMSetGameTimer))

(event Custom|StopTimer
  (Utilities|Time|ClearandInvalidateTimerbyHandle (Variables|Default|GetTimerHandle)))

(event EventBeginPlay
  (Networking|SwitchHasAuthority
    (:Authority
      (bind _asbp_game_instance_main (Utilities|Casting|CastToBP_GameInstance_Main (Game|GetGameInstance)))
      (EventDispatchers|BindEventtoGameIsOver _asbp_game_instance_main (delegate Custom|StopTimer))
      (bind _returnvalue (Actor|GetActorOfClass "/Game/_Overseas/Development/Blueprints/Systems/Enemy_Ship/BP_Enemy_Ship_Manager.BP_Enemy_Ship_Manager_C"))
      (Utilities|IsValid _returnvalue
        (:Is%20Valid
          (EventDispatchers|BindEventtoOnShipSpawned _returnvalue (delegate Custom|StartGameTimer)))
        (:Is%20Not%20Valid
          _))
      (bind _asbp_game_instance_main_2 (Utilities|Casting|CastToBP_GameInstance_Main (Game|GetGameInstance)))
      (Variables|Default|SetGameMode _asbp_game_instance_main_2))
    (:Remote
      _))
  (bind _aswb_alarm_clock (Utilities|Casting|CastToWB_AlarmClock (UserInterface|GetWidget (Variables|Default|GetComp_Widget))))
  (Variables|/Game/_Overseas/Development/Blueprints/Widgets/Systems/Clock/WB_AlarmClock.WB_AlarmClock_C|SetTimeInSeconds _aswb_alarm_clock (Variables|Default|GetTimeInSeconds))
  (Variables|Default|SetClockWidget _aswb_alarm_clock)
  (if (Variables|Default|GetIsLobbyClock)
    (Networking|SwitchHasAuthority
      (:Authority
        (Variables|Default|SetTimeInSeconds (Variables|/Game/_Overseas/Development/Game/BP_GameInstance_Main.BP_GameInstance_Main_C|GetTimePlayersSurvived (Variables|Default|GetGameMode)))
        (CallFunction|RPMSetGameTimer)))))

(event Collision|EventActorBeginOverlap
  (params (OtherActor :type Actor%20Object%20Reference)))

(event EventTick
  (params (DeltaSeconds :type Float%20%28single-precision%29)))

(fn ConstructionScript)