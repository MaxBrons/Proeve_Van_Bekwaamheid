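; Manager for the breakable, repairable rooms that handles random room damage, hammer-driven wall selection and room destruction notification.
; On BeginPlay it gathers rooms and their walls' select components, binds hammer and health events, and puts the hammer in the first slot.
; Grabbing or releasing the hammer toggles wall selection for the owning player only.
; The server picks three distinct random rooms and multicasts their damage; any room reaching zero health triggers RoomDestroyed.
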(event Custom|Multi_DamageRoom
  (params (Room%20To%20Damage :type Array%20of%20Integers))
  (for _array_element Room%20To%20Damage
    (Utilities|IsValid (Utilities|Array|Get(acopy) (Variables|Internal|GetBreakable%20Rooms) _array_element)
      (:Is%20Valid
        (Default|Damage (Utilities|Array|Get(acopy) (Variables|Internal|GetBreakable%20Rooms) _array_element) 35.0)))))

(event Custom|Damage%20Random%20Rooms
  (CallFunction|ServerDamageRoom))

(event Custom|Grabbed
  (params (Pawn :type BP%20Pawn%20Base%20Object%20Reference) (Hammer%20Reference :type BP%20Hammer%20Object%20Reference))
  (Utilities|IsReplicatedOwner Pawn
    (:Owner
      (for _array_element (Variables|Internal|GetSelect%20Components)
        (Default|SetSelectedEnabled _array_element true)))))

(event Custom|Released
  (params (Pawn :type BP%20Pawn%20Base%20Object%20Reference) (Hammer%20Reference :type BP%20Hammer%20Object%20Reference))
  (Utilities|IsReplicatedOwner Pawn
    (:Owner
      (for _array_element (Variables|Internal|GetSelect%20Components)
        (Default|SetSelectedEnabled _array_element false)))))

(event Custom|Server_DamageRoom
  (bind _room_indexes (CallFunction|GetRandomRooms 3))
  (CallFunction|MultiDamageRoom _room_indexes))

(event Custom|On%20Health%20Updated
  (params (Current%20Health :type Float%20%28single-precision%29))
  (if (<= Current%20Health 0.0)
    (Default|CallOnRoomDestroyed)))

(event EventBeginPlay
  (bind _self self)
  (bind _player_pawn (CallFunction|GetMainPlayerPawn _self))
  (Utilities|FlowControl|Sequence
    (:then_0
      (bind _outactors (Actor|GetAllActorsOfClass "/Game/_Overseas/Development/Blueprints/Assets/Repairing/BP_Breakable_Rooms.BP_Breakable_Rooms_C"))
      (bind _output_get (Variables|Internal|SetBreakable%20Rooms _outactors))
      (bind _select_components (CallFunction|GetSelectComponents _output_get))
      (Variables|Internal|SetSelect%20Components _select_components)
      (bind _returnvalue (Actor|GetActorOfClass "/Game/_Overseas/Development/Blueprints/Assets/Repairing/BP_Hammer.BP_Hammer_C"))
      (Utilities|IsValid _returnvalue
        (:Is%20Valid
          (EventDispatchers|BindEventtoOnGrabbed _returnvalue (delegate Custom|Grabbed))
          (EventDispatchers|BindEventtoOnReleased _returnvalue (delegate Custom|Released))
          (bind _outactors_2 (Actor|GetAllActorsOfClass "/Game/_Overseas/Development/Blueprints/Assets/Repairing/BP_Hammer_Slot.BP_Hammer_Slot_C"))
          (bind _output_get_2 (Variables|Internal|SetHammer%20Slots _outactors_2))
          (Utilities|IsValid (Utilities|Array|Get(acopy) _output_get_2)
            (:Is%20Valid
              (Default|OccupySlot (Utilities|Array|Get(acopy) _output_get_2) _returnvalue))))))
    (:then_1
      (Utilities|WaitforObjecttoValidate _player_pawn 0.05
        (:Is%20Valid
          (CallFunction|Released _player_pawn))))
    (:then_2
      (for _array_element (Variables|Internal|GetBreakable%20Rooms)
        (EventDispatchers|BindEventtoOnHealthUpdated _array_element (delegate Custom|On%20Health%20Updated))))))

(fn ConstructionScript)

(fn GetSelectComponents
  (params (Rooms :type Array%20of%20BP%20Breakable%20Rooms%20Object%20References))
  (for _array_element Rooms
    (for _array_element_2 (Variables|/Game/_Overseas/Development/Blueprints/Assets/Repairing/BP_Breakable_Rooms.BP_Breakable_Rooms_C|GetWalls%20To%20Damage _array_element)
      (Utilities|IsValid (Actor|GetComponentbyClass _array_element_2 "/Game/_Overseas/Development/Blueprints/Components/Core/Comp_Select.Comp_Select_C")
        (:Is%20Valid
          (Utilities|Array|Add (LocalVariables|GetReturn) (Actor|GetComponentbyClass _array_element_2 "/Game/_Overseas/Development/Blueprints/Components/Core/Comp_Select.Comp_Select_C"))))))
  (return (LocalVariables|GetReturn)))

(fn GetHammerfromPlayer
  (params (Pawn :type BP%20Pawn%20Base%20Object%20Reference))
  (for _array_element (Actor|GetAttachedActors Pawn true)
    (if (or (== (Utilities|GetClass _array_element) "/Game/_Overseas/Development/Blueprints/Assets/Repairing/BP_Hammer.BP_Hammer_C") (Utilities|ClassIsChildOf (Utilities|GetClass _array_element) "/Game/_Overseas/Development/Blueprints/Assets/Repairing/BP_Hammer.BP_Hammer_C"))
      (bind _asbp_hammer (Utilities|Casting|CastToBP_Hammer _array_element))
      (return _asbp_hammer))))

(fn GetRandomRooms
  (params (Amount :type Integer))
  (for _index (range 0 (- Amount 1))
    (bind _output_get (LocalVariables|SetCurrent%20Index (Math|Random|RandomIntegerinRange 0 (- (Utilities|Array|Length (Variables|Internal|GetBreakable%20Rooms)) 1)) :!label _label))
    (if (Utilities|Array|ContainsItem (LocalVariables|GetIndexes) _output_get)
      (goto _label)
      (else
        (Utilities|Array|Add (LocalVariables|GetIndexes) _output_get))))
  (return (LocalVariables|GetIndexes)))