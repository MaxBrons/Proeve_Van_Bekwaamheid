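; BP_Hammer is a grabbable hammer item that a screen pawn picks up through its interaction component.
; On press, the owning pawn calls GrabHammer, the authority disables interaction, collision turns off and OnGrabbed fires.
; Release restores collision and fires OnReleased.
; It caches the breakable-rooms manager at BeginPlay and offers a lookup for a hammer attached to a pawn.
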(event PressedInteraction(Comp_Interaction)
  (params (Pawn :type BP%20Pawn%20Base%20Object%20Reference) (Souce%20Actor :type Actor%20Object%20Reference) (Hit%20Location :type Vector :default "0, 0, 0") (Hit%20Distance :type Float%20%28single-precision%29) (Hit%20Component :type Actor%20Component%20Object%20Reference))
  (bind _self self)
  (Utilities|IsReplicatedOwner Pawn
    (:Owner
      (bind _asbp_pawn_screen (Utilities|Casting|CastToBP_Pawn_Screen Pawn))
      (Default|GrabHammer _asbp_pawn_screen _self))
    (:Not%20Owner
      _))
  (Networking|SwitchHasAuthority
    (:Authority
      (Default|SetInteractionEnabled (Variables|Default|GetComp_Interaction) false))
    (:Remote
      _))
  (Collision|SetActorEnableCollision false)
  (Default|CallOnGrabbed Pawn _self))

(event Custom|Release%20Hammer
  (params (Pawn :type BP%20Pawn%20Base%20Object%20Reference))
  (Default|CallOnReleased Pawn self)
  (Collision|SetActorEnableCollision true))

(event EventBeginPlay
  (bind _returnvalue (Actor|GetActorOfClass "/Game/_Overseas/Development/Blueprints/Assets/Repairing/BP_Manager_Breakable_Rooms.BP_Manager_Breakable_Rooms_C"))
  (Variables|Internal|SetRoom%20Manager _returnvalue))

(fn ConstructionScript)

(fn GetHammerfromPlayer
  (params (Pawn :type BP%20Pawn%20Base%20Object%20Reference))
  (for _array_element (Actor|GetAttachedActors Pawn true)
    (if (or (== (Utilities|GetClass _array_element) "BP_Hammer_C") (Utilities|ClassIsChildOf (Utilities|GetClass _array_element) "BP_Hammer_C"))
      (bind _asbp_hammer (Utilities|Casting|CastToBP_Hammer _array_element))
      (return _asbp_hammer))))