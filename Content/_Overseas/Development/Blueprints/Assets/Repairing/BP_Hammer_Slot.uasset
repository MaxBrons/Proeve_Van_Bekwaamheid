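; BP_Hammer_Slot is a holder actor where a player puts down a repair hammer.
; Interaction on the owning side asks BP_Pawn_Screen to release its hammer to this slot.
; OccupySlot teleports the hammer to the Sphere, disables slot collision and enables hammer interaction.
; The slot listens for the hammer's OnGrabbed event, then unbinds and restores its collision, freeing itself for reuse.
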(event PressedInteraction(Comp_Interaction)
  (params (Pawn :type BP%20Pawn%20Base%20Object%20Reference) (Souce%20Actor :type Actor%20Object%20Reference) (Hit%20Location :type Vector :default "0, 0, 0") (Hit%20Distance :type Float%20%28single-precision%29) (Hit%20Component :type Actor%20Component%20Object%20Reference))
  (Utilities|IsReplicatedOwner Pawn
    (:Owner
      (bind _asbp_pawn_screen (Utilities|Casting|CastToBP_Pawn_Screen Pawn))
      (Default|ReleaseHammer _asbp_pawn_screen self))))

(event Custom|Unoccupy
  (Variables|Internal|SetOccupied false)
  (Collision|SetActorEnableCollision true))

(event Custom|Occupy%20Slot
  (params (Hammer :type BP%20Hammer%20Object%20Reference))
  (Variables|Internal|SetOccupied true)
  (Transformation|SetActorTransform Hammer (Transformation|GetWorldTransform (Variables|Default|GetSphere)) false true)
  (Collision|SetActorEnableCollision false)
  (Default|SetInteractionEnabled (Variables|/Game/_Overseas/Development/Blueprints/Assets/Repairing/BP_Hammer.BP_Hammer_C|GetComp_Interaction Hammer) true)
  (EventDispatchers|BindEventtoOnGrabbed Hammer (delegate Custom|On%20Grabbed)))

(event Custom|On%20Grabbed
  (params (Pawn :type BP%20Pawn%20Base%20Object%20Reference) (Hammer%20Reference :type BP%20Hammer%20Object%20Reference))
  (EventDispatchers|UnbindEventfromOnGrabbed Hammer%20Reference (delegate Custom|On%20Grabbed))
  (CallFunction|Unoccupy))

(fn ConstructionScript)

(fn GetHammerfromPlayer
  (params (Pawn :type BP%20Pawn%20Base%20Object%20Reference))
  (for _array_element (Actor|GetAttachedActors Pawn true)
    (if (or (== (Utilities|GetClass _array_element) "/Game/_Overseas/Development/Blueprints/Assets/Repairing/BP_Hammer.BP_Hammer_C") (Utilities|ClassIsChildOf (Utilities|GetClass _array_element) "/Game/_Overseas/Development/Blueprints/Assets/Repairing/BP_Hammer.BP_Hammer_C"))
      (bind _asbp_hammer (Utilities|Casting|CastToBP_Hammer _array_element))
      (return _asbp_hammer))))