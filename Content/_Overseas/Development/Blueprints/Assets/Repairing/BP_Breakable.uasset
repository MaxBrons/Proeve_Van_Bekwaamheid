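; BP_Breakable is an object with health that can be damaged and repaired.
; It calls Repair with MaxHealth on BeginPlay, so it starts at full health.
; Damage and Repair subtract or add the given amount, clamp Health between zero and MaxHealth, then fire the OnHealthUpdated dispatcher with the new value.
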(event Custom|Repair
  (params (Percentage :type Float%20%28single-precision%29))
  (Variables|Internal|SetHealth (Math|Float|Clamp(Float) (+ (Variables|Internal|GetHealth) Percentage) 0.0 (Variables|Settings|GetMax%20Health)))
  (Default|CallOnHealthUpdated (Variables|Internal|GetHealth)))

(event Custom|Damage
  (params (Percentage :type Float%20%28single-precision%29))
  (Variables|Internal|SetHealth (Math|Float|Clamp(Float) (- (Variables|Internal|GetHealth) Percentage) 0.0 (Variables|Settings|GetMax%20Health)))
  (Default|CallOnHealthUpdated (Variables|Internal|GetHealth)))

(event EventBeginPlay
  (CallFunction|Repair (Variables|Settings|GetMax%20Health)))

(fn ConstructionScript)