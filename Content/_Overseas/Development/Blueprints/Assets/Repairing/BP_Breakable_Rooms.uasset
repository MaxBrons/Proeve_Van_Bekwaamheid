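; BP_Breakable_Rooms is a breakable room whose damaged walls the player repairs by holding select on them.
; Select components on WallsToDamage drive highlight and press events, with a retriggerable gate hiding the health widget once highlighting stops.
; The Controll Repair gate-and-delay loop applies RepairRate repeatedly until release.
; Repair and Damage extend the parent's logic and refresh the health percentage shown on the screen pawn's HUD.
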(event Custom|Update%20Widget
  (bind _breakable_widget (Variables|Internal|GetBreakable%20Widget)
    (:then
      (Default|SetupWidget _breakable_widget (Math|Float|Clamp(Float) (* (/ 1e+02 (Variables|Default|GetMax%20Health)) (Variables|Default|GetHealth)) 0.0 1e+02)))
    (:else)))

(event Custom|On%20Highlight
  (params (Pawn :type BP%20Pawn%20Base%20Object%20Reference) (Source%20Actor :type Actor%20Object%20Reference) (Hit%20Location :type Vector) (Hit%20Rotation :type Rotator) (Hit%20Component :type Actor%20Component%20Object%20Reference))
  (Utilities|RetriggerableGate 0.1
    (:Output
      (Variables|Internal|SetCurrent%20Pawn Pawn)
      (CallFunction|ShowWidget true))
    (:Reset
      (CallFunction|ShowWidget false)
      (Variables|Internal|SetCurrent%20Pawn 0))))

(event Custom|On%20Select
  (params (Pawn :type BP%20Pawn%20Base%20Object%20Reference) (Souce%20Actor :type Actor%20Object%20Reference) (Hit%20Location :type Vector) (Hit%20Component :type Actor%20Component%20Object%20Reference))
  (Utilities|ControllRepair (Variables|Settings|GetRepair%20Delay)))

(event Custom|On%20Released
  (Utilities|ControllRepair (Variables|Settings|GetRepair%20Delay)) ; enters at Stop
)

(event Custom|Show%20Widget
  (params (Set :type Boolean))
  (bind _self self)
  (bind _returnvalue (Utilities|GetObjectName _self))
  (bind _returnvalue_2 (Utilities|String|StringToName _returnvalue))
  (bind _current_pawn (Variables|Internal|GetCurrent%20Pawn)
    (:then
      (bind _asbp_pawn_screen (Utilities|Casting|CastToBP_Pawn_Screen _current_pawn))
      (bind _breakable_widget (Variables|Internal|GetBreakable%20Widget)
        (:then
          (if Set
            (Default|AddWidgettoViewport _asbp_pawn_screen _returnvalue_2 _breakable_widget 1)
            (CallFunction|UpdateWidget)
            (else
              (Default|RemoveWidgetfromViewport _asbp_pawn_screen _returnvalue_2))))
        (:else)))
    (:else)))

(event EventBeginPlay
  (|CallParentFunction)
  (bind _returnvalue (UserInterface|CreateWidget "/Game/_Overseas/Development/Blueprints/Widgets/HUD/WB_Screen_Breakable.WB_Screen_Breakable_C" 0 0 0))
  (Variables|Internal|SetBreakable%20Widget _returnvalue)
  (for _array_element (Variables|Settings|GetWalls%20To%20Damage)
    (Utilities|IsValid (Actor|GetComponentbyClass _array_element "/Game/_Overseas/Development/Blueprints/Components/Core/Comp_Select.Comp_Select_C")
      (:Is%20Valid
        (EventDispatchers|BindEventtoHighlightSelect (Actor|GetComponentbyClass _array_element "/Game/_Overseas/Development/Blueprints/Components/Core/Comp_Select.Comp_Select_C") (delegate Custom|On%20Highlight))
        (EventDispatchers|BindEventtoPressedSelect (Actor|GetComponentbyClass _array_element "/Game/_Overseas/Development/Blueprints/Components/Core/Comp_Select.Comp_Select_C") (delegate Custom|On%20Select))
        (EventDispatchers|BindEventtoReleasedSelect (Actor|GetComponentbyClass _array_element "/Game/_Overseas/Development/Blueprints/Components/Core/Comp_Select.Comp_Select_C") (delegate Custom|On%20Released)))))
  (Variables|Default|SetHealth 15.0))

(event EventRepair
  (params (Percentage :type Float%20%28single-precision%29))
  (|CallParentFunction Percentage)
  (CallFunction|UpdateWidget))

(event EventDamage
  (params (Percentage :type Float%20%28single-precision%29))
  (|CallParentFunction Percentage)
  (CallFunction|UpdateWidget))

(fn ConstructionScript
  (|CallParentFunction))