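; Torpedo loading hole with a hinged hatch (Klep) that toggles open and closed on interaction, plus a torpedo mesh that shows whether it is occupied.
; The Open timeline acts as a tick, stepping the hatch's yaw until a computed angle passes its start or open limit.
; Opened and Occupied changes fire TorpedoHoleUpdated; both variables have empty OnRep functions.
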(event PressedInteraction(Comp_Interaction)
  (params (Pawn :type BP%20Pawn%20Base%20Object%20Reference) (Souce%20Actor :type Actor%20Object%20Reference) (Hit%20Location :type Vector :default "0, 0, 0") (Hit%20Distance :type Float%20%28single-precision%29) (Hit%20Component :type Actor%20Component%20Object%20Reference))
  (bind _open_rotation (Variables|Internal|GetOpen%20Rotation))
  (bind _start_rotation (Variables|Internal|GetStart%20Rotation))
  (bind _klep (Variables|Default|GetKlep))
  (Utilities|FlowControl|Sequence
    (:then_0
      (goto _label Reset))
    (:then_1
      (goto _label_2 Reset))
    (:then_2
      (Utilities|FlowControl|FlipFlop
        (:A
          (bind (_direction _alpha) (Timeline|Open Play)
            (:Update
              (switch Utilities|FlowControl|Switch|SwitchonETimelineDirection _direction
                (:Forward
                  (if (>= (CallFunction|GetKlepLocalRotation) _open_rotation)
                    (Utilities|FlowControl|DoOnce false :!label _label
                      (:Completed
                        (bind _output_get (Variables|Internal|SetOpened true))
                        (Default|CallTorpedoHoleUpdated _output_get (Variables|Internal|GetOccupied))))
                    (else
                      (Transformation|AddLocalRotation _klep (Math|Rotator|MakeRotator 0.0 0.0 (/ _open_rotation (Variables|Internal|GetSteps))) false false))))
                (:Backward
                  (if (<= (CallFunction|GetKlepLocalRotation) _start_rotation)
                    (Utilities|FlowControl|DoOnce false :!label _label_2
                      (:Completed
                        (bind _output_get_2 (Variables|Internal|SetOpened false))
                        (Default|CallTorpedoHoleUpdated _output_get_2 (Variables|Internal|GetOccupied))))
                    (else
                      (Transformation|AddLocalRotation _klep (Math|Rotator|MakeRotator 0.0 0.0 (* (/ (- (Variables|Internal|GetOpen%20Rotation) _start_rotation) (Variables|Internal|GetSteps)) -1.0)) false false))))))))
        (:B
          (Timeline|Open Reverse))))))

(event Custom|Set%20Torpedo%20Active
  (params (Set :type Boolean))
  (Development|SetHiddeninGame (Variables|Default|GetTorpedo) (not Set) false)
  (bind _output_get (Variables|Internal|SetOccupied Set))
  (Default|CallTorpedoHoleUpdated (Variables|Internal|GetOpened) _output_get))

(event EventBeginPlay
  (Variables|Internal|SetStart%20Rotation (CallFunction|GetKlepLocalRotation))
  (Variables|Internal|SetOpen%20Rotation (+ (Variables|Internal|GetStart%20Rotation) 1.5e+02)))

(fn ConstructionScript)

(fn GetKlepLocalRotation
  (return (- (+ (* (.yaw (Transformation|GetWorldRotation (Variables|Default|GetDefaultSceneRoot))) -1.0) (.yaw (Variables|/Script/Engine.SceneComponent|GetRelativeRotation (Variables|Default|GetKlep)))) 9e+01)))

(fn IsOpened
  (return (Variables|Internal|GetOpened)))

(fn IsOccupied
  (return (Variables|Internal|GetOccupied)))

(fn OnRepOccupied)

(fn OnRepOpened)