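; Radar actor that plots enemy ships on a WB_Radar widget and triggers a steering task for the player.
; On BeginPlay it binds to the widget and to BP_Enemy_Ship_Manager's spawn and destroy events.
; Spawned ships become dots at a 0–360 degree bearing from the radar, computed with Atan2, and destroyed ships lose theirs.
; When the widget generates a course, the player pawn's HandleTask updates the configured steering task's state.
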(event Custom|Ship%20Spawned
  (params (Ship%20Reference :type BP%20Enemy%20Ship%20Object%20Reference) (Spawn%20Location :type Vector))
  (bind _radar_widget (Variables|Internal|GetRadar%20Widget)
    (:then
      (Default|AddDot _radar_widget (CallFunction|CalculateCource Spawn%20Location) Ship%20Reference))
    (:else)))

(event Custom|Course%20Generated
  (params (Course :type Integer))
  ;[1 1 1] Start the steering task
  (bind _steering_task_to_activate (Variables|Settings|GetSteering%20Task%20To%20Activate)
    (:then
      (Default|HandleTask (CallFunction|GetMainPlayerPawn self) _steering_task_to_activate "NewEnumerator1"))
    (:else)))

(event Custom|Ship%20Destroyed
  (params (Ship%20Reference :type BP%20Enemy%20Ship%20Object%20Reference) (Course :type Float%20%28single-precision%29))
  (bind _radar_widget (Variables|Internal|GetRadar%20Widget)
    (:then
      (Default|RemoveDot _radar_widget Ship%20Reference))
    (:else)))

(event EventBeginPlay
  (bind _current_widget (Variables|/Game/_Overseas/Development/Blueprints/Components/Core/Comp_Widget.Comp_Widget_C|GetCurrent%20Widget (Variables|Default|GetComp_Widget))
    (:then
      (bind _aswb_radar (Utilities|Casting|CastToWB_Radar _current_widget))
      (bind _output_get (Variables|Internal|SetRadar%20Widget _aswb_radar))
      (EventDispatchers|BindEventtoOnCourseGenerated _output_get (delegate Custom|Course%20Generated))
      (bind _returnvalue (Actor|GetActorOfClass "/Game/_Overseas/Development/Blueprints/Systems/Enemy_Ship/BP_Enemy_Ship_Manager.BP_Enemy_Ship_Manager_C"))
      (Variables|Internal|SetShip%20Manager _returnvalue)
      (bind _ship_manager (Variables|Internal|GetShip%20Manager)
        (:then
          (EventDispatchers|BindEventtoOnShipSpawned _ship_manager (delegate Custom|Ship%20Spawned))
          (EventDispatchers|BindEventtoOnShipDestroyed _ship_manager (delegate Custom|Ship%20Destroyed)))
        (:else)))
    (:else)))

(fn ConstructionScript)

(fn CalculateCource
  (params (Location :type Vector))
  (bind _returnvalue (Transformation|GetActorLocation))
  (bind _returnvalue_2 (- Location _returnvalue))
  (bind _returnvalue_3 (Class|KismetMathLibrary|DegAtan2 (.y _returnvalue_2) (.x _returnvalue_2)))
  (bind _returnvalue_4 (< _returnvalue_3 0.0))
  (bind _returnvalue_5 (- 3.6e+02 _returnvalue_3))
  (bind _returnvalue_6 (select _returnvalue_4 _returnvalue_5 _returnvalue_3))
  (return (select (> _returnvalue_6 3.6e+02) (+ 3.6e+02 _returnvalue_3) _returnvalue_6)))