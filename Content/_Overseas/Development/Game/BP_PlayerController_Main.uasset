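; Main player controller that handles spawn placement, pawn switching and HUD color updates.
; InitiatePlayer finds a PlayerStart and retries on a short delay until a controlled pawn exists, then moves it there.
; SwitchPawn fades the camera out, possesses the new pawn, fades back in and calls OnPawnSwitched.
; UpdateHUDColor sets the main HUD to either a given color or its default.
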(event Custom|Switch%20Pawn
  (params (New%20Pawn :type BP%20Pawn%20Base%20Object%20Reference))
  (bind _returnvalue (Game|GetPlayerCameraManager 0))
  (CameraFades|StartCameraFade :self _returnvalue :FromAlpha 0.0 :ToAlpha 1.0 :Duration 0.8 :bHoldWhenFinished true)
  (Utilities|FlowControl|Delay 0.8)
  (Pawn|Possess New%20Pawn)
  (CameraFades|StartCameraFade :self _returnvalue :FromAlpha 1.0 :ToAlpha 0.0 :Duration 0.8 :bHoldWhenFinished true)
  (Default|CallOnPawnSwitched (.AsBP%20Player%20Controller%20Main (Utilities|Casting|CastToBP_PlayerController_Main (Pawn|GetController New%20Pawn))) New%20Pawn))

(event Custom|Update%20HUD%20Color
  (params (Color :type Linear%20Color%20Structure :default "(R=0.000000,G=0.630561,B=1.000000,A=1.000000)") (Use%20Default :type Boolean))
  (bind _asbp_hud_main (Utilities|Casting|CastToBP_HUD_Main (HUD|GetHUD)))
  (Variables|/Game/_Overseas/Development/Game/BP_HUD_Main.BP_HUD_Main_C|SetHUD%20Color _asbp_hud_main (Math|Color|SelectColor (Variables|/Game/_Overseas/Development/Game/BP_HUD_Main.BP_HUD_Main_C|GetDefault%20Color _asbp_hud_main) Color Use%20Default)))

(event Custom|Initiate%20Player
  (bind _returnvalue (Pawn|GetControlledPawn))
  (bind _player_start (CallFunction|GetSpawnPosition))
  (Utilities|IsValid _player_start
    (:Is%20Valid
      (Utilities|IsValid _returnvalue :!label _label
        (:Is%20Valid
          (Transformation|SetActorTransform _returnvalue (Math|Transform|MakeTransform (.location (Transformation|GetActorTransform _player_start)) (.rotation (Transformation|GetActorTransform _player_start)) "1,1,1")))
        (:Is%20Not%20Valid
          (Utilities|FlowControl|Delay 0.05)
          (goto _label))))))

(fn ConstructionScript)

(fn GetSpawnPosition
  (bind _returnvalue (Actor|GetActorOfClass "/Script/Engine.PlayerStart"))
  (return _returnvalue))