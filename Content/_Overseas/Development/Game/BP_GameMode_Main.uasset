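; Main game mode that keeps a roster of connected players, each with a numeric ID.
; PostLogin and logout handle only BP_PlayerController_Main, adding it to or removing it from the PlayerList map, then calling the matching login or logout notification.
; GetFreePlayerID assigns IDs by counting upward until it finds a value not already in the map, so freed IDs can be reused.
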(event EventBeginPlay)

(event EventTick
  (params (DeltaSeconds :type Float%20%28single-precision%29)))

(event EventPostLogin
  (params (NewPlayer :type Player%20Controller%20Object%20Reference))
  (|CallParentFunction NewPlayer)
  (bind _asbp_player_controller_main (Utilities|Casting|CastToBP_PlayerController_Main NewPlayer))
  (CallFunction|AddPlayer _asbp_player_controller_main)
  (Default|CallOnPlayerLogin))

(event EventOnLogout
  (params (ExitingController :type Controller%20Object%20Reference))
  (|CallParentFunction ExitingController)
  (bind _asbp_player_controller_main (Utilities|Casting|CastToBP_PlayerController_Main ExitingController))
  (CallFunction|RemovePlayer _asbp_player_controller_main)
  (Default|CallOnPlayerLogOut))

(fn ConstructionScript)

(fn AddPlayer
  (params (Controller :type BP%20Player%20Controller%20Main%20Object%20Reference))
  (bind _asbp_player_controller_main (Utilities|Casting|CastToBP_PlayerController_Main Controller))
  (Utilities|Map|Add (Variables|Settings|GetPlayer%20List) _asbp_player_controller_main (CallFunction|GetFreePlayerID)))

(fn RemovePlayer
  (params (Controller :type BP%20Player%20Controller%20Main%20Object%20Reference))
  (Utilities|Map|Remove (Variables|Settings|GetPlayer%20List) Controller))

(fn GetFreePlayerID
  (bind _id (LocalVariables|GetID))
  (bind _values (Utilities|Map|Values (Variables|Settings|GetPlayer%20List) :!label _label))
  (if (Utilities|Array|ContainsItem _values (LocalVariables|GetID))
    (Math|Integer|IncrementInt _id
      (:%20%20
        (goto _label)))
    (else
      (return _id))))