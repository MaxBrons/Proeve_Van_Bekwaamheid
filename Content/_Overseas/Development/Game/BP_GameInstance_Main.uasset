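; Main game instance that creates and destroys online sessions and handles transitions between levels.
; Initiating a session sets a session-active flag on success, then switches to the given map info's level.
; Level switching optionally fades the camera out, stores the current map info, then opens the level, as a listen server if a session is active.
; Requested server travel runs only on the server, using a console command during active sessions.
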(event Custom|Switch%20Level
  (params (Map%20Info :type BP%20Map%20Info%20Object%20Reference) (With%20Fade :type Boolean) (Server%20Travel :type Boolean))
  ;[1 1 1] Use camera fade and set the currently used map info
  (Utilities|IsValid Map%20Info
    (:Is%20Valid
      (if With%20Fade
        (CameraFades|StartCameraFade :self (Game|GetPlayerCameraManager 0) :ToAlpha 1.0 :Duration 0.8)
        (Utilities|FlowControl|Delay 0.8))
      (Variables|Internal|SetCurrent%20Map%20Info Map%20Info)
      ;[1 1 1] Do a server transition or open a normal level
      (if Server%20Travel
        (if (Networking|IsServer)
          (if (Variables|Internal|GetSession%20Active)
            (Development|ExecuteConsoleCommand (Utilities|String|Append "servertravel " (Utilities|String|ToString(Name) (Variables|/Game/_Overseas/Development/Game/BP_MapInfo.BP_MapInfo_C|GetMap%20To%20Transition%20To (Variables|Internal|GetCurrent%20Map%20Info)))) (Game|GetPlayerController 0))
            (else
              (Game|OpenLevel(byName) (Variables|/Game/_Overseas/Development/Game/BP_MapInfo.BP_MapInfo_C|GetMap%20To%20Transition%20To (Variables|Internal|GetCurrent%20Map%20Info)) true (select (Variables|Internal|GetSession%20Active) "listen" "") :!label _label))))
        (else
          (goto _label))))
    (:Is%20Not%20Valid
      (Development|PrintString "No Map Info found"))))

(event Custom|Remove%20Session
  ;[1 1 1] Create or destroy a session and transfer the player to the next level when the session is created
  (|DestroySession (Game|GetPlayerController 0)
    (:OnSuccess
      (Variables|Internal|SetSession%20Active false))))

(event Custom|Initiate%20Session
  (params (Map%20Info :type BP%20Map%20Info%20Object%20Reference))
  ;[1 1 1] Create or destroy a session and transfer the player to the next level when the session is created
  (|Session (Game|GetPlayerController 0) 10 false
    (:OnSuccess
      (Variables|Internal|SetSession%20Active true)
      (CallFunction|SwitchLevel Map%20Info true false))))