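; Temporary desktop player pawn with first-person movement, mouse look and object selection.
; On BeginPlay it attaches the spring arm to the mesh's head socket and fades the camera in; input axes drive capsule-relative movement and controller rotation.
; A visibility line trace from the camera's forward vector feeds highlighting and HUD color updates each tick, and selection of Comp_Select objects when Fire is pressed.
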(event EventBeginPlay
  ;[1 1 1] Attach the camera to the head of the player mesh and fade in
  (Transformation|AttachComponentToComponent (Variables|Default|GetSpringArm) (Variables|Character|GetMesh) "head" "KeepWorld" "KeepWorld" "KeepWorld" true)
  (CameraFades|StartCameraFade :self (Game|GetPlayerCameraManager 0) :FromAlpha 1.0 :Duration 0.8))

(event EventTick
  (params (DeltaSeconds :type Float%20%28single-precision%29))
  ;[1 1 1] Update the highlight, the hud color and the physics handle location;
  (|CallParentFunction DeltaSeconds)
  (Utilities|IsValid (Game|GetPlayerController 0)
    (:Is%20Valid
      (bind _out_hit (CallFunction|TraceforMouse))
      (CallFunction|TrytoHighlight _out_hit)
      (CallFunction|UpdateHUDColor _out_hit))))

(event Input|ActionEvents|InputActionFire
  (params (Key :type Key%20Structure :default "None"))
  ;[1 1 1] Try to select an object with a Comp_Select on it, when the fire button is pressed
  (:Pressed
    (bind _out_hit (CallFunction|TraceforMouse))
    (CallFunction|TrytoSelect _out_hit)))

(event Input|AxisEvents|InputAxisMoveForward
  (params (AxisValue :type Float%20%28single-precision%29))
  ;[1 1 1] Player Movement
  ;;[1 1 1] Movement for moving forward or backwards
  (Pawn|Input|AddMovementInput (Math|Vector|GetForwardVector (Variables|Default|GetCapsuleComponent)) (* AxisValue (Variables|Default|GetMovement%20Speed) (Utilities|Time|GetWorldDeltaSeconds)) false))

(event Input|AxisEvents|InputAxisMoveRight
  (params (AxisValue :type Float%20%28single-precision%29))
  ;[1 1 1] Player Movement
  ;;[1 1 1] Movement for moving right and left
  (Pawn|Input|AddMovementInput (Math|Vector|GetRightVector (Variables|Default|GetCapsuleComponent)) (* AxisValue (Variables|Default|GetMovement%20Speed) (Utilities|Time|GetWorldDeltaSeconds)) false))

(event Input|AxisEvents|InputAxisTurn
  (params (AxisValue :type Float%20%28single-precision%29))
  ;[1 1 1] Player Movement
  ;;[1 1 1] Handle rotation. Only rotate when the right mousebutton is pressed
  (Pawn|Input|AddControllerYawInput (* AxisValue (.x (Variables|Default|GetMouse%20Sensitivity)) (Utilities|Time|GetWorldDeltaSeconds))))

(event Input|AxisEvents|InputAxisLookUp
  (params (AxisValue :type Float%20%28single-precision%29))
  ;[1 1 1] Player Movement
  ;;[1 1 1] Handle rotation. Only rotate when the right mousebutton is pressed
  (Pawn|Input|AddControllerPitchInput (* AxisValue (.y (Variables|Default|GetMouse%20Sensitivity)) (Utilities|Time|GetWorldDeltaSeconds))))

(fn ConstructionScript
  (|CallParentFunction))

(fn TraceforMouse
  (bind _camera (Variables|Default|GetCamera))
  (bind _returnvalue (Transformation|GetWorldLocation _camera))
  (bind _outhit (Collision|LineTraceByChannel _returnvalue (+ (* (Math|Vector|GetForwardVector (Transformation|GetWorldRotation _camera)) 5e+03) _returnvalue) "TraceTypeQuery1" false 0 "None"))
  (return _outhit))